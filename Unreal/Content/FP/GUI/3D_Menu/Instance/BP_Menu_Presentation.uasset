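; BP_Menu_Presentation is a 3D menu actor for the presentation screen, whose Iniciar (start) button launches the intro.
; On BeginPlay it casts the 3dButtonIniciar child actor to BP_Menu_Text3D_Button_Master and binds its click event.
; A click calls StartIntro on the GameMode through BPI_GameMode_Master.
; An unconnected LevelRestart chain via BPI_Level_Master remains in the graph and never runs.
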(event Custom|3DButtonOnClickonClick_Event_Button_Iniciar
  (params (ButtonMasterObject :type BP%20Menu%20Text%203D%20Button%20Master%20Object%20Reference))
  (bind _asbpi_game_mode_master (Utilities|Casting|CastToBPI_GameMode_Master (Game|GetGameMode)))
  (Default|StartIntro _asbpi_game_mode_master))

(event EventBeginPlay
  (|CallParentFunction)
  (Utilities|FlowControl|Sequence
    (:then_0
      (bind _asbp_menu_text_3d_button_master (Utilities|Casting|CastToBP_Menu_Text3D_Button_Master (Variables|/Script/Engine.ChildActorComponent|GetChildActor (Variables|Default|Get3dButton_Iniciar))))
      (EventDispatchers|Assign3DButtononClick _asbp_menu_text_3d_button_master (delegate Custom|3DButtonOnClickonClick_Event_Button_Iniciar)))))

(event Collision|EventActorBeginOverlap
  (params (OtherActor :type Actor%20Object%20Reference))
  (|CallParentFunction OtherActor) ; This node is disabled and will not be called.\nDrag off pins to build functionality.
)

(event EventTick
  (params (DeltaSeconds :type Float%20%28single-precision%29))
  (|CallParentFunction DeltaSeconds) ; This node is disabled and will not be called.\nDrag off pins to build functionality.
)

(fn ConstructionScript
  (|CallParentFunction))