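; BP_Menu_Pause is the 3D pause menu, providing a Continue action through a 3D text button.
; On BeginPlay it casts the Continuar child actor to BP_Menu_Text3D_Button_Master and binds its click to the Continue event.
; Continue casts the game mode to the BPI_GameMode_Master interface and calls OnPause, leaving the pause handling to the game mode.
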(event Custom|Continue
  (bind _asbpi_game_mode_master (Utilities|Casting|CastToBPI_GameMode_Master (Game|GetGameMode)))
  (Default|OnPause _asbpi_game_mode_master))

(event EventBeginPlay
  (|CallParentFunction)
  (bind _asbp_menu_text_3d_button_master (Utilities|Casting|CastToBP_Menu_Text3D_Button_Master (Variables|/Script/Engine.ChildActorComponent|GetChildActor (Variables|Default|GetBP_Menu_Text3D_Button_Master_Continuar))))
  (EventDispatchers|BindEventto3DButtononClick _asbp_menu_text_3d_button_master (delegate Custom|Continue)))

(event Collision|EventActorBeginOverlap
  (params (OtherActor :type Actor%20Object%20Reference))
  (|CallParentFunction OtherActor) ; This node is disabled and will not be called.\nDrag off pins to build functionality.
)

(event EventTick
  (params (DeltaSeconds :type Float%20%28single-precision%29))
  (|CallParentFunction DeltaSeconds) ; This node is disabled and will not be called.\nDrag off pins to build functionality.
)

(fn ConstructionScript
  (|CallParentFunction))