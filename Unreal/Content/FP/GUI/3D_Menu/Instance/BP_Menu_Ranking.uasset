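; 3D menu screen that shows Top 10 rankings for the Easy, Medium and Hard difficulties.
; The construction script fetches the three rankings through GISSRanking and spawns a 3D text button child actor for each, mapping ranking to component.
; A click handler matches the button in that map, then SetRanking moves the indicator beside it and refreshes the Top 10 widget.
; Per-difficulty events remain, but their button bindings are disconnected.
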(event Custom|setRanking_Hard
  (params (ButtonMasterObject :type BP%20Menu%20Text%203D%20Button%20Master%20Object%20Reference))
  (bind _ranking (Default|GetRankingObject (Subsystems|GetGISSRanking) "NewEnumerator2"))
  (CallFunction|SetRanking _ranking))

(event Custom|setRanking_Easy
  (params (ButtonMasterObject :type BP%20Menu%20Text%203D%20Button%20Master%20Object%20Reference))
  (Default|GetRankingObject (Subsystems|GetGISSRanking) "NewEnumerator0")
  (CallFunction|SetRanking))

(event Custom|setRanking_Medium
  (params (ButtonMasterObject :type BP%20Menu%20Text%203D%20Button%20Master%20Object%20Reference))
  (bind _ranking (Default|GetRankingObject (Subsystems|GetGISSRanking) "NewEnumerator1"))
  (CallFunction|SetRanking _ranking))

(event EventBeginPlay
  (|CallParentFunction))

(event Collision|EventActorBeginOverlap
  (params (OtherActor :type Actor%20Object%20Reference))
  (|CallParentFunction OtherActor) ; This node is disabled and will not be called.\nDrag off pins to build functionality.
)

(event EventTick
  (params (DeltaSeconds :type Float%20%28single-precision%29))
  (|CallParentFunction DeltaSeconds) ; This node is disabled and will not be called.\nDrag off pins to build functionality.
)

(fn ConstructionScript
  (|CallParentFunction)
  (CallFunction|Setup))

(fn SetRanking
  (params (Ranking%20Object :type BPO%20Ranking%20Object%20Reference))
  (Variables|Default|SetCurrentRanking Ranking%20Object)
  (CallFunction|ShowSelector)
  (Default|SetRankingTop10 (Variables|Default|GetWidget%20Ranking%20Top%2010) Ranking%20Object))

(fn ShowSelector
  (bind (_keypin _valuepin) (Utilities|Map|ForEachLoop(Map) (Variables|Default|GetRankingSelectorList) :!label _label)
    (:then
      (if (Utilities|Enum|Equal(Enum) (Class|RankingNameInterface|GetRankName (Variables|Default|GetCurrentRanking)) (Class|RankingNameInterface|GetRankName _keypin))
        (Transformation|SetRelativeLocation (Variables|Default|GetIndicator) (Math|Vector|MakeVector -1e+01 (- (.y (Variables|/Script/Engine.SceneComponent|GetRelativeLocation _valuepin)) 7e+01) (.z (Variables|/Script/Engine.SceneComponent|GetRelativeLocation _valuepin))) false false)
        (goto _label BreakPin)))
    (:CompletedPin
      (CallFunction|DebugLogString self "ALGO"))))

(fn Setup
  (bind _returnvalue (Subsystems|GetGISSRanking))
  (bind _rankinglist (LocalVariables|GetRankingList))
  (Utilities|FlowControl|Sequence
    (:then_0
      (bind _asbp_widget_ranking_top_10 (Utilities|Casting|CastToBP_Widget_Ranking_Top10 (Variables|/Script/Engine.ChildActorComponent|GetChildActor (Variables|Default|GetWidget_top10))))
      (Variables|Default|SetWidget%20Ranking%20Top%2010 _asbp_widget_ranking_top_10))
    (:then_1
      (bind _ranking (Default|GetRankingObject _returnvalue "NewEnumerator0"))
      (Utilities|Array|Add _rankinglist _ranking)
      (bind _ranking_2 (Default|GetRankingObject _returnvalue "NewEnumerator1"))
      (Utilities|Array|Add _rankinglist _ranking_2)
      (bind _ranking_3 (Default|GetRankingObject _returnvalue "NewEnumerator2"))
      (Utilities|Array|Add _rankinglist _ranking_3))
    (:then_2
      (for (_array_element _array_index) (LocalVariables|GetRankingList)
        (bind _childactorcomponent (CallFunction|InstanciateRankingSelector _array_index _array_element))
        (Utilities|Map|Add (Variables|Default|GetRankingSelectorList) _array_element _childactorcomponent)))))

(fn InstanciateRankingSelector
  (params (Index :type Integer) (Ranking%20Object :type BPO%20Ranking%20Object%20Reference))
  (bind _returnvalue (AddComponent|AddChildActorComponent false (Math|Transform|MakeTransform (Math|Vector|MakeVector -1e+01 -7e+02 (- (Math|Float|MakeLiteralFloat 1.5e+02) (* Index 80))))))
  (ChildActorComponent|SetChildActorClass _returnvalue "/Game/FP/BluePrints/Objects/MenuButtons/Master/BP_Menu_Text3D_Button_Master.BP_Menu_Text3D_Button_Master_C")
  (bind _asbp_menu_text_3d_button_master (Utilities|Casting|CastToBP_Menu_Text3D_Button_Master (Variables|/Script/Engine.ChildActorComponent|GetChildActor _returnvalue)))
  (Variables|/Game/FP/BluePrints/Objects/MenuButtons/Master/BP_Menu_Text3D_Button_Master.BP_Menu_Text3D_Button_Master_C|SetAlignment _asbp_menu_text_3d_button_master "NewEnumerator0")
  (Default|SetText _asbp_menu_text_3d_button_master (Utilities|Text|ToText(String) (Default|GetCaption Ranking%20Object)))
  (EventDispatchers|BindEventto3DButtononClick _asbp_menu_text_3d_button_master (EventDispatchers|CreateEvent :!event BPMenuRankingAutoGenFunc))
  (return _asbp_menu_text_3d_button_master _returnvalue))

(fn BPMenuRankingAutoGenFunc
  (params (ButtonMasterObject :type BP%20Menu%20Text%203D%20Button%20Master%20Object%20Reference))
  (bind (_keypin _valuepin) (Utilities|Map|ForEachLoop(Map) (Variables|Default|GetRankingSelectorList))
    (:then
      (bind _asbp_menu_text_3d_button_master (Utilities|Casting|CastToBP_Menu_Text3D_Button_Master (Variables|/Script/Engine.ChildActorComponent|GetChildActor _valuepin)))
      (if (== _asbp_menu_text_3d_button_master ButtonMasterObject)
        (CallFunction|SetRanking _keypin)))))