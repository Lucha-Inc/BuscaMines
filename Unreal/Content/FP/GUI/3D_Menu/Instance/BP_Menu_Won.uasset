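; BP_Menu_Won is the 3D win menu actor that displays the player's score.
; On BeginPlay it runs the parent logic and then Setup, which reads the score from the BoardMaster's stats, reached through the custom GameModeMaster.
; Setup casts the score child actor to BP_Text3D_text and sets its text to a hardcoded Spanish "Puntaje" label followed by the points.
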(event Custom|setup
  (Utilities|FlowControl|Sequence
    (:then_0
      (bind _gamemode_master (CallFunction|GetCustomClasses self))
      (bind _statobject (Default|GetStats (Variables|/Game/FP/BluePrints/Global/GM_GameModes/BP_Abstract_GameMode_Master.BP_Abstract_GameMode_Master_C|GetBoard_Master _gamemode_master)))
      (bind _score (Default|GetScore _statobject))
      (bind _asbp_text_3d_text (Utilities|Casting|CastToBP_Text3D_text (Variables|/Script/Engine.ChildActorComponent|GetChildActor (Variables|Default|GetBP_Text3D_text_Score))))
      (Default|SetText _asbp_text_3d_text (Utilities|Text|FormatText "Puntaje: {points}" _score)))))

(event EventBeginPlay
  (|CallParentFunction)
  (CallFunction|Setup))

(event Collision|EventActorBeginOverlap
  (params (OtherActor :type Actor%20Object%20Reference))
  (|CallParentFunction OtherActor) ; This node is disabled and will not be called.\nDrag off pins to build functionality.
)

(event EventTick
  (params (DeltaSeconds :type Float%20%28single-precision%29))
  (|CallParentFunction DeltaSeconds) ; This node is disabled and will not be called.\nDrag off pins to build functionality.
)

(fn ConstructionScript
  (|CallParentFunction))