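; Master 3D menu actor that provides a menu panel with a 3D text title and a solid or transparent background.
; BaseSolidReference's scale drives the layout: construction places the title child actor, and BeginPlay sizes the rounded widget background used in transparent mode.
; ShowMenu unhides the root and calls Shown.
; Getters expose default and actor-scaled dimensions plus the screen width relation.
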(event Custom|setup_background
  (bind _widget_background (Variables|Default|GetWidget_background))
  (bind _base_solid_reference (Variables|Default|Getbase_solid_reference))
  (bind _returnvalue (Transformation|GetRelativeTransform _widget_background))
  (bind _returnvalue_2 (Transformation|GetRelativeTransform _base_solid_reference))
  (Utilities|FlowControl|Sequence
    (:then_0
      (Development|SetHiddeninGame (Variables|Default|Getbase_solid_visible) (Variables|Layout|Gettransparent_background) false))
    (:then_1
      (Development|SetHiddeninGame (Variables|Default|GetWidget_background) (not (Variables|Layout|Gettransparent_background)) false)
      (Class|WidgetComponent|SetDrawSize (Variables|Default|GetWidget_background) (Math|Vector2D|MakeVector2D (* (.y (.scale _returnvalue_2)) 1e+02) (* (.z (.scale _returnvalue_2)) 1e+02)))
      (Transformation|SetRelativeTransform _widget_background (Math|Transform|MakeTransform (.location _returnvalue_2) (.rotation _returnvalue) (.scale _returnvalue)) false false)
      (Transformation|AddLocalOffset _widget_background (Math|Vector|MakeVector (+ (* (.x (.scale _returnvalue_2)) 5e+01) 1.0) 0.0 0.0) false false)
      (bind _asrounded_base (Utilities|Casting|CastToRoundedBase (UserInterface|GetUserWidgetObject (Variables|Default|GetWidget_background))))
      (Default|SetupProps _asrounded_base (* (.y (.scale (Transformation|GetRelativeTransform (Variables|Default|Getbase_solid_reference)))) 3.0) 0.95))))

(event Custom|ShowMenu
  (Development|SetHiddeninGame (Variables|Default|GetDefaultSceneRoot) false false)
  (Default|CallShown))

(event EventBeginPlay
  (CallFunction|SetupBackground))

(event Collision|EventActorBeginOverlap
  (params (OtherActor :type Actor%20Object%20Reference)))

(event EventTick
  (params (DeltaSeconds :type Float%20%28single-precision%29)))

(event Custom|SetTitle
  (params (NewTitle :type Text))
  (Variables|parameters|SetsTitleText NewTitle)
  (bind _asbp_text_3d_title (Utilities|Casting|CastToBP_Text3D_Title (Variables|/Script/Engine.ChildActorComponent|GetChildActor (Variables|Default|GetBP_Menu_Text3D_Title))))
  (Default|SetText _asbp_text_3d_title (Variables|parameters|GetsTitleText)))

(fn ConstructionScript
  (bind _bp_menu_text3d_title (Variables|Default|GetBP_Menu_Text3D_Title))
  (bind _base_solid_reference (Variables|Default|Getbase_solid_reference))
  (bind _returnvalue (Transformation|GetRelativeTransform _base_solid_reference))
  (Utilities|FlowControl|Sequence
    (:then_0
      (Utilities|FlowControl|Sequence
        (:then_0
          (CallFunction|SetTitle (Variables|parameters|GetsTitleText)))
        (:then_1
          (Transformation|SetRelativeTransform _bp_menu_text3d_title (Math|Transform|MakeTransform (.location _returnvalue) (.rotation _returnvalue) "2.000000,2.000000,2.000000") false false)
          (Transformation|AddLocalOffset _bp_menu_text3d_title (Math|Vector|MakeVector (- (* (.x (.scale _returnvalue)) -5e+01) 1e+01) 0.0 (- (* (.z (.scale _returnvalue)) 5e+01) 3.5e+02)) false false))))
    (:then_1
      (Utilities|FlowControl|Sequence))))

(fn GetCurrentDimension
  (bind _returnvalue (Transformation|GetActorScale3D))
  (bind _defaultdimension (CallFunction|GetDefaultDimension))
  (return (Math|Vector2D|MakeVector2D (* (.y _returnvalue) (.x _defaultdimension)) (* (.z _returnvalue) (.y _defaultdimension)))))

(fn GetDefaultDimension
  (bind _base_solid_reference (Variables|Default|Getbase_solid_reference))
  (bind _returnvalue (Transformation|GetRelativeTransform _base_solid_reference))
  (return (Math|Vector2D|MakeVector2D (* (.y (.scale _returnvalue)) 1e+02) (* (.z (.scale _returnvalue)) 1e+02))))

(fn GetWidthScreenRelation
  (return (Variables|Layout|GetwidthScreenRelation)))