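; BPC_tickCounter is a component that counts frames and fires calls on every second, fifth and tenth tick.
; Event Tick increments TickCounter, then uses modulo checks in a sequence to trigger Call2Ticks, Call5Ticks and Call10Ticks.
; The counter resets to zero on each tenth tick, just before Call10Ticks fires.
; A separate EveryTick function also increments the counter but is not called in these graphs.
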(event EventBeginPlay)

(event EventTick
  (params (DeltaSeconds :type Float%20%28single-precision%29))
  (bind _output_get (Variables|Default|SettickCounter (+ (Variables|Default|GettickCounter) 1)))
  (Utilities|FlowControl|Sequence
    (:then_0
      (if (== (Math|Integer|%(Integer) _output_get 2) 0)
        (Default|Call2Ticks)))
    (:then_1
      (if (== (Math|Integer|%(Integer) _output_get 5) 0)
        (Default|Call5Ticks)))
    (:then_2
      (if (== (Math|Integer|%(Integer) _output_get 10) 0)
        (Variables|Default|SettickCounter 0)
        (Default|Call10Ticks)))))

(fn EveryTick
  (bind _output_get (Variables|Default|SettickCounter (+ (Variables|Default|GettickCounter) 1))))