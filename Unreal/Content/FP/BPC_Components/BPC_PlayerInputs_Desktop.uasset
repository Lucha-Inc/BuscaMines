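; Desktop input component for a board game with mine squares, relaying Enhanced Input actions to the player controller.
; Setup stores the controller and enable flag, then tracks game-mode pause changes.
; While enabled and unpaused, Tick traces under the cursor to set the current square for select and suspect actions.
; Movement, look, pause and menu scroll are forwarded; sideways menu input only logs, and the outline-toggling SetSquare helper is not called here.
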(event Custom|Setup
  (params (Player%20Controller :type BP%20Player%20Controller%20Master%20Object%20Reference) (Enable :type Boolean))
  (Variables|Default|SetPlayerController Player%20Controller)
  (Variables|Default|SetEnable Enable)
  (bind _gamemode_master (CallFunction|GetCustomClasses self))
  (EventDispatchers|BindEventtoPauseChanged _gamemode_master (delegate Custom|onPauseChange))
  (Variables|Default|SetPaused (Default|IsPaused _gamemode_master)))

(event Custom|onPauseChange
  (params (PauseStatus :type Boolean))
  (Variables|Default|SetPaused PauseStatus))

(event EventBeginPlay)

(event EventTick
  (params (DeltaSeconds :type Float%20%28single-precision%29))
  (if (and (Variables|Default|GetEnable) (not (Variables|Default|GetPaused)))
    (bind _asbp_square (Utilities|Casting|CastToBP_Square (.hitactor (.HitResult (Game|Player|GetHitResultUnderCursorbyChannel (Variables|Default|GetPlayerController) "TraceTypeQuery4" true))))
      (:then
        _)
      (:CastFailed
        _))
    (Variables|Default|SetCurrentSquare _asbp_square)))

(event Input|EnhancedActionEvents|EnhancedInputActionmenu_moving_sides
  (params (ActionValue :type Float%20%28double-precision%29) (ElapsedSeconds :type Float%20%28double-precision%29) (TriggeredSeconds :type Float%20%28double-precision%29) (InputAction :type Input%20Action%20Object%20Reference :default "/Game/FP/Inputs/Others/Menu3D/menu_moving_sides.menu_moving_sides"))
  (if (Variables|Default|GetEnable)
    (CallFunction|DebugLogString (Variables|Default|GetPlayerController) (Utilities|String|ToString(Float) ActionValue))))

(event Input|EnhancedActionEvents|EnhancedInputActionmenu_scroll
  (params (ActionValue :type Float%20%28double-precision%29) (ElapsedSeconds :type Float%20%28double-precision%29) (TriggeredSeconds :type Float%20%28double-precision%29) (InputAction :type Input%20Action%20Object%20Reference :default "/Game/FP/Inputs/Others/Menu3D/menu_scroll.menu_scroll"))
  (if (Variables|Default|GetEnable)
    (Default|MenuScroll (Variables|Default|GetPlayerController) ActionValue)))

(event Input|EnhancedActionEvents|EnhancedInputActionplayer_up_down
  (params (ActionValue :type Float%20%28double-precision%29) (ElapsedSeconds :type Float%20%28double-precision%29) (TriggeredSeconds :type Float%20%28double-precision%29) (InputAction :type Input%20Action%20Object%20Reference :default "/Game/FP/Inputs/Others/Player/player_up_down.player_up_down"))
  (if (Variables|Default|GetEnable)
    (Default|PlayerMoveZ (Variables|Default|GetPlayerController) ActionValue)))

(event Input|EnhancedActionEvents|EnhancedInputActiongaming_pause
  (params (ActionValue :type Boolean) (ElapsedSeconds :type Float%20%28double-precision%29) (TriggeredSeconds :type Float%20%28double-precision%29) (InputAction :type Input%20Action%20Object%20Reference :default "/Game/FP/Inputs/Others/Pause/gaming_pause.gaming_pause"))
  (if (Variables|Default|GetEnable)
    (Default|OnPause (Variables|Default|GetPlayerController))))

(event Input|EnhancedActionEvents|EnhancedInputActionboard_suspectMine
  (params (ActionValue :type Boolean) (ElapsedSeconds :type Float%20%28double-precision%29) (TriggeredSeconds :type Float%20%28double-precision%29) (InputAction :type Input%20Action%20Object%20Reference :default "/Game/FP/Inputs/Others/Board/board_suspectMine.board_suspectMine"))
  (bind _currentsquare (Variables|Default|GetCurrentSquare))
  ;[1 1 1] Sospecha una Casilla
  (if (Variables|Default|GetEnable)
    (if (Utilities|IsValid _currentsquare)
      (Default|BoardSuspectSquare (Variables|Default|GetPlayerController) (Default|GetCoords _currentsquare)))))

(event Input|EnhancedActionEvents|EnhancedInputActionboard_selection
  (params (ActionValue :type Boolean) (ElapsedSeconds :type Float%20%28double-precision%29) (TriggeredSeconds :type Float%20%28double-precision%29) (InputAction :type Input%20Action%20Object%20Reference :default "/Game/FP/Inputs/Others/Board/board_selection.board_selection"))
  (bind _currentsquare (Variables|Default|GetCurrentSquare))
  ;[1 1 1] Selecciona una Casilla
  (if (Variables|Default|GetEnable)
    (if (Utilities|IsValid _currentsquare)
      (Default|BoardSelectSquare (Variables|Default|GetPlayerController) (Default|GetCoords _currentsquare)))))

(event Input|EnhancedActionEvents|EnhancedInputActionplayer_movement
  (params (ActionValue :type Vector%202D%20Structure) (ElapsedSeconds :type Float%20%28double-precision%29) (TriggeredSeconds :type Float%20%28double-precision%29) (InputAction :type Input%20Action%20Object%20Reference :default "/Game/FP/Inputs/Others/Player/player_movement.player_movement"))
  (if (Variables|Default|GetEnable)
    (Default|PlayerMoveXY (Variables|Default|GetPlayerController) (Math|Vector2D|MakeVector2D (.x ActionValue) (.y ActionValue)))))

(event Input|EnhancedActionEvents|EnhancedInputActionplayer_looking
  (params (ActionValue :type Vector%202D%20Structure) (ElapsedSeconds :type Float%20%28double-precision%29) (TriggeredSeconds :type Float%20%28double-precision%29) (InputAction :type Input%20Action%20Object%20Reference :default "/Game/FP/Inputs/Others/Player/player_looking.player_looking"))
  (if (Variables|Default|GetEnable)
    (Default|PlayerLook (Variables|Default|GetPlayerController) (Math|Vector2D|MakeVector2D (.x ActionValue) (.y ActionValue)))))

(fn SetSquare
  (params (NewSquare :type BP%20Square%20Object%20Reference))
  (if (== NewSquare (Variables|Default|GetCurrentSquare))
    (return false)
    (else
      (if (Utilities|IsValid (Variables|Default|GetCurrentSquare))
        (Default|SetOutlineonView (Variables|Default|GetCurrentSquare) false))
      (if (Utilities|IsValid NewSquare)
        (bind _output_get (Variables|Default|SetCurrentSquare NewSquare))
        (Default|SetOutlineonView _output_get true)
        (else
          (Variables|Default|SetCurrentSquare 0)))
      (return true))))