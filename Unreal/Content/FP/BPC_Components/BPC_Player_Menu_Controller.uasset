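; Player menu controller component that shows 3D menu actors in front of its owner via an attached holder actor.
; SetMenu3D spawns the requested menu class into the holder and flags menu mode, while ClearMenus destroys attached menus.
; On resolution change, it resizes the holder background and menu using menu-mode FOV, distance and aspect ratio.
; Computed height limits clamp vertical scrolling; menu in/out transitions are empty stubs.
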(event Custom|Setup
  (Utilities|FlowControl|DoOnce false
    (:Completed
      (Utilities|FlowControl|Sequence
        (:then_0
          ;[1 1 1] Bind On FOV Change
          (bind _asbp_abstract_game_mode_master (Utilities|Casting|CastToBP_Abstract_GameMode_Master (Game|GetGameMode)))
          (Variables|Scene|SetTransition%20Props (Variables|/Game/FP/BluePrints/Global_BP/GM_GameModes/BP_Abstract_GameMode_Master.BP_Abstract_GameMode_Master_C|GetTransitionProps _asbp_abstract_game_mode_master)))
        (:then_1
          ;[1 1 1] Save Player ref
          (bind _asbp_player (Utilities|Casting|CastToBP_player (Game|Player|GetPlayerPawn 0)))
          (Variables|Actors|SetPlayer _asbp_player))
        (:then_2
          ;[1 1 1] Create Menu Holder Actor
          (bind _returnvalue (Game|SpawnActorfromClass "/Game/FP/BluePrints/Objects/Menu/BP_Actor_Menu3D_Holder.BP_Actor_Menu3D_Holder_C" (Math|Transform|MakeTransform "0, 0, 0") "Undefined" "MultiplyWithRoot" 0 (Variables|scene|GetDefault_x_Distance) 0))
          (bind _output_get (Variables|Actors|SetMenuHolder _returnvalue))
          (Transformation|AttachActorToActor _output_get (Components|GetOwner) "" "KeepRelative" "KeepRelative" "KeepRelative" true))
        (:then_3
          ;[1 1 1] Adapt to Viewport Resolution
          (bind _asbp_player_controller_master (Utilities|Casting|CastToBP_PlayerController_Master (Game|GetPlayerController 0)))
          (EventDispatchers|BindEventtoOnResolutionChange (Variables|/Game/FP/BluePrints/Global_BP/PC_PlayerController/BP_PlayerController_Master.BP_PlayerController_Master_C|GetBPC_PlayerController_ResulutionChange _asbp_player_controller_master) (delegate Custom|onResolutionChange)))))))

(event Custom|onResolutionChange
  (params (Resolution :type Vector%202D%20Structure) (Ratio_X:Y :type Float%20%28double-precision%29))
  ;[1 1 1] Adapt to Viewport Resolution
  (CallFunction|HolderUpdateResolution)
  (CallFunction|MenuUpdateResolution))

(event EventBeginPlay
  (CallFunction|Setup))

(event Custom|ClearMenus
  (Utilities|FlowControl|Sequence
    (:then_0
      (for _array_element (Actor|GetAttachedActors (Variables|Actors|GetMenuHolder) true false)
        (if (Utilities|ClassIsChildOf (Utilities|GetClass _array_element) "/Game/FP/GUI/3D_Menu/Master/BP_Actor_Menu3D.BP_Actor_Menu3D_C")
          (Actor|DestroyActor _array_element))))
    (:then_1
      (Variables|Props|Setmode_menu_ON false))))

(event Custom|MenuUpdateResolution
  (bind _menu3d (Variables|Actors|GetMenu3D))
  (Utilities|IsValid (Variables|Actors|GetMenu3D)
    (:Is%20Valid
      (bind _screenrelation (Class|BPIMenu3D|GetWidthScreenRelation(Message) _menu3d))
      (bind _defaultdimension (Default|GetDefaultDimension _menu3d))
      (Transformation|SetActorScale3D _menu3d (Math|Conversions|ToVector(Float) (/ (* _screenrelation (.X (CallFunction|ExpectedWidgetResolution (Variables|scene|GetDefault_x_Distance) (.menumode_fov (Variables|Scene|GetTransition%20Props))))) (.x _defaultdimension))))
      (CallFunction|SetMaxMinLocation))))

(event Custom|ResetLocation
  (bind _menu3d (Variables|Actors|GetMenu3D))
  (Transformation|AddActorLocalOffset _menu3d (Math|Vector|MakeVector 0.0 0.0 (- (Variables|Default|GetMenu3D_Z_Top_Position) (.z (.location (Transformation|GetRelativeTransform (Variables|/Script/Engine.Actor|GetRootComponent _menu3d)))))) false false))

(event Custom|setMaxMinLocation
  ;[1 1 1] Offset para que no esté en la parte superior de la pantalla.
  (Variables|Default|SetMenu3D_Z_Top_Position_margin (/ (Variables|scene|GetDefault_x_Distance) 5.0))
  (bind _dimension (Class|BPIMenu3D|GetCurrentDimension(Message) (Variables|Actors|GetMenu3D)))
  (bind _output_get (Variables|Default|SetMenu3D_Z_Top_Position (* (* (- (+ (.y _dimension) (Variables|Default|GetMenu3D_Z_Top_Position_margin)) (.Y (CallFunction|ExpectedWidgetResolution (Variables|scene|GetDefault_x_Distance) (.menumode_fov (Variables|Scene|GetTransition%20Props))))) 0.5) -1.0)))
  ;[1 1 1] Si el Menú es menor a la pantalla, el BOTTOM es igual al TOP.
  (if (< (* (- (+ (.y _dimension) (Variables|Default|GetMenu3D_Z_Top_Position_margin)) (.Y (CallFunction|ExpectedWidgetResolution (Variables|scene|GetDefault_x_Distance) (.menumode_fov (Variables|Scene|GetTransition%20Props))))) 0.5) 0.0)
    (Variables|Default|SetMenu3D_Z_Botton_Position _output_get)
    (else
      (Variables|Default|SetMenu3D_Z_Botton_Position (* (- (+ (.y _dimension) (Variables|Default|GetMenu3D_Z_Top_Position_margin)) (.Y (CallFunction|ExpectedWidgetResolution (Variables|scene|GetDefault_x_Distance) (.menumode_fov (Variables|Scene|GetTransition%20Props))))) 0.5)))))

(event Custom|onScroll
  (params (scroll_value :type Float%20%28double-precision%29))
  (bind _menu3d (Variables|Actors|GetMenu3D))
  (bind _menu3d_z_top_position (Variables|Default|GetMenu3D_Z_Top_Position))
  (bind _menu3d_z_botton_position (Variables|Default|GetMenu3D_Z_Botton_Position))
  (bind _rootcomponent (Variables|/Script/Engine.Actor|GetRootComponent _menu3d))
  (bind _relativelocation (Variables|/Script/Engine.SceneComponent|GetRelativeLocation _rootcomponent))
  (Transformation|SetRelativeLocation _rootcomponent (Math|Vector|MakeVector (.x _relativelocation) (.y _relativelocation) (Math|Float|Clamp(Float) (+ (.z _relativelocation) (* scroll_value (Variables|Props|Getscroll_speed))) (Math|Float|Min(Float) _menu3d_z_top_position _menu3d_z_botton_position) (Math|Float|Max(Float) _menu3d_z_top_position _menu3d_z_botton_position))) false false))

(event Custom|HolderUpdateResolution
  (bind _default_x_distance (Variables|scene|GetDefault_x_Distance))
  (bind _transition_props (Variables|Scene|GetTransition%20Props))
  (bind (_x _y) (CallFunction|ExpectedWidgetResolution _default_x_distance (.menumode_fov _transition_props)))
  (Class|WidgetComponent|SetDrawSize (Variables|/Game/FP/BluePrints/Objects/Menu/BP_Actor_Menu3D_Holder.BP_Actor_Menu3D_Holder_C|GetWidget_background (Variables|Actors|GetMenuHolder)) (Math|Vector2D|MakeVector2D _x _y)))

(fn SetMenu3D
  (params (Menu_3D_Class :type BP%20Actor%20Menu%203D%20Class%20Reference))
  (CallFunction|TransitionMenuOUT)
  (bind _menu_3d (CallFunction|InstanciateMenu Menu_3D_Class))
  (CallFunction|TransitionMenuIN)
  (Variables|Props|Setmode_menu_ON true)
  (return _menu_3d))

(fn TransitionMenuOUT
  (return false))

(fn TransitionMenuIN
  (return false))

(fn InstanciateMenu
  (params (Menu%203D%20Class :type BP%20Actor%20Menu%203D%20Class%20Reference))
  (Utilities|FlowControl|Sequence
    (:then_0
      (Variables|Actors|SetMenu3D_Old (Variables|Actors|GetMenu3D)))
    (:then_1
      (bind _returnvalue (Game|SpawnActorfromClass Menu%203D%20Class (Math|Transform|MakeTransform (Math|Vector|MakeVector (Variables|scene|GetDefault_x_Distance) 0.0 0.0)) "Undefined" "MultiplyWithRoot" 0 false 0.6 0))
      (bind _output_get (Variables|Actors|SetMenu3D _returnvalue)))
    (:then_2
      (Transformation|AttachActorToActor (Variables|Actors|GetMenu3D) (Variables|Actors|GetMenuHolder) "" "KeepRelative" "KeepRelative" "KeepRelative" true))
    (:then_3
      (CallFunction|MenuUpdateResolution)
      (CallFunction|ResetLocation)
      (return _output_get))))

(fn ExpectedWidgetResolution
  (params (distance :type Float%20%28double-precision%29) (FOV :type Float%20%28double-precision%29))
  (bind _returnvalue (Viewport|GetViewportSize))
  (bind _returnvalue_2 (!= FOV 0.0))
  (bind _returnvalue_3 (!= distance 0.0))
  (bind _default_x_distance (Variables|scene|GetDefault_x_Distance))
  (bind _transition_props (Variables|Scene|GetTransition%20Props))
  (bind _returnvalue_4 (Math|Float|SelectFloat FOV (.menumode_fov _transition_props) _returnvalue_2))
  (bind _returnvalue_5 (Math|Float|SelectFloat distance _default_x_distance _returnvalue_3))
  (bind _returnvalue_6 (/ _returnvalue_4 2.0))
  (bind _returnvalue_7 (Math|Trig|Tan(Degrees) _returnvalue_6))
  (bind _returnvalue_8 (* _returnvalue_7 1.2))
  (bind _returnvalue_9 (* _returnvalue_5 _returnvalue_8))
  (return (* (/ (.x _returnvalue) (.y _returnvalue)) _returnvalue_9) _returnvalue_9))