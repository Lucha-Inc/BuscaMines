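; BPO_Touch tracks one finger on mobile and turns it into player movement, look and selection input.
; Each move promotes the gesture from undefined to single or double swipe, pairing with the other touch through the controller's mobile input component.
; Single swipes pan XY, double swipes look and pinch along Z when finger motions oppose, with deltas ramped up over an initial time.
; Releasing without a swipe calls Select or Suspect, depending on hold time and finger.
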(event Custom|setCurrentData
  (params (current_ScreenPosition :type Vector%202D%20Structure) (current_Time :type Float%20%28double-precision%29))
  (bind _output_get (Variables|Current|Setcurrent_ScreenPosition current_ScreenPosition))
  (Variables|Current|Setcurrent_MovementVector (- _output_get (Variables|Last|Getlast_ScreenPosition)))
  (Variables|Current|Setcurrent_TimeDelay (- current_Time (Variables|Ini|GetIni_Time))))

(event Custom|setLastData
  (Variables|Last|Setlast_ScreenPosition (Variables|Current|Getcurrent_ScreenPosition))
  (Variables|Last|Setlast_MovementVector (Variables|Current|Getcurrent_MovementVector)))

(fn Moved
  (params (current_ScreenPosition :type Vector%202D%20Structure) (current_Time :type Float%20%28double-precision%29))
  (CallFunction|SetCurrentData current_ScreenPosition current_Time)
  (switch Utilities|FlowControl|Switch|SwitchonETouchIndex (Variables|Properties|GetTouchIndex)
    (:Touch1
      _)
    (:Touch2
      _))
  (CallFunction|EvaluateGesture)
  (CallFunction|SwipeMovements)
  (CallFunction|SetLastData))

(fn Release
  (params (new_ScreenPosition :type Vector%202D%20Structure) (current_Time :type Float%20%28double-precision%29))
  (switch Utilities|FlowControl|Switch|SwitchonETouchIndex (Variables|Properties|GetTouchIndex)
    (:Touch1
      (if (Utilities|Enum|Equal(Enum) (Variables|Properties|GetGesture) "NewEnumerator5")
        (if (> (- current_Time (Variables|Ini|GetIni_Time)) (Variables|Config|GetShortTouchMaxTime))
          (Default|Suspect (Variables|/Game/FP/BluePrints/Controller/BP_PlayerController_Master.BP_PlayerController_Master_C|GetBPC_PlayerInputs_Mobile (Variables|Properties|GetPlayerController)) new_ScreenPosition)
          (else
            (Default|Select (Variables|/Game/FP/BluePrints/Controller/BP_PlayerController_Master.BP_PlayerController_Master_C|GetBPC_PlayerInputs_Mobile (Variables|Properties|GetPlayerController)) new_ScreenPosition)))))
    (:Touch2
      (if (and (.valid (CallFunction|GetTouchbyIndex "Touch1")) (Utilities|Enum|Equal(Enum) (Variables|Properties|GetGesture) "NewEnumerator5"))
        (Default|Suspect (Variables|/Game/FP/BluePrints/Controller/BP_PlayerController_Master.BP_PlayerController_Master_C|GetBPC_PlayerInputs_Mobile (Variables|Properties|GetPlayerController)) new_ScreenPosition)))))

(fn ValidateSwipeMinDistance
  (params (current_ScreenPosition :type Vector%202D%20Structure))
  (return (> (Math|Vector2D|Vector2DLength (- current_ScreenPosition (Variables|Ini|GetIni_ScreenPosition))) (Variables|Config|GetSwipeMinDistance))))

(fn GetTouchbyIndex
  (params (Index :type ETouchIndex%20Enum :default "Touch1"))
  (bind _playercontroller (Variables|Properties|GetPlayerController))
  (bind _bpc_playerinputs_mobile (Variables|/Game/FP/BluePrints/Controller/BP_PlayerController_Master.BP_PlayerController_Master_C|GetBPC_PlayerInputs_Mobile _playercontroller))
  (bind _touchlist (Default|GetTouchList _bpc_playerinputs_mobile))
  (bind (_value _returnvalue) (Utilities|Map|Find _touchlist Index))
  (return _value _returnvalue))

(fn EvaluateGesture
  (bind (_touch _valid) (CallFunction|GetTouchbyIndex "Touch2"))
  (bind (_touch_2 _valid_2) (CallFunction|GetTouchbyIndex "Touch1"))
  (switch Utilities|FlowControl|Switch|SwitchonEnum_Touch_Gesture (Variables|Properties|GetGesture) :!label _label
    (:NewEnumerator5
      (if (CallFunction|ValidateSwipeMinDistance (Variables|Current|Getcurrent_ScreenPosition))
        (Variables|Properties|SetGesture "NewEnumerator2")
        (goto _label)))
    (:NewEnumerator2
      (switch Utilities|FlowControl|Switch|SwitchonETouchIndex (Variables|Properties|GetTouchIndex)
        (:Touch1
          (if _valid
            (Variables|Properties|SetGesture "NewEnumerator3")
            (bind _output_get (Variables|Properties|SetpairTouch _touch))
            (Variables|BPO_Touch_C|SetGesture _output_get "NewEnumerator3")))
        (:Touch2
          (if _valid_2
            (Variables|Properties|SetGesture "NewEnumerator3")
            (bind _output_get_2 (Variables|Properties|SetpairTouch _touch_2))
            (Variables|BPO_Touch_C|SetGesture _output_get_2 "NewEnumerator3")))))
    (:NewEnumerator3
      (switch Utilities|FlowControl|Switch|SwitchonETouchIndex (Variables|Properties|GetTouchIndex)
        (:Touch1
          (if (not (.valid (CallFunction|GetTouchbyIndex "Touch2")))
            (Variables|Properties|SetGesture "NewEnumerator2")
            (Variables|Properties|SetpairTouch 0)))
        (:Touch2
          (if (not (.valid (CallFunction|GetTouchbyIndex "Touch1")))
            (Variables|Properties|SetGesture "NewEnumerator2")
            (Variables|Properties|SetpairTouch 0)))))))

(fn SwipeMovements
  (bind _swipevector (CallFunction|GetSwipeVector))
  (bind _swipevector_2 (CallFunction|GetSwipeVector))
  (switch Utilities|FlowControl|Switch|SwitchonEnum_Touch_Gesture (Variables|Properties|GetGesture) :!label _label
    (:NewEnumerator2
      ;[0.15 0.15 0.15 0.5] Comment
      (Default|PlayerMoveXY (Variables|Properties|GetPlayerController) (* (Math|Vector2D|MakeVector2D (.y _swipevector_2) (* (.x _swipevector_2) -1.0)) (Variables|Default|Getsensibility_move_XY_default))))
    (:NewEnumerator3
      (Utilities|IsValid (Variables|Properties|GetpairTouch)
        (:Is%20Valid
          (Utilities|FlowControl|Sequence
            (:then_0
              ;[0.15 0.15 0.15 0.5] DualSwipe
              (Default|PlayerLook (Variables|Properties|GetPlayerController) (* (Math|Vector2D|MakeVector2D (.x _swipevector) (* (.y _swipevector) -1.0)) (Variables|Default|Getsensibility_look_default))))
            (:then_1
              ;[0.15 0.15 0.15 0.5] Pinch
              (if (<= (Math|Vector2D|DotProduct(2D) (Variables|Current|Getcurrent_MovementVector) (Variables|BPO_Touch_C|Getlast_MovementVector (Variables|Properties|GetpairTouch))) 0.0)
                (Default|PlayerMoveZ (Variables|Properties|GetPlayerController) (* (- (Math|Vector2D|Vector2DLength (- (Variables|BPO_Touch_C|Getlast_ScreenPosition (Variables|Properties|GetpairTouch)) (Variables|Last|Getlast_ScreenPosition))) (Math|Vector2D|Vector2DLength (- (Variables|BPO_Touch_C|Getlast_ScreenPosition (Variables|Properties|GetpairTouch)) (Variables|Current|Getcurrent_ScreenPosition)))) (Variables|Default|Getsensibility_move_Z_default)))))))
        (:Is%20Not%20Valid
          (Variables|Properties|SetGesture "NewEnumerator2")
          (goto _label))))))

(fn GetSwipeVector
  (bind _initialgradualtime (Variables|Config|GetInitialGradualTime))
  (return (* (- (Variables|Current|Getcurrent_ScreenPosition) (Variables|Last|Getlast_ScreenPosition)) (/ (Math|Float|Min(Float) (Variables|Current|Getcurrent_TimeDelay) _initialgradualtime) _initialgradualtime) 0.2)))