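; BPO_Ranking is a Blueprint wrapper around the GISSRanking system for reading and writing one leaderboard.
; It builds an uppercase ranking key from its Mode, Difficulty, Type and Order enums, so each combination addresses a separate table.
; Through that key it fetches the top 10, reports new entries with a default user name when none is given, and renames the entry at a given position.
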(fn GetTop10
  (return (Class|GameInstanceSubsystemRanking|GetRankTop10 (Variables|Default|GetGISS_Ranking) (CallFunction|GetRankName))))

(fn ReportEntry
  (params (Value :type Float%20%28double-precision%29) (Name :type String))
  (bind _returnvalue (Class|GameInstanceSubsystemRanking|ReportRankEntry (Variables|Default|GetGISS_Ranking) (CallFunction|GetRankName) (Utilities|String|SelectString (Variables|Default|GetDefaultUserName) Name (Utilities|Array|IsEmpty Name)) Value))
  (return _returnvalue))

(fn UpdatelastRecordName
  (params (Position :type Integer) (NewName :type String))
  (bind _returnvalue (Class|GameInstanceSubsystemRanking|UpdateRankName (Variables|Default|GetGISS_Ranking) (CallFunction|GetRankName) Position NewName))
  (return _returnvalue))

(fn GetRankName
  (return (Class|KismetStringLibrary|ToUpper (Utilities|String|Append "RANKING_" (Utilities|String|EnumtoString (Variables|Default|GetMode)) "_" (Utilities|String|EnumtoString (Variables|Default|GetDifficulty)) "_" (Utilities|String|EnumtoString (Variables|Default|GetType)) "_" (Utilities|String|EnumtoString (Variables|Default|GetOrder))))))