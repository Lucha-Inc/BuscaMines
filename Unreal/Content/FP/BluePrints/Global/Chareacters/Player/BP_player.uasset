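; Player Blueprint that lets mouse clicks and first-finger touches press and release widgets through a WidgetInteraction component.
; Screen positions are deprojected into a short visibility line trace, drawn in debug mode, and fed to the component as a custom hit result.
; Pointer key is Touch1 on mobile, otherwise left mouse button.
; Mouse presses shortly after a touch are ignored to avoid double input on touchscreen notebooks.
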(event EventBeginPlay)

(event Collision|EventActorBeginOverlap
  (params (OtherActor :type Actor%20Object%20Reference)))

(event EventTick
  (params (DeltaSeconds :type Float%20%28single-precision%29)))

(event Input|MouseEvents|LeftMouseButton
  (params (Key :type Key%20Structure :default "None"))
  (bind _returnvalue (Game|GetPlayerController 0))
  (bind (_worldlocation _worlddirection) (Game|Player|ConvertMouseLocationToWorldSpace _returnvalue))
  (:Pressed
    (if (> (- (Utilities|Time|GetGameTimeinSeconds) (Variables|Default|GetlastTouchSeconds)) 1.0)
      (CallFunction|PressWidgetInteraction _worldlocation (+ _worldlocation (* _worlddirection 1e+03)))))
  (:Released
    (CallFunction|ReleaseWidgetInteraction)))

(event Input|TouchEvents|InputTouch
  (params (Location :type Vector) (FingerIndex :type ETouchIndex%20Enum))
  (bind _returnvalue (Game|GetPlayerController 0))
  (bind _returnvalue_2 (Math|Conversions|ToVector2D(Vector) Location))
  (bind (_worldposition _worlddirection) (Class|GameplayStatics|DeprojectScreentoWorld _returnvalue _returnvalue_2))
  (:Pressed
    (switch Utilities|FlowControl|Switch|SwitchonETouchIndex FingerIndex
      (:Touch1
        (Variables|Default|SetlastTouchSeconds (Utilities|Time|GetGameTimeinSeconds))
        (CallFunction|PressWidgetInteraction _worldposition (+ _worldposition (* _worlddirection 1e+03))))))
  (:Released
    (switch Utilities|FlowControl|Switch|SwitchonETouchIndex FingerIndex
      (:Touch1
        (CallFunction|ReleaseWidgetInteraction)))))

(fn ConstructionScript)

(fn PressWidgetInteraction
  (params (StartTrace :type Vector) (EndTrace :type Vector))
  (bind _widgetinteraction (Variables|Default|GetWidgetInteraction))
  (bind _debugmode (CallFunction|GetDebugMode self))
  (bind _outhit (Collision|LineTraceByChannel StartTrace EndTrace "TraceTypeQuery1" true 0 (select _debugmode "ForDuration" "None") true "(R=1.000000,G=0.811949,B=0.000000,A=1.000000)"))
  (Class|WidgetInteractionComponent|SetCustomHitResult (Variables|Default|GetWidgetInteraction) _outhit)
  (if (CallFunction|IsMobile)
    (Class|WidgetInteractionComponent|PressPointerKey _widgetinteraction "Touch1")
    (else
      (Class|WidgetInteractionComponent|PressPointerKey _widgetinteraction "LeftMouseButton"))))

(fn ReleaseWidgetInteraction
  (bind _widgetinteraction (Variables|Default|GetWidgetInteraction))
  (if (CallFunction|IsMobile)
    (Class|WidgetInteractionComponent|ReleasePointerKey _widgetinteraction "Touch1")
    (else
      (Class|WidgetInteractionComponent|ReleasePointerKey _widgetinteraction "LeftMouseButton"))))