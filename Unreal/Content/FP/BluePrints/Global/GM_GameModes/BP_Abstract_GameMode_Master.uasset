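; Abstract master game mode for board-based levels, driving status from setup and presentation through camera intro, timed play and game end.
; Board completion stops the timer, reports the score to a ranking object and opens a ranking, win or lose 3D menu.
; Menus come from spawned creator actors kept in a back-navigation list.
; Switching between menu and game swaps Enhanced Input contexts and music, with a reversible timeline animating camera and menu scale.
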(event Custom|BoardStatsUpdated
  (params (StatsObject :type BP%20Stats%20Master%20Object%20Reference)))

(event Custom|BoardFinished
  (params (Won :type Boolean))
  (CallFunction|LevelCompleted Won))

(event EventBeginPlay
  (bind _self self)
  (Utilities|FlowControl|Sequence
    (:then_0
      (bind (_gameinstance _thememanager _soundmanager_app _player _gamemode_master _playercontroller_master) (CallFunction|GetCustomClasses _self))
      (Variables|Managers|SetPlayer%20Controller%20Master _playercontroller_master)
      (Variables|Managers|SetPlayer _player))
    (:then_1
      (bind _hud_classic (CallFunction|GetCustomClassic _self))
      (Variables|Managers|SetHUD _hud_classic))
    (:then_3
      (bind _gameinstance_2 (CallFunction|GetCustomClasses _self))
      (bind _soundmanager (Default|GetSoundClassManager _gameinstance_2))
      (Default|SetMute _soundmanager "NewEnumerator4" true))))

(event EventOnKeyPressed
  (params (char :type String)))

(event EventSetup
  (params (Level :type BPI%20Level%20Master%20Interface) (Board :type BP%20Board%20Master%20Object%20Reference) (Sound%20Manager%20Level :type BP%20Sound%20Class%20Manager%20Level%20Object%20Reference) (PostProcessVolume :type Post%20Process%20Volume%20Object%20Reference))
  (Utilities|FlowControl|Sequence
    (:then_0
      (Status|SetStatus "NewEnumerator0"))
    (:then_1
      (Variables|Level|SetLevel Level)
      (Variables|Level|SetPostProcessVolume PostProcessVolume))
    (:then_2
      (Variables|Managers|SetSound%20Manager%20Level Sound%20Manager%20Level))
    (:then_3
      (bind _output_get (Variables|Board|SetBoard_Master Board))
      (EventDispatchers|BindEventtoBoardStatsUpdated _output_get (delegate Custom|BoardStatsUpdated))
      (EventDispatchers|BindEventtoBoardFinished _output_get (delegate Custom|BoardFinished)))
    (:then_5
      (bind (_gameinstance _thememanager _soundmanager_app) (CallFunction|GetCustomClasses self))
      (Variables|Managers|SetGame%20Instance _gameinstance)
      (Variables|Managers|SetSound%20Manager%20App _soundmanager_app))
    (:then_6
      (Default|ShowDebugModeUW (Variables|Managers|GetHUD)))))

(event Custom|setPauseOn
  (CallFunction|SetPauseto true))

(event Custom|setPauseOff
  (CallFunction|SetPauseto true))

(event Custom|setPauseTo
  (params (pause :type Boolean))
  (if (!= pause (Variables|State|Getpaused))
    (bind _output_get (Variables|State|Setpaused pause))
    (Default|SetPauseto (Variables|Default|GetTimer) _output_get)
    (Default|CallPauseChanged _output_get)))

(event Custom|setPauseToogle
  (CallFunction|SetPauseto (not (Variables|State|Getpaused))))

(event Custom|_Menu%20Transition
  (params (toMenuMode :type Boolean) (Menu%203D :type BP%20Actor%20Menu%203D%20Object%20Reference))
  (bind _returnvalue (Game|GetPlayerCharacter 0))
  (bind _returnvalue_2 (Game|GetPlayerCharacter 0))
  (bind _returnvalue_3 (Transformation|GetActorTransform _returnvalue))
  (bind _returnvalue_4 (Transformation|GetActorTransform _returnvalue_2))
  (if toMenuMode
    (Variables|Menus|SetTransitionProps (Utilities|Struct|MakeStruct_Transition_Menu_Game_Mode (.gamemode_fov (Variables|Menus|GetTransitionProps)) (.z (.location _returnvalue_4)) (.pitch (.rotation _returnvalue_4)) (.menumode_fov (Variables|Menus|GetTransitionProps)) (Math|Float|Max(Float) (.menumode_z_heigh (Variables|Menus|GetTransitionProps)) (.z (.location _returnvalue_4))) (.menumode_y_angle (Variables|Menus|GetTransitionProps)) (Transformation|GetActorScale3D Menu%203D) (.blur (Variables|Menus|GetTransitionProps)) (.alpha (Variables|Menus|GetTransitionProps)) (.transitiontime (Variables|Menus|GetTransitionProps))))
    (Components|Timeline|SetPlayRate (Variables|Default|GetTransition_MenuMode_Timeline) (/ 1.0 (.transitiontime (Variables|Menus|GetTransitionProps))))
    (bind _alpha_auto (Timeline|Transition_MenuMode_Timeline Play)
      (:Update
        (Utilities|FlowControl|Sequence
          (:then_0
            ;[0.15 0.15 0.15 0.5] Set FOV
            (Camera|SetFieldOfView (Variables|/Game/FP/BluePrints/Global/Chareacters/Player/BP_player.BP_player_C|GetCamera (Variables|Managers|GetPlayer)) (Math|Float|Lerp (.gamemode_fov (Variables|Menus|GetTransitionProps)) (.menumode_fov (Variables|Menus|GetTransitionProps)) _alpha_auto))
            (Default|CallChangingFOV (Math|Float|Lerp (.gamemode_fov (Variables|Menus|GetTransitionProps)) (.menumode_fov (Variables|Menus|GetTransitionProps)) _alpha_auto)))
          (:then_1
            ;[0.15 0.15 0.15 0.5] Set Player Location and Rotation
            (if (Utilities|Enum|Equal(Enum) (Variables|State|Getstatus) "NewEnumerator4")
              (Transformation|SetActorLocationAndRotation _returnvalue (Math|Vector|MakeVector (.x (.location _returnvalue_3)) (.y (.location _returnvalue_3)) (Math|Float|Lerp (.gamemode_z_heigh (Variables|Menus|GetTransitionProps)) (.menumode_z_heigh (Variables|Menus|GetTransitionProps)) _alpha_auto)) (Math|Rotator|MakeRotator (.roll (.rotation _returnvalue_3)) (Math|Float|Lerp (.gamemode_y_angle (Variables|Menus|GetTransitionProps)) (.menumode_y_angle (Variables|Menus|GetTransitionProps)) _alpha_auto) (.yaw (.rotation _returnvalue_3))))))
          (:then_2
            ;[0.15 0.15 0.15 0.5] Set Menu Scale
            (Utilities|IsValid Menu%203D
              (:Is%20Valid
                (Transformation|SetActorScale3D Menu%203D (Math|Vector|Lerp(Vector) "0, 0, 0" (.menumode_finalscale (Variables|Menus|GetTransitionProps)) _alpha_auto))))))))
    (else
      (Components|Timeline|SetPlayRate (Variables|Default|GetTransition_MenuMode_Timeline) (/ 1.0 (.transitiontime (Variables|Menus|GetTransitionProps))))
      (Timeline|Transition_MenuMode_Timeline Reverse))))

(event Custom|SetGame
  (Utilities|FlowControl|Sequence
    (:then_0
      (Variables|/Script/Engine.PostProcessVolume|SetbEnabled (Variables|Level|GetPostProcessVolume) true))
    (:then_1
      ;[1 1 1] Si no viene de un modo MENU, hace una transición Visual
      (if (Variables|State|GetmenuMode)
        (bind _output_get (Variables|State|SetmenuMode false))
        (CallFunction|MenuTransition _output_get)
        (CallFunction|RemoveMenuInputs)
        (else
          (Default|PlayLevelGameMusicBg (Variables|Managers|GetSound%20Manager%20Level)))))
    (:then_2
      (Default|ClearMenus3D (Variables|Managers|GetPlayer%20Controller%20Master))
      (Utilities|Array|Clear (Variables|Menus|GetMenuList)))
    (:then_3
      (switch Utilities|FlowControl|Switch|SwitchonEGameMode_Status (Variables|State|Getstatus)
        (:NewEnumerator4
          (Default|ShowGaming (Variables|Managers|GetHUD))
          (CallFunction|AddGameInputs))))))

(event Custom|_Add_MenuInputs
  (Inputs|AddRemoveMappingContext "/Game/FP/Inputs/Others/Menu3D/menu_inputs.menu_inputs" true)
  (Variables|/Script/Engine.PlayerController|SetbShowMouseCursor (Variables|Managers|GetPlayer%20Controller%20Master) true))

(event Custom|_Remove_MenuInputs
  (Inputs|AddRemoveMappingContext "/Game/FP/Inputs/Others/Menu3D/menu_inputs.menu_inputs" false)
  (Variables|/Script/Engine.PlayerController|SetbShowMouseCursor (Variables|Managers|GetPlayer%20Controller%20Master) false))

(event Custom|_Add_GameInputs
  (bind _player_controller_master (Variables|Managers|GetPlayer%20Controller%20Master))
  (Inputs|AddRemoveMappingContext "/Game/FP/Inputs/Others/Board/board_inputs.board_inputs" true)
  (Inputs|AddRemoveMappingContext "/Game/FP/Inputs/Others/Player/player_inputs.player_inputs" true)
  ;[0.15 0.15 0.15 0.5] To see the Mouse in the Game
  (Variables|/Script/Engine.PlayerController|SetbShowMouseCursor _player_controller_master true)
  (Variables|/Script/Engine.PlayerController|SetbEnableClickEvents _player_controller_master true)
  (Variables|/Script/Engine.PlayerController|SetbEnableMouseOverEvents _player_controller_master true)
  (Default|SetGameInputsEnable (Variables|Managers|GetPlayer%20Controller%20Master) true))

(event Custom|Remove_GameInputs
  (bind _player_controller_master (Variables|Managers|GetPlayer%20Controller%20Master))
  (Inputs|AddRemoveMappingContext "/Game/FP/Inputs/Others/Board/board_inputs.board_inputs" false)
  (Inputs|AddRemoveMappingContext "/Game/FP/Inputs/Others/Player/player_inputs.player_inputs" false)
  ;[0.15 0.15 0.15 0.5] To see the Mouse in the Game
  (Variables|/Script/Engine.PlayerController|SetbShowMouseCursor _player_controller_master false)
  (Variables|/Script/Engine.PlayerController|SetbEnableClickEvents _player_controller_master false)
  (Variables|/Script/Engine.PlayerController|SetbEnableMouseOverEvents _player_controller_master false)
  (Default|SetGameInputsEnable (Variables|Managers|GetPlayer%20Controller%20Master) false))

(event Custom|LevelCompleted
  (params (won :type Boolean))
  (bind _hud (Variables|Managers|GetHUD))
  (bind _hud_2 (Variables|Managers|GetHUD))
  (Status|SetStatus "NewEnumerator6")
  (Default|EndTimer (Variables|Default|GetTimer))
  (Inputs|AddRemoveMappingContext "/Game/FP/Inputs/Others/Pause/pause_inputs.pause_inputs" false)
  (if won
    (bind _statobject (Default|GetStats (Variables|Board|GetBoard_Master)))
    (bind _score (Default|GetScore _statobject))
    (bind _ranking (Default|GetRankingObject self))
    (bind _pos (Default|ReportEntry _ranking (Math|Conversions|ToFloat(Integer) _score) "Crack"))
    (if (> _pos 0)
      (Default|ClearAllUW _hud)
      (Default|PlayLevelFinishWin (Variables|Managers|GetSound%20Manager%20Level))
      (bind _returnvalue (Game|SpawnActorfromClass "/Game/FP/BluePrints/Objects/Menu/MenuCreators/BP_MenuCreator_Won_Ranking.BP_MenuCreator_Won_Ranking_C" (Math|Transform|MakeTransform "0, 0, 0") "Undefined" "MultiplyWithRoot" 0 _ranking _pos 0 0))
      (CallFunction|GotoMenubyCreator _returnvalue)
      (else
        (Default|ClearAllUW _hud)
        (Default|PlayLevelFinishWin (Variables|Managers|GetSound%20Manager%20Level))
        (CallFunction|SetMenubyClass "/Game/FP/GUI/3D_Menu/Instance/BP_Menu_Won.BP_Menu_Won_C")))
    (else
      ;[0.15 0.15 0.15 0.5] BORRAR
      (bind _statobject_2 (Default|GetStats (Variables|Board|GetBoard_Master)))
      (bind _score_2 (Default|GetScore _statobject_2))
      (bind _ranking_2 (Default|GetRankingObject self))
      (bind _pos_2 (Default|ReportEntry _ranking_2 (Math|Conversions|ToFloat(Integer) _score_2) "Crack"))
      (if (> _pos_2 0)
        (Default|ClearAllUW _hud_2)
        (Default|PlayLevelFinishWin (Variables|Managers|GetSound%20Manager%20Level))
        (bind _returnvalue_2 (Game|SpawnActorfromClass "/Game/FP/BluePrints/Objects/Menu/MenuCreators/BP_MenuCreator_Won_Ranking.BP_MenuCreator_Won_Ranking_C" (Math|Transform|MakeTransform "0, 0, 0") "Undefined" "MultiplyWithRoot" 0 _ranking_2 _pos_2 0 0))
        (CallFunction|GotoMenubyCreator _returnvalue_2)
        (else
          ;[0.15 0.15 0.15 0.5] no borrar
          (Default|ClearAllUW _hud_2)
          (Default|PlayLevelFinishLose (Variables|Managers|GetSound%20Manager%20Level))
          (CallFunction|SetMenubyClass "/Game/FP/GUI/3D_Menu/Instance/BP_Menu_Lose.BP_Menu_Lose_C"))))))

(event EventOnLevelReady
  ;[1 1 1] Show Presentation Menu
  (Utilities|FlowControl|Sequence
    (:then_0
      (Status|SetStatus "NewEnumerator1"))
    (:then_1
      (Default|PlayLevelIntroMusicBg (Variables|Managers|GetSound%20Manager%20Level))
      (bind _new_menu_3d (CallFunction|SetMenubyClass "/Game/FP/GUI/3D_Menu/Instance/BP_Menu_Presentation.BP_Menu_Presentation_C"))
      (bind _difficultyname (Default|GetDifficultyName (Variables|Board|GetDifficulty)))
      (Default|SetTitle _new_menu_3d _difficultyname)
      (Default|ShowDebugModeUW (Variables|Managers|GetHUD)))))

(event EventStartIntro
  (bind _sound_manager_level (Variables|Managers|GetSound%20Manager%20Level))
  (Status|SetStatus "NewEnumerator2")
  (Default|StopLevelIntroMusicBg _sound_manager_level)
  (Default|PlayLevelGameMusicBg _sound_manager_level)
  (CallFunction|SetGame)
  ;[1 1 1] Intro Movemente of Camera
  (bind _playermovement (CallFunction|GetCustomPlayer self))
  (Default|PlayMovement _playermovement (Default|GetStartPosition (Variables|Board|GetBoard_Master)) 6.0)
  (EventDispatchers|BindEventtoMovementFinished _playermovement (delegate EventOnIntroReady)))

(event EventOnIntroReady
  (bind _board_master (Variables|Board|GetBoard_Master))
  (bind _bounds (Default|GetBoardMovementsBounds _board_master))
  (Status|SetStatus "NewEnumerator4")
  (bind (_gameinstance _thememanager _soundmanager_app _player _gamemode_master _playercontroller_master) (CallFunction|GetCustomClasses self))
  (Utilities|FlowControl|Sequence
    (:then_0
      (bind _soundmanager (Default|GetSoundClassManager _gameinstance))
      (Default|SetMute _soundmanager "NewEnumerator4" false))
    (:then_1
      (bind _debugmode (CallFunction|GetDebugMode self))
      (Default|SetPlayerMovementBounds _playercontroller_master (Utilities|Struct|MakePlayerMovementBoundsDefinition (not _debugmode) (.bounds_origin _bounds) (+ (.bounds_extents _bounds) "1000.000000,1000.000000,1500.000000") "500.000000,500.000000,500.000000" (.normal_vector_x _bounds) (.normal_vector_y _bounds))))
    (:then_2
      (Default|StartTimer (Variables|Default|GetTimer))
      (CallFunction|SetGame)
      (Inputs|AddRemoveMappingContext "/Game/FP/Inputs/Others/Pause/pause_inputs.pause_inputs" true))
    (:then_3
      (Default|BoardStart (Variables|Board|GetBoard_Master)))))

(fn ConstructionScript)

(fn AddRemoveMappingContext
  (params (Input%20Mapping%20Context :type Input%20Mapping%20Context%20Object%20Reference) (Add%20Input :type Boolean))
  (if Add%20Input
    (Inputs|AddMappingContext Input%20Mapping%20Context)
    (else
      (Inputs|RemoveMappingContext Input%20Mapping%20Context))))

(fn IsPaused
  (return (Variables|State|Getpaused)))

(fn SetStatus
  (params (NewStatus :type EGameMode_Status%20Enum :default "NewEnumerator7"))
  (bind _output_get (LocalVariables|SetNewLocalVar (Variables|State|Getstatus)))
  (bind _output_get_2 (Variables|State|Setstatus NewStatus))
  (Default|CallOnGameStatusChange _output_get_2 _output_get)
  (switch Utilities|FlowControl|Switch|SwitchonEGameMode_Status _output_get_2
    (:NewEnumerator4
      (Utilities|FlowControl|DoOnce false
        (:Completed
          (Default|CallOnGameStart))))
    (:NewEnumerator6
      (Utilities|FlowControl|DoOnce false
        (:Completed
          (Default|CallOnGameEnd))))))

(fn GetStatus
  (return (Variables|State|Getstatus)))

(fn AddMappingContext
  (params (Mapping%20Context :type Input%20Mapping%20Context%20Object%20Reference))
  (Input|AddMappingContext (PlayerController|LocalPlayerSubsystems|GetEnhancedInputLocalPlayerSubsystem (Game|GetPlayerController 0)) Mapping%20Context 0 "(bIgnoreAllPressedKeysUntilRelease=True,bForceImmediately=False,bNotifyUserSettings=False)"))

(fn RemoveMappingContext
  (params (MappingContext :type Input%20Mapping%20Context%20Object%20Reference))
  (Input|RemoveMappingContext (PlayerController|LocalPlayerSubsystems|GetEnhancedInputLocalPlayerSubsystem (Game|GetPlayerController 0)) MappingContext "(bIgnoreAllPressedKeysUntilRelease=True,bForceImmediately=False,bNotifyUserSettings=False)"))

(fn SetMenubyClass
  (params (Menu_3D_Class :type BP%20Actor%20Menu%203D%20Class%20Reference))
  (bind _menu3d_creator (CallFunction|GetMenuCreatorbyMenu3DClass Menu_3D_Class))
  (bind _new_menu_3d (CallFunction|SetMenu _menu3d_creator))
  (return _new_menu_3d))

(fn SetMenu
  (params (MenuCreator :type BPI%20Menu%203D%20Creator%20Interface))
  (Utilities|FlowControl|Sequence
    (:then_0
      (Default|ClearMenus3D (Variables|Managers|GetPlayer%20Controller%20Master))
      (Utilities|Array|Add (Variables|Menus|GetMenuList) MenuCreator)
      (bind _menu_3d (Default|ShowMenu3DbyCreator (Variables|Managers|GetPlayer%20Controller%20Master) MenuCreator))
      (LocalVariables|SetNewMenu3D _menu_3d))
    (:then_1
      (if (not (Variables|State|GetmenuMode))
        (bind _output_get (Variables|State|SetmenuMode true))
        (CallFunction|MenuTransition _output_get (LocalVariables|GetNewMenu3D))
        (CallFunction|RemoveGameInputs)
        (CallFunction|AddMenuInputs)
        (Variables|/Script/Engine.PlayerController|SetbEnableClickEvents (Game|GetPlayerController 0) true)
        (switch Utilities|FlowControl|Switch|SwitchonEGameMode_Status (Variables|State|Getstatus)
          (:NewEnumerator4
            (Default|StopLevelGameMusicBg (Variables|Managers|GetSound%20Manager%20Level))))))
    (:then_2
      (Variables|/Script/Engine.PostProcessVolume|SetbEnabled (Variables|Level|GetPostProcessVolume) false))
    (:then_3
      (return (LocalVariables|GetNewMenu3D)))))

(fn GetMenuCreatorbyMenu3DClass
  (params (Menu3D_Class :type BP%20Actor%20Menu%203D%20Class%20Reference))
  (bind _returnvalue (Game|SpawnActorfromClass "/Game/FP/BluePrints/Objects/Menu/MenuCreators/BP_MenuCreator_Generic.BP_MenuCreator_Generic_C" (Math|Transform|MakeTransform "0, 0, 0") "Undefined" "MultiplyWithRoot" 0 Menu3D_Class 0))
  (return _returnvalue))

(fn GoBacktoLastMenu
  (bind _menulist (Variables|Menus|GetMenuList))
  (bind _menulist_2 (Variables|Menus|GetMenuList))
  (if (CallFunction|LastMenuIsValid)
    (Utilities|Array|RemoveIndex _menulist_2 (- (Utilities|Array|Length _menulist_2) 1))
    (bind _menu3d (CallFunction|GotoMenubyCreator (Utilities|Array|Get(acopy) _menulist (- (Utilities|Array|Length _menulist) 1))))
    (return _menu3d true)
    (else
      (return 0 false))))

(fn LastMenuIsValid
  (return (>= (Utilities|Array|Length (Variables|Menus|GetMenuList)) 2)))

(fn GetRankingObject)

(fn GotoMenubyClass
  (params (menu3DClass :type BP%20Actor%20Menu%203D%20Class%20Reference))
  (bind _menu3d_creator (CallFunction|GetMenuCreatorbyMenu3DClass menu3DClass))
  (bind _menu3d (CallFunction|GotoMenubyCreator _menu3d_creator))
  (return _menu3d))

(fn GotoMenubyCreator
  (params (Menu3D_Creator :type BPI%20Menu%203D%20Creator%20Interface))
  (bind _new_menu_3d (CallFunction|SetMenu Menu3D_Creator))
  (switch Utilities|FlowControl|Switch|SwitchonEGameMode_Status (Variables|State|Getstatus)
    (:NewEnumerator7
      _)
    (:NewEnumerator0
      _)
    (:NewEnumerator1
      _)
    (:NewEnumerator2
      _)
    (:NewEnumerator4
      (if (Variables|State|Getpaused)
        _
        (else
          (CallFunction|SetPauseon)
          (Default|ShowPause (Variables|Managers|GetHUD)))))
    (:NewEnumerator6
      _))
  (return _new_menu_3d))

(fn ReportRankEntry
  (params (RankValue :type Float%20%28double-precision%29) (RankUser :type String))
  (return 0))