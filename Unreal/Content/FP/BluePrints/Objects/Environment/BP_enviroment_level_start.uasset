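; BP_enviroment_level_start is an environment object that marks where the player starts in a level.
; Two getters, one for the initial position and one for start relocation, both return the world transform of its Camera component.
; On BeginPlay, it reads debug mode and shows EnvironmentBox only when that mode is on, setting both visibility and hidden-in-game.
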(event EventBeginPlay
  (bind _environmentbox (Variables|Default|GetEnvironmentBox))
  (bind _debugmode (CallFunction|GetDebugMode self))
  (Rendering|SetVisibility _environmentbox _debugmode false)
  (Development|SetHiddeninGame _environmentbox (not _debugmode) false))

(event EventTick
  (params (DeltaSeconds :type Float%20%28single-precision%29)))

(fn ConstructionScript)

(fn GetPlayerInitialPosition
  (return (Transformation|GetWorldTransform (Variables|Default|GetCamera))))

(fn GetPlayerStartRelocation
  (return (Transformation|GetWorldTransform (Variables|Default|GetCamera))))