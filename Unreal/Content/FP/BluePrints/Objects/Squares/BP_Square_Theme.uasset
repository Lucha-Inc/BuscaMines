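; BP_Square_Theme is a square object that varies the look of its Square mesh through randomized orientation.
; The construction script adds random quarter-turn rotations on all three axes.
; SetupTheme assigns the SquareMeshBORRAR mesh and, if SquareTheme allows XYZ rotation, sets a new random right-angle rotation, never 270 degrees.
; A separate event, not called here, adds slight random yaw noise.
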(event EventBeginPlay
  (|CallParentFunction) ; This node is disabled and will not be called.\nDrag off pins to build functionality.
)

(event Collision|EventActorBeginOverlap
  (params (OtherActor :type Actor%20Object%20Reference))
  (|CallParentFunction OtherActor) ; This node is disabled and will not be called.\nDrag off pins to build functionality.
)

(event EventTick
  (params (DeltaSeconds :type Float%20%28single-precision%29))
  (|CallParentFunction DeltaSeconds) ; This node is disabled and will not be called.\nDrag off pins to build functionality.
)

(event Custom|setRandomOrientation
  (Transformation|AddRelativeRotation (Variables|Default|GetSquare) (Math|Rotator|MakeRotator (Math|Conversions|ToFloat(Integer) (* (Math|Random|RandomIntegerinRange 0 3) 90)) (Math|Conversions|ToFloat(Integer) (* (Math|Random|RandomIntegerinRange 0 3) 90)) (Math|Conversions|ToFloat(Integer) (* (Math|Random|RandomIntegerinRange 0 3) 90))) false false))

(event Custom|setZOrientationNoise
  (Transformation|AddRelativeRotation (Variables|Default|GetSquare) (Math|Rotator|MakeRotator 0.0 0.0 (Math|Random|RandomFloatinRange -2.0 2.0)) false false))

(fn ConstructionScript
  (|CallParentFunction)
  (CallFunction|SetRandomOrientation))

(fn SetupTheme
  (Utilities|FlowControl|Sequence
    (:then_0
      (Components|StaticMesh|SetStaticMesh (Variables|Default|GetSquare) (Variables|Default|Getsquare_mesh_BORRAR))
      (if (.allow_xyz_roation (Variables|Theme|Getsquare_theme))
        (Transformation|SetRelativeRotation (Variables|Default|GetSquare) (Math|Rotator|MakeRotator (Math|Conversions|ToFloat(Integer) (* (Math|Random|RandomInteger 3) 90)) (Math|Conversions|ToFloat(Integer) (* (Math|Random|RandomInteger 3) 90)) (Math|Conversions|ToFloat(Integer) (* (Math|Random|RandomInteger 3) 90))) false false)))))