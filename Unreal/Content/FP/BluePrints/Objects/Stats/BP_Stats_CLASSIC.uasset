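; BP_Stats_CLASSIC holds the statistics and end-of-game rules for the classic mode of a Minesweeper-style game.
; It reports a loss once any mine is selected and a win when the only unselected squares equal the mine total.
; Score weights squares cleared beyond the initial selections plus correct and incorrect flags, scaled by average speed against a reference pace.
; Completed percentage divides selected mines, not selected squares, by total squares.
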(fn GetStats
  (return (Variables|Default|GetBoardStats)))

(fn GetCompletedPercentage
  (bind _boardstats (Variables|Default|GetBoardStats))
  (return (/ (.mines_selected _boardstats) (.squares_total _boardstats))))

(fn Finished
  (bind _boardstats (Variables|Default|GetBoardStats))
  (Utilities|FlowControl|Sequence
    (:then_0
      (if (> (.mines_selected (Variables|Default|GetBoardStats)) 0)
        (return true false)))
    (:then_1
      (if (== (- (.squares_total _boardstats) (.square_selected _boardstats)) (.mines_total _boardstats))
        (return true true)))
    (:then_2
      (return false false))))

(fn GetScore
  (bind _boardinitialselections (Variables|Default|GetBoardInitialSelections))
  (bind _boardstats (Variables|Default|GetBoardStats))
  (bind _returnvalue (- (.square_selected _boardstats) _boardinitialselections))
  (if (== _returnvalue 0)
    (return 0)
    (else
      (return (Math|Float|Truncate (/ (+ (* _returnvalue (Variables|Default|GetScore_SquareCleared)) (* (.flags_correct _boardstats) (Variables|Default|GetScore_FlagCorrect)) (* (.flags_incorrect _boardstats) (Variables|Default|GetScore_FlagIncorrect))) (/ (/ (Variables|/Game/FP/BPC_Components/BPC_GameTimer.BPC_GameTimer_C|GetTime%20Elapsed (Variables|Default|GetGameTimer)) _returnvalue) (Variables|Default|GetScore_AvgSpeed_SecondPerSquare))))))))