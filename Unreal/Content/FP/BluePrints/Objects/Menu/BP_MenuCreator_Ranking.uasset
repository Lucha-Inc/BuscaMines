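; Menu creator for the ranking menu, which spawns the 3D ranking menu actor BP_Menu_Ranking.
; CreateMenu3D spawns it at the given transform with the supplied parent as owner, passes it RankingObject through SetRanking, then returns the new menu.
; The event graph holds only disabled default events, so all of the logic lives in that factory function.
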(event EventBeginPlay
  (|CallParentFunction) ; This node is disabled and will not be called.\nDrag off pins to build functionality.
)

(event Collision|EventActorBeginOverlap
  (params (OtherActor :type Actor%20Object%20Reference))
  (|CallParentFunction OtherActor) ; This node is disabled and will not be called.\nDrag off pins to build functionality.
)

(event EventTick
  (params (DeltaSeconds :type Float%20%28single-precision%29))
  (|CallParentFunction DeltaSeconds) ; This node is disabled and will not be called.\nDrag off pins to build functionality.
)

(fn ConstructionScript
  (|CallParentFunction))

(fn CreateMenu3D
  (params (Parent :type Actor%20Object%20Reference) (Transform :type Transform))
  (bind _returnvalue (Game|SpawnActorfromClass "/Game/FP/GUI/3D_Menu/Instance/BP_Menu_Ranking.BP_Menu_Ranking_C" Transform "Undefined" "MultiplyWithRoot" Parent false 0.6 0))
  (Default|SetRanking _returnvalue (Variables|Default|GetRankingObject))
  (return _returnvalue))