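; BP_Text3D_Selector is a 3D text selector actor that continuously pulses in size.
; Tick ping-pongs a uniform scale between min and max by flipping the direction at each limit.
; The construction script applies the text and tints all four text faces (front, back, extrude, bevel) through one dynamic material's BaseColor.
; It also exposes the text component's bounds extents.
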(event EventBeginPlay)

(event Collision|EventActorBeginOverlap
  (params (OtherActor :type Actor%20Object%20Reference)))

(event EventTick
  (params (DeltaSeconds :type Float%20%28single-precision%29))
  (bind _output_get (Variables|Default|SetcurrentScale (+ (Variables|Default|GetcurrentScale) (* DeltaSeconds (Variables|Default|GetscaleSpeed) (Variables|Default|Getdirection)))))
  (CallFunction|SetScale)
  (if (>= _output_get (Variables|Default|GetmaxScale))
    (Variables|Default|Setdirection -1.0)
    (elif (<= _output_get (Variables|Default|GetminScale))
      (Variables|Default|Setdirection 1.0))))

(event Custom|setText
  (params (text :type Text))
  (Class|Text3DComponent|SetText (Variables|Default|GetSelector) text))

(event Custom|setColor
  (params (material :type Material%20Instance%20Object%20Reference) (color :type Linear%20Color%20Structure))
  (bind _selector (Variables|Default|GetSelector))
  (Utilities|IsValid material
    (:Is%20Valid
      (bind _returnvalue (Rendering|Material|CreateDynamicMaterialInstance material "None" "None" :!class /Script/Engine.KismetMaterialLibrary))
      (Rendering|Material|SetVectorParameterValue _returnvalue "BaseColor" color :!class /Script/Engine.MaterialInstanceDynamic)
      (Class|Text3DComponent|SetFrontMaterial _selector _returnvalue)
      (Class|Text3DComponent|SetBackMaterial _selector _returnvalue)
      (Class|Text3DComponent|SetExtrudeMaterial _selector _returnvalue)
      (Class|Text3DComponent|SetBevelMaterial _selector _returnvalue))))

(fn ConstructionScript
  (CallFunction|SetText (Variables|Config|GetText))
  (CallFunction|SetColor (Variables|Config|GetMaterial) (Variables|Config|GetColor)))

(fn GetBoundsExtents
  (return (.BoxExtent (Class|Text3DComponent|GetBounds (Variables|Default|GetSelector)))))

(fn SetScale
  (Transformation|SetRelativeScale3D (Variables|Default|GetSelector) (Math|Conversions|ToVector(Float) (Variables|Default|GetcurrentScale))))