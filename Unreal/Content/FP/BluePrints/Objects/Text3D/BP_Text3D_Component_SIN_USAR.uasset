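; BP_Text3D_Component_SIN_USAR is an actor wrapping a Text3D component for displaying 3D text, marked by name as unused ("sin usar").
; The construction script applies the default text and color through setup events that other Blueprints can also call.
; Color setup creates a dynamic material instance, sets BaseColor, and assigns it to front, back, extrude and bevel.
; GetTextBounds exposes the text's origin and extent; the EventGraph is empty.
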(event EventBeginPlay)

(event Collision|EventActorBeginOverlap
  (params (OtherActor :type Actor%20Object%20Reference)))

(event EventTick
  (params (DeltaSeconds :type Float%20%28single-precision%29)))

(event Custom|setupColor
  (params (material :type Material%20Object%20Reference) (color :type Linear%20Color%20Structure))
  (bind _text3d_master (Variables|Default|GetText3D_Master))
  (Utilities|IsValid material
    (:Is%20Valid
      (bind _returnvalue (Rendering|Material|CreateDynamicMaterialInstance material "None" "None" :!class /Script/Engine.KismetMaterialLibrary))
      (Rendering|Material|SetVectorParameterValue _returnvalue "BaseColor" color :!class /Script/Engine.MaterialInstanceDynamic)
      (Class|Text3DComponent|SetFrontMaterial _text3d_master _returnvalue)
      (Class|Text3DComponent|SetBackMaterial _text3d_master _returnvalue)
      (Class|Text3DComponent|SetExtrudeMaterial _text3d_master _returnvalue)
      (Class|Text3DComponent|SetBevelMaterial _text3d_master _returnvalue))))

(event Custom|setupText
  (params (text :type Text))
  (Class|Text3DComponent|SetText (Variables|Default|GetText3D_Master) text))

(fn ConstructionScript
  (CallFunction|SetupText (Variables|Default|GetdefaultText))
  (CallFunction|SetupColor (Variables|Default|GettextMaterial) (Variables|Default|GettextColor)))

(fn GetTextBounds
  (bind _text3d_master (Variables|Default|GetText3D_Master))
  (bind (_origin _boxextent) (Class|Text3DComponent|GetBounds _text3d_master))
  (return _origin _boxextent))