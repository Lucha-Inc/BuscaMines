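; BP_Text3D_text is a 3D text actor whose Text3D component takes its text, material and color from variables applied in the Construction Script.
; Setting the color creates a dynamic instance of a valid material, sets its BaseColor parameter and assigns it to the front, back, extrude and bevel faces.
; A helper function returns the text's box extent, and the Event Graph has no active logic.
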(event EventBeginPlay)

(event Collision|EventActorBeginOverlap
  (params (OtherActor :type Actor%20Object%20Reference)))

(event EventTick
  (params (DeltaSeconds :type Float%20%28single-precision%29)))

(event Custom|setText
  (params (text :type Text))
  (Class|Text3DComponent|SetText (Variables|Default|GetText3D) text))

(event Custom|setColor
  (params (material :type Material%20Instance%20Object%20Reference) (color :type Linear%20Color%20Structure))
  (bind _text3d (Variables|Default|GetText3D))
  (Utilities|IsValid material
    (:Is%20Valid
      (bind _returnvalue (Rendering|Material|CreateDynamicMaterialInstance material "None" "None" :!class /Script/Engine.KismetMaterialLibrary))
      (Rendering|Material|SetVectorParameterValue _returnvalue "BaseColor" color :!class /Script/Engine.MaterialInstanceDynamic)
      (Class|Text3DComponent|SetFrontMaterial _text3d _returnvalue)
      (Class|Text3DComponent|SetBackMaterial _text3d _returnvalue)
      (Class|Text3DComponent|SetExtrudeMaterial _text3d _returnvalue)
      (Class|Text3DComponent|SetBevelMaterial _text3d _returnvalue))))

(fn ConstructionScript
  (CallFunction|SetText (Variables|Default|GetText))
  (CallFunction|SetColor (Variables|Default|GetMaterial) (Variables|Default|GetColor)))

(fn GetBoundsExtents
  (return (.BoxExtent (Class|Text3DComponent|GetBounds (Variables|Default|GetText3D)))))