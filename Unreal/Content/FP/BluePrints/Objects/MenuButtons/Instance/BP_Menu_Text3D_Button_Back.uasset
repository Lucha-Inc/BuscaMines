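; A 3D text menu button that takes the player back to the previous menu.
; On construction it shows or hides the BPMenuText3DButton component, without propagating to children, based on whether the GameModeMaster reports a valid last menu.
; Clicking runs the parent button's click logic, then calls GoBackToLastMenu on the GameModeMaster obtained through GetCustomClasses.
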(event EventBeginPlay
  (|CallParentFunction) ; This node is disabled and will not be called.\nDrag off pins to build functionality.
)

(event Collision|EventActorBeginOverlap
  (params (OtherActor :type Actor%20Object%20Reference)))

(event EventTick
  (params (DeltaSeconds :type Float%20%28single-precision%29)))

(fn ConstructionScript
  (|CallParentFunction)
  (bind _gamemode_master (CallFunction|GetCustomClasses self))
  (Rendering|SetVisibility (Variables|Default|GetBP_Menu_Text3D_Button) (Default|LastMenuIsValid _gamemode_master) false))

(fn OnClick
  (|CallParentFunction)
  (bind _gamemode_master (CallFunction|GetCustomClasses self))
  (Default|GoBacktoLastMenu _gamemode_master))