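; A 3D text menu button that takes the player to the ranking menu when clicked.
; Its click override runs the parent behavior, then fetches the ranking object from the GameModeMaster obtained via GetCustomClasses.
; It spawns a BP_MenuCreator_Ranking initialized with that object and hands it to the GameModeMaster's GoToMenuByCreator to switch menus.
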(event EventBeginPlay
  (|CallParentFunction) ; This node is disabled and will not be called.\nDrag off pins to build functionality.
)

(event Collision|EventActorBeginOverlap
  (params (OtherActor :type Actor%20Object%20Reference)))

(event EventTick
  (params (DeltaSeconds :type Float%20%28single-precision%29)))

(fn ConstructionScript
  (|CallParentFunction))

(fn OnClick
  (|CallParentFunction)
  (bind _gamemode_master (CallFunction|GetCustomClasses self))
  (bind _ranking (Default|GetRankingObject _gamemode_master))
  (bind _returnvalue (Game|SpawnActorfromClass "/Game/FP/BluePrints/Objects/Menu/MenuCreators/BP_MenuCreator_Ranking.BP_MenuCreator_Ranking_C" (Math|Transform|MakeTransform "0, 0, 0") "Undefined" "MultiplyWithRoot" 0 _ranking 0 0))
  (Default|GotoMenubyCreator _gamemode_master _returnvalue))