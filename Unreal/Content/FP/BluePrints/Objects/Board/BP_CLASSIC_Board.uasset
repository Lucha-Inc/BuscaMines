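; Classic Minesweeper board actor that builds a centred grid of themed squares sized by Difficulty, with mines rolled independently per square by probability.
; Construction sets up the squares, selects a random empty one as the opening, then fits bounds and starting point.
; Stat updates tally mines, selections and flags into a BP_Stats_CLASSIC object, signalling board updates and a win or loss.
; BeginPlay creates the theme-based sound manager.
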(event EventBeginPlay
  (Utilities|FlowControl|Sequence
    (:then_0
      (bind _gameinstance (CallFunction|GetCustomClasses self))
      (bind _da_theme_board (CallFunction|GetTheme))
      (bind _returnvalue (Game|ConstructObjectfromClass "/Game/FP/BluePrints/Managers/Sound/BP_SoundClass_Manager_Board.BP_SoundClass_Manager_Board_C" _da_theme_board _gameinstance))
      (Variables|Default|SetSound%20Manager%20Board _returnvalue))))

(event EventSetupBounds
  (Utilities|FlowControl|Sequence
    (:then_0
      (bind _size (CallFunction|GetBoardSize))
      (Components|Box|SetBoxExtent (Variables|Default|Getboard_bounds) (/ _size 2) false))
    (:then_1
      (|CallParentFunction))))

(event EventUpdateStats
  (params (SetupInitialStat :type Boolean))
  (bind _bp_stats_classic (CallFunction|UpdatingStats SetupInitialStat))
  (Default|CallBoardStatsUpdated _bp_stats_classic)
  ;[1 1 1] Si Finalizó
  (bind (_isfinished _won) (Default|Finished _bp_stats_classic))
  (if _isfinished
    (Default|CallBoardFinished _won)))

(fn ConstructionScript
  (|CallParentFunction)
  (Utilities|FlowControl|Sequence
    (:then_0
      (bind _gamemode_master (CallFunction|GetCustomClasses self))
      (bind _returnvalue (Game|ConstructObjectfromClass "/Game/FP/BluePrints/Objects/Stats/BP_Stats_CLASSIC.BP_Stats_CLASSIC_C" (Variables|/Game/FP/BluePrints/Global/GM_GameModes/BP_Abstract_GameMode_Master.BP_Abstract_GameMode_Master_C|GetTimer _gamemode_master)))
      (Variables|Stats|SetStats_Classic_Object _returnvalue))))

(fn BoardConstruction
  (bind _emptysquares (LocalVariables|GetemptySquares))
  (bind _outitem (Utilities|Array|Random _emptysquares))
  (Utilities|FlowControl|Sequence
    (:then_1
      (CallFunction|SquareCreation))
    (:then_2
      ;[1 1 1] Inicializa los números de cada Square
      (bind _values (Utilities|Map|Values (Variables|Default|Getsquares)))
      (for _array_element _values
        (Default|Setup _array_element)))
    (:then_3
      ;[1 1 1] Selecciona solo un EMPTY al inicio
      (bind _values_2 (Utilities|Map|Values (Variables|Default|Getsquares)))
      (for _array_element_2 _values_2
        (if (Default|IsEmptyArea _array_element_2)
          (Utilities|Array|Add (LocalVariables|GetemptySquares) _array_element_2)))
      (Utilities|IsValid _outitem
        (:Is%20Valid
          (Default|Select _outitem))))
    (:then_4
      (CallFunction|SetupBounds))
    (:then_5
      (CallFunction|SetupStartingPoint))
    (:then_7
      (return (Variables|Default|Getsquares)))))

(fn UpdatingStats
  (params (SetupInitialStat :type Boolean))
  (bind _values (Utilities|Map|Values (Variables|Default|Getsquares)))
  (for _array_element _values
    ;[1 1 1] Temporal Variables
    (Math|Integer|IncrementInt (LocalVariables|GetTempSquares)
      (:%20%20
        (LocalVariables|SetTempSquaresCorrectSelected (+ (and (not (.withMine (Default|GetStatus _array_element))) (.isSelected (Default|GetStatus _array_element))) (LocalVariables|GetTempSquaresCorrectSelected)))
        (LocalVariables|SetTempMines (+ (.withMine (Default|GetStatus _array_element)) (LocalVariables|GetTempMines)))
        (LocalVariables|SetTempFlagCorrect (+ (and (.withMine (Default|GetStatus _array_element)) (.isSuspected (Default|GetStatus _array_element))) (LocalVariables|GetTempFlagCorrect)))
        (LocalVariables|SetTempFlagIncorrect (+ (and (not (.withMine (Default|GetStatus _array_element))) (.isSuspected (Default|GetStatus _array_element))) (LocalVariables|GetTempFlagIncorrect)))
        (LocalVariables|SetTempMinesSelected (+ (and (.withMine (Default|GetStatus _array_element)) (.isSelected (Default|GetStatus _array_element))) (LocalVariables|GetTempMinesSelected))))))
  (Utilities|FlowControl|Sequence
    (:then_0
      (Variables|/Game/FP/BluePrints/Objects/Stats/BP_Stats_CLASSIC.BP_Stats_CLASSIC_C|SetBoardStats (Variables|Stats|GetStats_Classic_Object) (Utilities|Struct|MakeStruct_Board_CLASSIC_Stats (LocalVariables|GetTempSquares) (LocalVariables|GetTempSquaresCorrectSelected) (LocalVariables|GetTempMines) (LocalVariables|GetTempMinesSelected) (LocalVariables|GetTempFlagCorrect) (LocalVariables|GetTempFlagIncorrect))))
    (:then_1
      (if SetupInitialStat
        (Variables|/Game/FP/BluePrints/Objects/Stats/BP_Stats_CLASSIC.BP_Stats_CLASSIC_C|SetBoardInitialSelections (Variables|Stats|GetStats_Classic_Object) (LocalVariables|GetTempSquaresCorrectSelected))))
    (:then_2
      (return (Variables|Stats|GetStats_Classic_Object)))))

(fn GetStats
  (return (Variables|Stats|GetStats_Classic_Object)))

(fn SquareCreation
  (bind _difficulty (Variables|Board|GetDifficulty))
  (bind _square_width (Variables|Default|Getsquare_width))
  (bind _square_separation (Variables|Default|Getsquare_separation))
  (bind _returnvalue (+ _square_width _square_separation))
  ;[1 1 1] Squares Creation
  (for _index (range 1 (Default|GetBoardRows _difficulty))
    (for _index_2 (range 1 (Default|GetBoardColumns _difficulty))
      ;;[1 1 1] Add Offset to center in the Board
      (bind _size (CallFunction|GetBoardSize))
      (bind _da_theme_board (CallFunction|GetTheme))
      (bind _returnvalue_2 (Game|SpawnActorfromClass "/Game/FP/BluePrints/Objects/Squares/BP_Square_Theme.BP_Square_Theme_C" (Math|Transform|MakeTransform (- (Math|Vector|MakeVector (* (- _index 1) _returnvalue) (* (- _index_2 1) _returnvalue) 0.0) (/ (Math|Vector|MakeVector (.x _size) (.y _size) 0.0) 2))) "Undefined" "MultiplyWithRoot" 0 "/Game/FP/Meshes/Squares/Wood/square_wood_v3.square_wood_v3" 0 0 (Variables|/Game/FP/Data/DataAsset/Board/DA_ThemeData_Board.DA_ThemeData_Board_C|Getsquare_theme _da_theme_board) (Utilities|Struct|MakeCoord_2D _index _index_2) self (< (Math|Random|RandomFloatinRange 0.0 1.0) (Default|GetMineProbability _difficulty)) 0))
      (Transformation|AttachActorToActor _returnvalue_2 self "Squares" "KeepRelative" "KeepRelative" "KeepRelative" true)
      (Utilities|Map|Add (Variables|Default|Getsquares) (Utilities|Struct|MakeCoord_2D _index _index_2) _returnvalue_2))))

(fn GetBoardSize
  (bind _difficulty (Variables|Board|GetDifficulty))
  (bind _square_separation (Variables|Default|Getsquare_separation))
  (bind _square_width (Variables|Default|Getsquare_width))
  (bind _square_separation_2 (Variables|Default|Getsquare_separation))
  (bind _returnvalue (+ _square_width _square_separation))
  (return (Math|Vector|MakeVector (- (* (Default|GetBoardRows _difficulty) _returnvalue) _square_separation_2) (- (* (Default|GetBoardColumns _difficulty) _returnvalue) _square_separation_2) _square_width)))

(fn GetBoardDifficulty
  (return (Variables|Board|GetDifficulty)))