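; Master player controller for a board game with a free-flying character camera and 3D menus.
; It enables desktop or mobile input components by platform; their events, mostly gated by a game-input flag, drive board square select/suspect, look and movement.
; Movement follows the bounds' axes and eases out near edges when bounds are active, while pitch stays downward except in debug mode.
; Menu calls forward to the player's menu component, pause to the GameMode.
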(event Custom|SetBoard
  (params (Board :type BP%20Board%20Master%20Object%20Reference))
  (Variables|Board|SetBoard Board))

(event Custom|SetPlayerMovementBounds
  (params (BoundsParameters :type Player%20Movement%20Bounds%20Definition%20Structure))
  (bind _output_get (Variables|Bounds|Setmovement_bounds BoundsParameters))
  (bind _debugmode (CallFunction|GetDebugMode self))
  (if _debugmode
    (Rendering|Debug|DrawDebugBox (.bounds_origin _output_get) (.bounds_extents _output_get) "(R=0.000000,G=1.000000,B=0.000000,A=1.000000)" (Math|Rotator|MakeRotfromX (.normal_vector_x _output_get)) 1.2e+02 5.0)))

(event EventBeginPlay
  (bind _ismobile (CallFunction|IsMobile))
  (Utilities|FlowControl|Sequence
    (:then_0
      ;[0.15 0.15 0.15 0.5] SetupManagers
      (bind _gamemode_master (CallFunction|GetCustomClasses self))
      (Variables|Managers|SetGameMode _gamemode_master))
    (:then_1
      ;[0.15 0.15 0.15 0.5] Set BPC Menu Controller
      (bind _asbp_player (Utilities|Casting|CastToBP_player (Game|GetPlayerCharacter 0)))
      (Variables|Menu3D|SetMenu3D_Controller (Variables|/Game/FP/BluePrints/Chareacters/Player/BP_player.BP_player_C|GetBPC_Player_Menu_Controller _asbp_player)))
    (:then_2
      ;[0.15 0.15 0.15 0.5] Setup Inputs Components
      (Default|Setup (Variables|Default|GetBPC_PlayerInputs_Desktop) self (not _ismobile))
      (Default|Setup (Variables|Default|GetBPC_PlayerInputs_Mobile) self _ismobile))
    (:then_3
      (bind _ascharacter (Utilities|Casting|CastToCharacter (Pawn|GetControlledPawn)))
      (Variables|/Script/Engine.CharacterMovementComponent|SetMaxFlySpeed (Variables|/Script/Engine.Character|GetCharacterMovement _ascharacter) 2.5e+03))))

(event Custom|Board_Suspect_Square
  (params (Square%20Coord :type Coord%202D%20Structure))
  (if (Variables|Default|GetGameInputsEnable)
    (Default|SuspectSquare (Variables|Board|GetBoard) Square%20Coord)))

(event Custom|Board_Select_Square
  (params (Square%20Coord :type Coord%202D%20Structure))
  (if (Variables|Default|GetGameInputsEnable)
    (Default|SelectSquare (Variables|Board|GetBoard) Square%20Coord)))

(event Custom|Set_GameInputsEnable
  (params (Enable :type Boolean))
  (Variables|Default|SetGameInputsEnable Enable))

(event Custom|OnPause
  (Default|OnPause (Variables|Managers|GetGameMode)))

(event Custom|Player_Move_XY
  (params (Movement :type Vector%202D%20Structure))
  (bind _returnvalue (Game|GetPlayerCharacter 0))
  (bind _returnvalue_2 (Game|GetPlayerCharacter 0))
  (bind _returnvalue_3 (Game|GetPlayerCharacter 0))
  (bind _movement_bounds (Variables|Bounds|Getmovement_bounds))
  (bind _movement_bounds_2 (Variables|Bounds|Getmovement_bounds))
  (bind _movement_bounds_3 (Variables|Bounds|Getmovement_bounds))
  (bind _returnvalue_4 (Transformation|GetActorLocation _returnvalue))
  (bind _returnvalue_5 (Transformation|GetActorLocation _returnvalue_3))
  (bind _returnvalue_6 (* (.y (.bounds_extents _movement_bounds_3)) -1.0))
  (bind _returnvalue_7 (* (.x (.bounds_extents _movement_bounds)) -1.0))
  (bind _returnvalue_8 (- _returnvalue_4 (.bounds_origin _movement_bounds)))
  (bind _returnvalue_9 (- _returnvalue_5 (.bounds_origin _movement_bounds_3)))
  (bind _returnvalue_10 (Math|Vector|DotProduct _returnvalue_9 (.normal_vector_y _movement_bounds_3)))
  (bind _returnvalue_11 (Math|Vector|DotProduct _returnvalue_8 (.normal_vector_x _movement_bounds)))
  (bind _returnvalue_12 (>= _returnvalue_10 0.0))
  (bind _returnvalue_13 (>= _returnvalue_11 0.0))
  (if (Variables|Default|GetGameInputsEnable)
    ;[0.15 0.15 0.15 0.5] DEBUG MODE sin límites
    (if (.bounds_active _movement_bounds_2)
      (Pawn|Input|AddMovementInput (Game|GetPlayerCharacter 0) (.normal_vector_x (Variables|Bounds|Getmovement_bounds)) (* (.x Movement) (select (Class|KismetMathLibrary|XORBoolean (>= (.x Movement) 0.0) _returnvalue_13) 1.0 (select _returnvalue_13 (Math|Float|MapRangeClamped _returnvalue_11 (.x (.bounds_extents _movement_bounds)) (- (.x (.bounds_extents _movement_bounds)) (.x (.bounds_offset _movement_bounds))) 0.0 1.0) (Math|Float|MapRangeClamped _returnvalue_11 (+ (.x (.bounds_offset _movement_bounds)) _returnvalue_7) _returnvalue_7 1.0 0.0)))) false)
      (Pawn|Input|AddMovementInput (Game|GetPlayerCharacter 0) (.normal_vector_y (Variables|Bounds|Getmovement_bounds)) (* (.y Movement) (select (Class|KismetMathLibrary|XORBoolean (>= (.y Movement) 0.0) _returnvalue_12) 1.0 (select _returnvalue_12 (Math|Float|MapRangeClamped _returnvalue_10 (.y (.bounds_extents _movement_bounds_3)) (- (.y (.bounds_extents _movement_bounds_3)) (.y (.bounds_offset _movement_bounds_3))) 0.0 1.0) (Math|Float|MapRangeClamped _returnvalue_10 (+ (.y (.bounds_offset _movement_bounds_3)) _returnvalue_6) _returnvalue_6 1.0 0.0)))) false)
      (else
        (Pawn|Input|AddMovementInput _returnvalue_2 (.normal_vector_x _movement_bounds_2) (.x Movement) false)
        (Pawn|Input|AddMovementInput _returnvalue_2 (.normal_vector_y _movement_bounds_2) (.y Movement) false)))))

(event Custom|Player_Look
  (params (Look :type Vector%202D%20Structure))
  (bind _returnvalue (Game|GetPlayerCharacter 0))
  (bind _returnvalue_2 (Transformation|GetActorRotation _returnvalue))
  (if (Variables|Default|GetGameInputsEnable)
    (Class|Actor|AddActorWorldRotation _returnvalue (Math|Rotator|MakeRotator 0.0 0.0 (.x Look)))
    (bind _debugmode (CallFunction|GetDebugMode self))
    (Transformation|AddActorLocalRotation _returnvalue (Math|Rotator|MakeRotator 0.0 (select _debugmode (.y Look) (Math|Float|Max(Float) (Math|Float|Min(Float) (.y Look) (- -3e+01 (.pitch _returnvalue_2))) (- -9e+01 (.pitch _returnvalue_2)))) 0.0) false false)))

(event Custom|Player_Move_Z
  (params (Movement%20Z :type Float%20%28double-precision%29))
  (bind _returnvalue (Game|GetPlayerCharacter 0))
  (bind _returnvalue_2 (>= Movement%20Z 0.0))
  (bind _movement_bounds (Variables|Bounds|Getmovement_bounds))
  (bind _returnvalue_3 (Transformation|GetActorLocation _returnvalue))
  (if (Variables|Default|GetGameInputsEnable)
    (Pawn|Input|AddMovementInput (Game|GetPlayerCharacter 0) "0.000000,0.000000,1.000000" (* Movement%20Z (select (and (not _returnvalue_2) (<= (.z _returnvalue_3) 0.0)) 0.0 (select (.bounds_active _movement_bounds) (select _returnvalue_2 (Math|Float|MapRangeClamped (.z _returnvalue_3) (.z (.bounds_extents _movement_bounds)) (- (.z (.bounds_extents _movement_bounds)) (.z (.bounds_offset _movement_bounds))) 0.0 1.0) 1.0) 1.0))) false)))

(event Custom|Menu_Scroll
  (params (Scroll_Speed :type Float%20%28double-precision%29))
  (Default|OnScroll (Variables|Menu3D|GetMenu3D_Controller) Scroll_Speed))

(fn ConstructionScript)

(fn ClearMenus3D
  (Default|ClearMenus (Variables|Menu3D|GetMenu3D_Controller)))

(fn ShowMenu3D
  (params (Menu3D :type BP%20Actor%20Menu%203D%20Class%20Reference))
  (bind _menu_3d (Default|SetMenu3D (Variables|Menu3D|GetMenu3D_Controller) Menu3D))
  (return _menu_3d))