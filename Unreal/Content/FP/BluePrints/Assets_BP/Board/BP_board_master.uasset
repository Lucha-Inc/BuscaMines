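; Base board Blueprint for a square-based game, with placeholder construction, size and stats functions.
; Loads a theme data asset, derives a start transform from board size, and exposes bounds and axes for movement.
; Selecting a square can disable game input; animating squares are tracked until all finish, then stats update and readiness is signaled.
; Suspecting a square updates stats immediately, and debug mode toggles helper component visibility.
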(event EventBeginPlay
  (bind _thememanager (CallFunction|GetCustomClasses self))
  (Variables|Theme|SetTheme_Board (Default|GetDataAssetThemeBoard _thememanager (Variables|Theme|GetEnum%20Theme%20Board))))

(event EventBoardStart
  (Utilities|FlowControl|DoOnce false
    (:Completed
      (CallFunction|UpdateStats self true))))

(event EventSetupBounds
  (Components|Box|SetBoxExtent (Variables|Default|GetEnvironmentBox) (+ (Variables|/Script/Engine.BoxComponent|GetBoxExtent (Variables|Default|Getboard_bounds)) "500.000000,500.000000,1000.000000") true))

(event EventSetupStartingPoint
  (bind _startingvector (Variables|Default|GetStartingVector))
  (bind _relativelocation (Variables|/Script/Engine.SceneComponent|GetRelativeLocation _startingvector))
  (Transformation|SetRelativeLocationAndRotation (Variables|Default|GetStartingVector) "0, 0, 0" "0, 0, 0" false false)
  (bind _size (CallFunction|GetBoardSize))
  (Transformation|AddLocalOffset (Variables|Default|GetStartingVector) (Math|Vector|MakeVector (- (.x (/ _size -2)) 5e+02) 0.0 (Math|Float|MapRangeClamped (.X (Math|Vector|BreakVector _size)) 1e+03 3e+03 5e+02 1e+03)) false false)
  (Transformation|AddLocalRotation _startingvector (Math|Rotator|MakeRotator 0.0 (/ (+ (.pitch (Math|Rotator|MakeRotfromX (- (Math|Vector|MakeVector (/ (.X (Math|Vector|BreakVector _size)) 2.0) 0.0 0.0) _relativelocation))) (.pitch (Math|Rotator|MakeRotfromX (- (Math|Vector|MakeVector (/ (.X (Math|Vector|BreakVector _size)) -2.0) 0.0 0.0) _relativelocation)))) 2.0) 0.0) false false))

(event Custom|disableUserInputs
  (bind _asbp_abstract_game_mode_master (Utilities|Casting|CastToBP_Abstract_GameMode_Master (Game|GetGameMode)))
  (Default|RemoveGameInputs _asbp_abstract_game_mode_master))

(event Custom|SelectSquare
  (params (SquareCoords :type Coord%202D%20Structure))
  (bind _squares (Variables|Board|Getsquares))
  (bind _value (Utilities|Map|Find _squares SquareCoords))
  (bind _expoted (Default|Select _value))
  (if _expoted
    (CallFunction|DisableUserInputs))
  (if (Default|IsReady _value)
    (CallFunction|OnSquareReady)
    (else
      (EventDispatchers|BindEventtoAnimationReady _value (delegate Custom|OnSquareReady))
      (Variables|Default|SetReady false)
      (Utilities|Array|Add (Variables|Default|GetSquaresInProcess) _value))))

(event Custom|OnSquareReady
  (params (Square :type BP%20Square%20Object%20Reference))
  (Utilities|IsValid Square
    (:Is%20Valid
      (Utilities|Array|RemoveItem (Variables|Default|GetSquaresInProcess) Square))
    (:Is%20Not%20Valid
      _))
  (if (Utilities|Array|IsEmpty (Variables|Default|GetSquaresInProcess))
    (Variables|Default|SetReady true)
    (CallFunction|OnBoardReady)))

(event Custom|onBoardReady
  (CallFunction|UpdateStats self false)
  (Default|CallAnimationsReady))

(event Custom|SuspectSquare
  (params (Square%20Coords :type Coord%202D%20Structure))
  (Default|Suspect (.Value (Utilities|Map|Find (Variables|Board|Getsquares) Square%20Coords)))
  (CallFunction|UpdateStats false))

(fn ConstructionScript
  (bind _board_axis_x (Variables|Default|Getboard_axis_x))
  (Utilities|FlowControl|Sequence
    (:then_0
      (bind _thememanager (CallFunction|GetCustomClasses self))
      (Variables|Theme|SetTheme_Board (Default|GetDataAssetThemeBoard _thememanager (Variables|Theme|GetEnum%20Theme%20Board))))
    (:then_1
      (bind _debugmode (CallFunction|GetDebugMode self))
      (Rendering|SetVisibility (Variables|Default|Getboard_bounds) _debugmode false))
    (:then_2
      (bind _debugmode_2 (CallFunction|GetDebugMode self))
      (Rendering|SetVisibility _board_axis_x _debugmode_2 false)
      (Development|SetHiddeninGame _board_axis_x false false))))

(fn GetSquares
  (return (Variables|Board|Getsquares)))

(fn GetBox
  (return (Variables|Components|Getbox_structure_BORRAR)))

(fn GetStartPosition
  (bind _startingvector (Variables|Default|GetStartingVector))
  (return (Math|Transform|MakeTransform (Transformation|GetWorldLocation _startingvector) (Transformation|GetWorldRotation _startingvector) "1.000000,1.000000,1.000000")))

(fn GetBoardMovementsBounds
  (bind _board_bounds (Variables|Default|Getboard_bounds))
  (bind (_directionvector_x _directionvector_y) (CallFunction|GetBoardDirectionVector))
  (return (Utilities|Struct|MakeBoardBoundsDefinition (Transformation|GetWorldLocation _board_bounds) (Variables|/Script/Engine.BoxComponent|GetBoxExtent _board_bounds) _directionvector_x _directionvector_y)))

(fn BoardConstruction
  (return 0))

(fn GetBoardDirectionVector
  (bind _board_axis_x (Variables|Default|Getboard_axis_x))
  (return (Math|Vector|GetForwardVector _board_axis_x) (Math|Vector|GetRightVector _board_axis_x)))

(fn GetBoardSize
  (return "0, 0, 0"))

(fn GetStats
  (return 0))