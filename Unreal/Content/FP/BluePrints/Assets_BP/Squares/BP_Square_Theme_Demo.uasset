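; BP_Square_Theme_Demo is a demo minesweeper square, apparently for previewing a square theme.
; Its construction script runs the parent's script, then sets visibility on the 3D mine-count text, flag, mine and square components from four Demo boolean variables, one per component.
; The event graph holds only disabled default events, so it adds no runtime behavior of its own.
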(event EventBeginPlay
  (|CallParentFunction) ; This node is disabled and will not be called.\nDrag off pins to build functionality.
)

(event Collision|EventActorBeginOverlap
  (params (OtherActor :type Actor%20Object%20Reference))
  (|CallParentFunction OtherActor) ; This node is disabled and will not be called.\nDrag off pins to build functionality.
)

(event EventTick
  (params (DeltaSeconds :type Float%20%28single-precision%29))
  (|CallParentFunction DeltaSeconds) ; This node is disabled and will not be called.\nDrag off pins to build functionality.
)

(fn ConstructionScript
  (|CallParentFunction)
  (Rendering|SetVisibility (Variables|Default|GetBP_Text3D_NumberMines) (Variables|Demo|Getdemo_number_visible) false)
  (Rendering|SetVisibility (Variables|Default|GetFlag) (Variables|Demo|Getdemo_flag_visible) false)
  (Rendering|SetVisibility (Variables|Default|GetMine) (Variables|Demo|Getdemo_mine_visible) false)
  (Rendering|SetVisibility (Variables|Default|GetSquare) (Variables|Demo|Getdemo_square_visible) false))