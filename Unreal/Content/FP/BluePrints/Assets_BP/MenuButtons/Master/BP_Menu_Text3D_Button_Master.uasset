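; Master 3D text button for menus, with a child-actor text whose content, material and color are set in the construction script.
; Shortly after BeginPlay it fits a collision Box to the text bounds plus padding; the Box is visible only in debug mode.
; Click or touch plays a UI sound, calls Call3DButtonOnClick and the empty OnClick hook.
; A goToMenu event forwards a valid menu class to the master GameMode.
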(event OnClicked(Box)
  (params (TouchedComponent :type Primitive%20Component%20Object%20Reference) (ButtonPressed :type Key%20Structure :default "None"))
  (CallFunction|PlayClickSound)
  (Default|Call3DButtononClick)
  (CallFunction|OnClick))

(event OnInputTouchBegin(Box)
  (params (FingerIndex :type ETouchIndex%20Enum :default "Touch1") (TouchedComponent :type Primitive%20Component%20Object%20Reference))
  (CallFunction|PlayClickSound)
  (Default|Call3DButtononClick)
  (CallFunction|OnClick))

(event Custom|goToMenu
  (params (toMenu :type BP%20Actor%20Menu%203D%20Class%20Reference))
  (if (Utilities|IsValidClass toMenu)
    (bind _asbpi_game_mode_master (Utilities|Casting|CastToBPI_GameMode_Master (Game|GetGameMode)))
    (Default|GotoMenu _asbpi_game_mode_master toMenu)))

(event Custom|setup
  ;[1 1 1] Cuando ocurre, el objeto ya fué escalado y nosotros lo dimensionamos con unas medidas sin escalar
  (Components|Box|SetBoxExtent (Variables|Default|GetBox) (+ (.BoxExtent (Class|Text3DComponent|GetBounds (Variables|/Game/FP/BluePrints/Assets_BP/Text3D/BP_Text3D_Button.BP_Text3D_Button_C|GetText3D (Variables|Default|Gettext3D)))) "40.000000,40.000000,40.000000") true))

(event EventBeginPlay
  (Utilities|FlowControl|Delay 0.2)
  (CallFunction|Setup))

(event Custom|PlayClickSound
  (bind _gameinstance (CallFunction|GetCustomClasses self))
  (bind _sound_manager_app (Default|GetSoundManagerApp _gameinstance))
  (Default|PlayUIButtonClick _sound_manager_app))

(fn ConstructionScript
  (Utilities|FlowControl|Sequence
    (:then_0
      (bind _asbp_text_3d_button (Utilities|Casting|CastToBP_Text3D_Button (Variables|/Script/Engine.ChildActorComponent|GetChildActor (Variables|Default|GetBP_Menu_Text3D_Button))))
      (bind _output_get (Variables|Default|Settext3D _asbp_text_3d_button))
      (Default|SetText _output_get (Variables|Default|GetText))
      (Default|SetColor _output_get (Variables|Default|GetMaterial) (Variables|Default|GetColor)))
    (:then_1
      (bind _debugmode (CallFunction|GetDebugMode self))
      (Rendering|SetVisibility (Variables|Default|GetBox) _debugmode false))))

(fn OnClick)