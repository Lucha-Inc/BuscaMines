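; Test player-input component (PRUEBA) that provides a unified pointer position and a placeholder board-select action.
; On BeginPlay it caches the first player controller and the master game mode, obtained through a custom-classes lookup.
; The pointer getter returns the Touch1 location while that touch is pressed, otherwise the viewport mouse position.
; The board-select action only writes a debug log, and the InputsActions graph is empty.
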(event EventBeginPlay
  (bind _output_get (Variables|Default|SetPlayer%20Controller (Game|GetPlayerController 0)))
  (bind _gamemode_master (CallFunction|GetCustomClasses _output_get))
  (Variables|Default|SetGame%20Mode%20Master _gamemode_master))

(event EventTick
  (params (DeltaSeconds :type Float%20%28single-precision%29)))

(event Input|EnhancedActionEvents|EnhancedInputActionIA_Board_Select
  (params (ActionValue :type Boolean) (ElapsedSeconds :type Float%20%28double-precision%29) (TriggeredSeconds :type Float%20%28double-precision%29) (InputAction :type Input%20Action%20Object%20Reference :default "/Game/FP/Inputs/Actions/IA_Board_Select.IA_Board_Select")))

(fn GetPointerPosition
  (bind _player_controller (Variables|Default|GetPlayer%20Controller))
  (bind (_locationx _locationy _biscurrentlypressed) (Class|PlayerController|GetInputTouchState _player_controller "Touch1"))
  (bind _returnvalue (Class|WidgetLayoutLibrary|GetMousePositiononViewport))
  (return (select _biscurrentlypressed (Math|Vector2D|MakeVector2D _locationx _locationy) _returnvalue)))

(fn ActionBoardSelect
  (CallFunction|DebugLogVector (Variables|Default|GetPlayer%20Controller) "ACTION SELECT" "0, 0, 0"))