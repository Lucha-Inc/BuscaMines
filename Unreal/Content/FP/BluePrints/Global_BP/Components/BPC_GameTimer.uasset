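; BPC_GameTimer is an actor component that tracks elapsed game time between a start and an end event.
; Tick runs while the timer is started and not ended, always adding to total elapsed time and adding to active time only when unpaused.
; Start, end and pause on, off, toggle and set events drive the state flags, with pause changes accepted only while running.
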(event EventBeginPlay)

(event EventTick
  (params (DeltaSeconds :type Float%20%28single-precision%29))
  (bind _running (CallFunction|IsRunning))
  (if _running
    (Utilities|FlowControl|Sequence
      (:then_0
        (Variables|Default|SetTimeElapsedTotal (+ (Variables|Default|GetTimeElapsedTotal) DeltaSeconds)))
      (:then_1
        (if (not (Variables|Default|Getpaused))
          (Variables|Default|SetTime%20Elapsed (+ DeltaSeconds (Variables|Default|GetTime%20Elapsed))))))))

(event Custom|startTimer
  (if (not (Variables|Default|Getended))
    (Variables|Default|Setstarted true)))

(event Custom|endTimer
  (if (Variables|Default|Getstarted)
    (Variables|Default|Setended true)))

(event Custom|setPauseOff
  ;[1 1 1] Comment
  (bind _running (CallFunction|IsRunning))
  (if _running
    (Variables|Default|Setpaused false)))

(event Custom|setPauseOn
  ;[1 1 1] Comment
  (bind _running (CallFunction|IsRunning))
  (if _running
    (Variables|Default|Setpaused true)))

(event Custom|setPauseToogle
  ;[1 1 1] Comment
  (bind _running (CallFunction|IsRunning))
  (if _running
    (Variables|Default|Setpaused (not (Variables|Default|Getpaused)))))

(event Custom|setPauseTo
  (params (pause :type Boolean))
  ;[1 1 1] Comment
  (bind _running (CallFunction|IsRunning))
  (if _running
    (Variables|Default|Setpaused pause)))

(fn IsRunning
  (return (and (Variables|Default|Getstarted) (not (Variables|Default|Getended)))))