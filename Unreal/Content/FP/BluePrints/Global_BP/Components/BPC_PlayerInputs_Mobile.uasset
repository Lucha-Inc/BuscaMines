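; Mobile input component that turns touches into square select and suspect actions on the game board.
; While enabled, it creates a BPO_Touch object for each of the first two fingers, tracked by finger index and fed move and release updates.
; Select and Suspect events line trace from screen position to a BP_Square and pass its coordinates to the PlayerController.
; Square lookup is blocked while the game mode is paused.
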(event Custom|Setup
  (params (Player%20Controller :type BP%20Player%20Controller%20Master%20Object%20Reference) (Enable :type Boolean))
  (bind _output_get (Variables|Default|SetPlayerController Player%20Controller))
  (Variables|/Script/Engine.PlayerController|SetbEnableTouchEvents _output_get true)
  (Variables|/Script/Engine.PlayerController|SetbEnableClickEvents _output_get true)
  (Variables|Default|SetEnable Enable)
  (bind _gamemode_master (CallFunction|GetCustomClasses self))
  (EventDispatchers|BindEventtoPauseChanged _gamemode_master (delegate Custom|onPauseChange))
  (Variables|Default|SetPaused (Default|IsPaused _gamemode_master)))

(event Custom|onPauseChange
  (params (PauseStatus :type Boolean))
  (Variables|Default|SetPaused PauseStatus))

(event EventBeginPlay)

(event EventTick
  (params (DeltaSeconds :type Float%20%28single-precision%29)))

(event Custom|Select
  (params (ScreenPosition :type Vector%202D%20Structure))
  (bind (_actor _validactor) (CallFunction|GetProjectEntitySquare ScreenPosition))
  (if _validactor
    (Default|BoardSelectSquare (Variables|Default|GetPlayerController) (Default|GetCoords _actor))))

(event Custom|Suspect
  (params (ScreenPosition :type Vector%202D%20Structure))
  (bind (_actor _validactor) (CallFunction|GetProjectEntitySquare ScreenPosition))
  (if _validactor
    (Default|BoardSuspectSquare (Variables|Default|GetPlayerController) (Default|GetCoords _actor))))

(event Input|TouchEvents|InputTouch
  (params (Location :type Vector) (FingerIndex :type ETouchIndex%20Enum))
  (bind _returnvalue (Math|Conversions|ToVector2D(Vector) Location))
  (bind _enable (Variables|Default|GetEnable))
  (bind _touchlist (Variables|Default|GetTouchList))
  (bind (_value _returnvalue_2) (Utilities|Map|Find _touchlist FingerIndex))
  (:Pressed
    (if _enable
      (switch Utilities|FlowControl|Switch|SwitchonETouchIndex FingerIndex
        (:Touch1
          _)
        (:Touch2
          _))
      (bind _returnvalue_3 (Game|ConstructObjectfromClass "/Game/FP/BluePrints/Clases/BPO_Touch.BPO_Touch_C" (Variables|Default|GetPlayerController) FingerIndex _returnvalue (Utilities|Time|GetRealTimeSeconds)))
      (Utilities|Map|Add (Variables|Default|GetTouchList) FingerIndex _returnvalue_3)))
  (:Released
    (if _enable
      (if _returnvalue_2
        (Default|Release _value _returnvalue (Utilities|Time|GetRealTimeSeconds))
        (Utilities|Map|Remove (Variables|Default|GetTouchList) FingerIndex))))
  (:Moved
    (if _enable
      (if _returnvalue_2
        (Default|Moved _value _returnvalue (Utilities|Time|GetRealTimeSeconds))))))

(fn GetProjectEntitySquare
  (params (ScreenPosition :type Vector%202D%20Structure))
  (bind _playercontroller (Variables|Default|GetPlayerController))
  (bind (_worldposition _worlddirection) (Class|GameplayStatics|DeprojectScreentoWorld _playercontroller ScreenPosition))
  (if (Variables|Default|GetPaused)
    (return 0 false)
    (else
      (bind _debugmode (CallFunction|GetDebugMode self))
      (bind _outhit (Collision|LineTraceByChannel _worldposition (+ _worldposition (* _worlddirection 10000)) "TraceTypeQuery4" false 0 (select _debugmode (Utilities|Enum|LiteralenumEDrawDebugTrace "ForDuration") (Utilities|Enum|LiteralenumEDrawDebugTrace "None"))))
      (bind _asbp_square (Utilities|Casting|CastToBP_Square (.hitactor _outhit))
        (:then
          (return _asbp_square true))
        (:CastFailed
          (return 0 false))))))

(fn GetTouchList
  (return (Variables|Default|GetTouchList)))