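; Game instance for the Minesweeper game that owns level flow and shared managers across maps.
; On Init it constructs the theme manager and fetches the app theme data asset, which feeds the lazily created app sound manager.
; Classic games open behind a fade-in widget, and restart replays the stored level config or returns to the menu.
; It also lazily spawns a hidden sound-class actor and exposes debug mode, disabled in distribution builds.
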(event EventInit
  (Utilities|FlowControl|Sequence
    (:then_0
      (switch string (Game|GetPlatformName)))
    (:then_1
      (bind _returnvalue (Game|ConstructObjectfromClass "/Game/FP/BluePrints/Global_BP/Managers/Theme/BP_ThemeManager.BP_ThemeManager_C"))
      (Variables|ManagersandDataAsset|SetTheme_Manager _returnvalue))
    (:then_2
      (Variables|Theme|SetDA%20Theme%20App (Default|GetDataAssetThemeApp (Variables|ManagersandDataAsset|GetTheme_Manager) "NewEnumerator0")))))

(event Custom|Go%20to%20level%20CLASSIC
  (params (Level%20Config :type Structu%20Level%20Configuration%20Structure))
  (Variables|Level|SetLast_level_config Level%20Config)
  (bind _returnvalue (UserInterface|CreateWidget "/Game/FP/GUI/Widgets/LevelTransition/LevelTransitio_FadeIn.LevelTransitio_FadeIn_C" (Game|GetPlayerController 0) true))
  (UserInterface|Viewport|AddtoViewport _returnvalue 0)
  (EventDispatchers|BindEventtoFadeinFinished _returnvalue (delegate Custom|createNewGameLevel)))

(event Custom|Go%20to%20level%20Main%20Menu
  (Game|OpenLevel(byObjectReference) "/Game/FP/Maps/menu_level.menu_level"))

(event Custom|Go%20to%20level%20Restart
  (bind _last_level_config (Variables|Level|GetLast_level_config))
  (bind _level (CallFunction|GetCurrentLevel))
  (switch Utilities|FlowControl|Switch|SwitchonEnum_Levels _level
    (:NewEnumerator0
      (CallFunction|GotoLevelMainMenu))
    (:NewEnumerator1
      (CallFunction|GotoLevelCLASSIC (Utilities|Struct|MakeStructu_Level_Configuration (.level_difficulty _last_level_config) (.level_theme _last_level_config) (.level_board_theme _last_level_config) "NewEnumerator1")))))

(event Custom|PlayBlackScreen
  (bind _returnvalue (UserInterface|CreateWidget "/Game/FP/GUI/Widgets/LevelTransition/LevelTransitio_BlackScreen.LevelTransitio_BlackScreen_C" (Game|GetPlayerController 0)))
  (UserInterface|Viewport|AddtoViewport _returnvalue 0))

(event Custom|PlayFadeOutLevel
  (Viewport|RemoveAllWidgets)
  (bind _returnvalue (UserInterface|CreateWidget "/Game/FP/GUI/Widgets/LevelTransition/LevelTransitio_FadeIn.LevelTransitio_FadeIn_C" (Game|GetPlayerController 0) false true))
  (UserInterface|Viewport|AddtoViewport _returnvalue 0))

(event Custom|createNewGameLevel
  (Game|OpenLevel(byObjectReference) "/Game/FP/Maps/game_level.game_level"))

(event Custom|SaveSoundClassesSetup
  (params (SoundClssesSetup :type Map%20of%20E_SoundClasses%20Enums%20to%20Structs :default "NewEnumerator0"))
  (Variables|Manager_Sound_Clsses|SetsoundClassesConfig SoundClssesSetup))

(fn GetLogOrder
  (bind _output_get (Variables|DEBUG|Setlog_counter (+ (Variables|DEBUG|Getlog_counter) 1)))
  (return _output_get))

(fn GetSoundClassManager
  (Utilities|IsValid (Variables|ManagerSoundClsses|GetSoundClass_Manager)
    (:Is%20Valid
      (return (Variables|ManagerSoundClsses|GetSoundClass_Manager)))
    (:Is%20Not%20Valid
      (bind _returnvalue (Game|SpawnActorfromClass "/Game/FP/BluePrints/Global_BP/Managers/Sound/BP_SoundClass_Manager.BP_SoundClass_Manager_C" (Math|Transform|MakeTransform "0, 0, 0") "AlwaysSpawn" "MultiplyWithRoot" 0 (Variables|Manager_Sound_Clsses|GetsoundClassesConfig) self 0))
      (Actor|SetLifeSpan _returnvalue 0.0)
      (Actor|Tick|SetActorTickEnabled _returnvalue)
      (Rendering|SetActorHiddenInGame _returnvalue true)
      (bind _output_get (Variables|ManagerSoundClsses|SetSoundClass_Manager _returnvalue))
      (return _output_get))))

(fn GetThemeManager
  (return (Variables|ManagersandDataAsset|GetTheme_Manager)))

(fn CreateAudio
  (params (Sound :type Sound%20Base%20Object%20Reference) (Persist :type Boolean) (Destroy :type Boolean))
  (bind _returnvalue (Audio|CreateSound2D Sound 1.0 1.0 0.0 0 Persist Destroy))
  (return _returnvalue))

(fn GetSoundManagerApp
  (Utilities|IsValid (Variables|ManagersAndDataAsset|GetSound_Manager_App)
    (:Is%20Valid
      (return (Variables|ManagersAndDataAsset|GetSound_Manager_App)))
    (:Is%20Not%20Valid
      (bind _returnvalue (Game|ConstructObjectfromClass "/Game/FP/BluePrints/Global_BP/Managers/Sound/BP_SoundClass_Manager_App.BP_SoundClass_Manager_App_C" (Variables|Theme|GetDA%20Theme%20App) self))
      (bind _output_get (Variables|ManagersAndDataAsset|SetSound_Manager_App _returnvalue))
      (return _output_get))))

(fn GetLastLevelConfig
  (return (Variables|Level|GetLast_level_config)))

(fn GetDebugMode
  (bind _returnvalue (Class|KismetSystemLibrary|IsPackagedforDistribution))
  (return (and (Variables|DEBUG|GetdebugMode) (not _returnvalue)) _returnvalue))

(fn SetDebugMode
  (params (debugMode :type Boolean))
  (Variables|DEBUG|SetdebugMode debugMode))

(fn GetCurrentLevel
  (bind _returnvalue (Game|GetCurrentLevelName true))
  (switch string _returnvalue
    (:Default
      _)
    (:menu_level
      (return "NewEnumerator0"))
    (:game_level
      _))
  (return "NewEnumerator1"))