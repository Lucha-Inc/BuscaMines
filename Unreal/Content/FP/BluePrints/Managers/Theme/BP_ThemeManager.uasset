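; BP_ThemeManager is a lookup manager for the game's Board, Level and App theme data assets.
; Each category has its own map and a getter that takes a theme key and returns the mapped entry.
; The getters return the Find value directly, without checking whether the key was found.
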(fn GetDataAssetThemeBoard
  (params (ThemeBoard :type Enum_Theme_Board%20Enum :default "NewEnumerator0"))
  (return (.Value (Utilities|Map|Find (Variables|Default|GetDA_Borad_List) ThemeBoard))))

(fn GetDataAssetThemeLevel
  (params (Theme%20Level :type Enum_Theme_Level%20Enum :default "NewEnumerator0"))
  (return (.Value (Utilities|Map|Find (Variables|Default|GetDA_Level_List) Theme%20Level))))

(fn GetDataAssetThemeApp
  (params (Theme%20App :type Enum_Theme_App%20Enum :default "NewEnumerator0"))
  (return (.Value (Utilities|Map|Find (Variables|Default|GetDA_App_List) Theme%20App))))