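; Player movement helper Blueprint that smoothly moves its parent actor to a target transform over a requested number of seconds.
; PlayMovement stores the parent's current transform and the target, then rescales the timeline play rate from a default duration to fit the requested time.
; Each timeline update lerps between the two transforms, applying only location and rotation, and completion fires MovementFinished.
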(event EventBeginPlay)

(event Collision|EventActorBeginOverlap
  (params (OtherActor :type Actor%20Object%20Reference)))

(event EventTick
  (params (DeltaSeconds :type Float%20%28single-precision%29)))

(event Custom|PlayMovement
  (params (To :type Transform) (inSeconds :type Float%20%28double-precision%29))
  (Components|Timeline|SetPlayRate (Variables|Default|GetTL_Movement) (/ (Variables|Default|GetdefaultDuration) inSeconds))
  (Variables|Default|SetendPosition To)
  (Variables|Default|SetiniPosition (Transformation|GetActorTransform (Actor|GetParentActor)))
  (bind _newtrack_0 (Timeline|TL_Movement Play)
    (:Update
      (Transformation|SetActorLocationAndRotation (Actor|GetParentActor) (.location (Math|Transform|Lerp(Transform) (Variables|Default|GetiniPosition) (Variables|Default|GetendPosition) _newtrack_0)) (Math|Rotator|MakeRotator (.roll (.rotation (Math|Transform|Lerp(Transform) (Variables|Default|GetiniPosition) (Variables|Default|GetendPosition) _newtrack_0))) (.pitch (.rotation (Math|Transform|Lerp(Transform) (Variables|Default|GetiniPosition) (Variables|Default|GetendPosition) _newtrack_0))) (.yaw (.rotation (Math|Transform|Lerp(Transform) (Variables|Default|GetiniPosition) (Variables|Default|GetendPosition) _newtrack_0))))))
    (:Finished
      (Default|CallMovementFinished))))

(fn ConstructionScript)