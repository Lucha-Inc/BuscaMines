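; Environment manager that hosts a PCG master as a child actor and signals when the environment is ready.
; On BeginPlay it binds to the master's PCG-generated event and calls environment ready when that fires.
; Debug mode skips the binding and signals readiness after a short delay.
; A Generate event triggers the master's PCG generation, while the location and bound-actor functions return false and empty.
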(event Custom|PCG_generated
  (Default|CallEnviromentReady))

(event EventBeginPlay
  (bind _debugmode (CallFunction|GetDebugMode self))
  (if _debugmode
    (Utilities|FlowControl|Delay 0.2)
    (Default|CallEnviromentReady)
    (else
      (bind _asa_pcg_master (Utilities|Casting|CastToA_PCG_Master (Variables|/Script/Engine.ChildActorComponent|GetChildActor (Variables|Default|GetPCG_Actor))))
      (EventDispatchers|BindEventtoPCGGenerated _asa_pcg_master (delegate Custom|PCG_generated)))))

(event Collision|EventActorBeginOverlap
  (params (OtherActor :type Actor%20Object%20Reference)))

(event EventTick
  (params (DeltaSeconds :type Float%20%28single-precision%29)))

(event Custom|Generate
  (bind _asa_pcg_master (Utilities|Casting|CastToA_PCG_Master (Variables|/Script/Engine.ChildActorComponent|GetChildActor (Variables|Default|GetPCG_Actor))))
  (Default|GeneratePCG _asa_pcg_master))

(fn ConstructionScript)

(fn HasFixedLocation
  (return false))

(fn GetBoundActor
  (return 0))