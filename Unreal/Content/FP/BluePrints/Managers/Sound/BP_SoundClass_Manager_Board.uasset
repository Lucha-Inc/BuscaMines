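; Board sound manager for a Minesweeper-style game, providing sounds for square selection, flag creation and removal, and mine explosion.
; Each Play function creates a non-persistent sound from the board theme data asset and returns it.
; Flag removal reuses the flag creation sound.
; MuteBoard and UnmuteBoard toggle one sound class through the shared sound class manager.
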(event Custom|MuteBoard
  (bind _sound_class_manager (CallFunction|GetSoundClassManager))
  (Default|SetMute _sound_class_manager "NewEnumerator4" true))

(event Custom|UnmuteBoard
  (bind _sound_class_manager (CallFunction|GetSoundClassManager))
  (Default|SetMute _sound_class_manager "NewEnumerator4" false))

(fn PlaySquareSelected
  (bind _audio_component (CallFunction|CreatePlaySound (Variables|/Game/FP/Data/DataAsset/Board/DA_ThemeData_Board.DA_ThemeData_Board_C|Getsound_square_selected (Variables|DataAsset|GetDA%20Theme%20Board)) 0 false true 0.0))
  (return _audio_component))

(fn PlayFlagCreation
  (bind _audio_component (CallFunction|CreatePlaySound (Variables|/Game/FP/Data/DataAsset/Board/DA_ThemeData_Board.DA_ThemeData_Board_C|Getsound_flag_create (Variables|DataAsset|GetDA%20Theme%20Board)) 0 false true 0.0))
  (return _audio_component))

(fn PlayFlagRemove
  (bind _audio_component (CallFunction|CreatePlaySound (Variables|/Game/FP/Data/DataAsset/Board/DA_ThemeData_Board.DA_ThemeData_Board_C|Getsound_flag_create (Variables|DataAsset|GetDA%20Theme%20Board)) 0 false true 0.0))
  (return _audio_component))

(fn PlayMineExplote
  (bind _audio_component (CallFunction|CreatePlaySound (Variables|/Game/FP/Data/DataAsset/Board/DA_ThemeData_Board.DA_ThemeData_Board_C|Getsound_square_explote (Variables|DataAsset|GetDA%20Theme%20Board)) 0 false true 0.0))
  (return _audio_component))