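; BP_SoundClass_Manager_Master is a sound manager that provides helper functions for creating, playing and stopping audio components.
; Creation is delegated to the GameInstance, with persist and auto-destroy options, and writes the component into a by-ref variable.
; Play wraps creation with a fade-in, while stop fades valid components out on an S-curve.
; A getter returns the GameInstance's sound class manager.
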(fn CreateAudioComponent
  (params (Sound%20base :type Sound%20Base%20Object%20Reference) (AudioComponent%20Variable :type Audio%20Component%20Object%20Reference%20%28by%20ref%29) (Persist :type Boolean) (AutoDestroy :type Boolean))
  (bind _audio_component (Default|CreateAudio (Variables|Default|GetGameInstance) Sound%20base Persist AutoDestroy))
  (|SetBy-RefVar AudioComponent%20Variable _audio_component)
  (return _audio_component))

(fn CreatePlaySound
  (params (Sound :type Sound%20Base%20Object%20Reference) (Audio%20Component%20Variable :type Audio%20Component%20Object%20Reference%20%28by%20ref%29) (Persist :type Boolean) (AutoDestroy :type Boolean) (FadeIn :type Float%20%28double-precision%29))
  (bind _audio_component (CallFunction|CreateAudioComponent Sound Audio%20Component%20Variable Persist AutoDestroy))
  (Audio|Components|Audio|FadeIn _audio_component FadeIn 1.0 0.0 "SCurve" :!class /Script/Engine.AudioComponent)
  (return _audio_component))

(fn StopAudioComponent
  (params (Audio%20Component :type Audio%20Component%20Object%20Reference) (FadeOut :type Float%20%28double-precision%29))
  (Utilities|IsValid Audio%20Component
    (:Is%20Valid
      (Audio|Components|Audio|FadeOut Audio%20Component FadeOut 0.0 "SCurve" :!class /Script/Engine.AudioComponent)
      (return Audio%20Component))))

(fn GetSoundClassManager
  (bind _soundmanager (Default|GetSoundClassManager (Variables|Default|GetGameInstance)))
  (return _soundmanager))