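; Base actor for clickable 3D text menu buttons, showing its label through a BP_Text3D_Button child actor set in construction.
; Shortly after BeginPlay it sizes its click Box to the text bounds divided by world scale, as the text is already scaled.
; A click plays the UI sound, fires the 3DButtonOnClick dispatcher and runs an empty OnClick hook.
; A goToMenu helper switches menus through the BPI_GameMode_Master interface.
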(event OnClicked(Box)
  (params (TouchedComponent :type Primitive%20Component%20Object%20Reference) (ButtonPressed :type Key%20Structure :default "None"))
  (CallFunction|PlayClickSound)
  (Default|Call3DButtononClick)
  (CallFunction|OnClick))

(event Custom|goToMenu
  (params (toMenu :type BP%20Actor%20Menu%203D%20Class%20Reference))
  (if (Utilities|IsValidClass toMenu)
    (bind _asbpi_game_mode_master (Utilities|Casting|CastToBPI_GameMode_Master (Game|GetGameMode)))
    (Default|GotoMenu _asbpi_game_mode_master toMenu)))

(event Custom|setup
  (bind _text3d (Variables|Btn|Gettext3D))
  (bind _text3d_2 (Variables|/Game/FP/GUI/UserWidgets/ActorsWidgets/Instance/BP_Text3D_Button.BP_Text3D_Button_C|GetText3D _text3d))
  ;[1 1 1] Cuando ocurre, el objeto ya fué escalado y nosotros lo dimensionamos con unas medidas sin escalar
  (Components|Box|SetBoxExtent (Variables|Default|GetBox) (/ (.BoxExtent (Class|Text3DComponent|GetBounds _text3d_2)) (.scale (Transformation|GetWorldTransform _text3d_2))) true))

(event EventBeginPlay
  (Utilities|FlowControl|Delay 0.2)
  (CallFunction|Setup))

(event Custom|PlayClickSound
  (bind _gameinstance (CallFunction|GetCustomClasses self))
  (bind _sound_manager_app (Default|GetSoundManagerApp _gameinstance))
  (Default|PlayUIButtonClick _sound_manager_app))

(fn ConstructionScript
  (Utilities|FlowControl|Sequence
    (:then_0
      (bind _asbp_menu_text_3d_button (Utilities|Casting|CastToBP_Text3D_Button (Variables|/Script/Engine.ChildActorComponent|GetChildActor (Variables|Default|GetBP_Menu_Text3D_Button))))
      (bind _output_get (Variables|Btn|Settext3D _asbp_menu_text_3d_button))
      (Default|SetText _output_get (Variables|Btn|Getbtn_text)))))

(fn OnClick)