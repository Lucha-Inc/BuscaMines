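; Player controller for a first-person Minesweeper-style board game, handling board, movement, pause and 3D menu input.
; Each tick a camera line trace finds and outlines the viewed BP_Square, whose coordinates feed the Board's select and suspect-mine actions.
; Movement follows the board's direction vector plus vertical input, and looking rotates the character actor directly.
; Menu calls forward to the character's menu component; bounds are stored, but their edge-slowdown logic is disconnected.
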(event Custom|Setup
  (params (Board :type BP%20Board%20Master%20Object%20Reference))
  (Utilities|FlowControl|Sequence
    (:then_0
      ;[1 1 1] Set BPC Menu Controller
      (bind _asbp_player (Utilities|Casting|CastToBP_player (Game|GetPlayerCharacter 0)))
      (bind _output_get (Variables|Menu3D|SetMenu3D_Controller (Variables|/Game/FP/BluePrints/Chareacters/Player/BP_player.BP_player_C|GetBPC_Player_Menu_Controller _asbp_player)))
      (Default|Setup _output_get))
    (:then_1
      ;[1 1 1] Setup ResolutionController
      (Default|Setup (Variables|Default|GetBPC_PlayerController_ResulutionChange)))
    (:then_2
      ;[1 1 1] Set Board
      (Variables|Board|SetBoard Board))))

(event EventBeginPlay)

(event EventTick
  (params (DeltaSeconds :type Float%20%28single-precision%29))
  (bind _self self)
  ;[1 1 1] Consulta que Casilla se está visualizando
  (bind (_startpoint _endpoint) (CallFunction|LineTracePointfromActor (Variables|Default|GetPlayerCameraManager _self) 1e+02))
  (bind _outhit (Collision|LineTraceByChannel _startpoint _endpoint "TraceTypeQuery4" false (Utilities|Array|MakeArray (Pawn|GetControlledPawn _self) 0) "None"))
  (bind _asbp_square (Utilities|Casting|CastToBP_Square (.hitactor _outhit))
    (:then
      _)
    (:CastFailed
      _))
  (CallFunction|SetSquare _asbp_square))

(event Input|EnhancedActionEvents|EnhancedInputActionboard_selection
  (params (ActionValue :type Boolean) (ElapsedSeconds :type Float%20%28double-precision%29) (TriggeredSeconds :type Float%20%28double-precision%29) (InputAction :type Input%20Action%20Object%20Reference :default "/Game/FP/BluePrints/Global_BP/Inputs/board_selection.board_selection"))
  (bind _currentsquare (Variables|Board|GetCurrentSquare))
  ;[1 1 1] Selecciona una Casilla
  (if (Utilities|IsValid _currentsquare)
    (Default|SelectSquare (Variables|Board|GetBoard) (Default|GetCoords _currentsquare))))

(event Input|EnhancedActionEvents|EnhancedInputActionboard_suspectMine
  (params (ActionValue :type Boolean) (ElapsedSeconds :type Float%20%28double-precision%29) (TriggeredSeconds :type Float%20%28double-precision%29) (InputAction :type Input%20Action%20Object%20Reference :default "/Game/FP/BluePrints/Global_BP/Inputs/board_suspectMine.board_suspectMine"))
  (bind _currentsquare (Variables|Board|GetCurrentSquare))
  ;[1 1 1] Sospecha una Casilla
  (if (Utilities|IsValid _currentsquare)
    (Default|SuspectSquare (Variables|Board|GetBoard) (Default|GetCoords _currentsquare))))

(event Input|EnhancedActionEvents|EnhancedInputActiongaming_pause
  (params (ActionValue :type Boolean) (ElapsedSeconds :type Float%20%28double-precision%29) (TriggeredSeconds :type Float%20%28double-precision%29) (InputAction :type Input%20Action%20Object%20Reference :default "/Game/FP/BluePrints/Global_BP/Inputs/gaming_pause.gaming_pause"))
  (bind _asbpi_game_mode_master (Utilities|Casting|CastToBPI_GameMode_Master (Game|GetGameMode)))
  (Default|OnPause _asbpi_game_mode_master))

(event Input|EnhancedActionEvents|EnhancedInputActiongaming_ESC
  (params (ActionValue :type Boolean) (ElapsedSeconds :type Float%20%28double-precision%29) (TriggeredSeconds :type Float%20%28double-precision%29) (InputAction :type Input%20Action%20Object%20Reference :default "/Game/FP/BluePrints/Global_BP/Inputs/gaming_ESC.gaming_ESC")))

(event Input|EnhancedActionEvents|EnhancedInputActionplayer_movement
  (params (ActionValue :type Vector%202D%20Structure) (ElapsedSeconds :type Float%20%28double-precision%29) (TriggeredSeconds :type Float%20%28double-precision%29) (InputAction :type Input%20Action%20Object%20Reference :default "/Game/FP/BluePrints/Global_BP/Inputs/player_movement.player_movement"))
  (bind _returnvalue (Game|GetPlayerCharacter 0))
  (bind _gamemode_master (CallFunction|GetCustomClasses self))
  (bind _directionvector (Default|GetBoardDirectionVector (Variables|/Game/FP/BluePrints/Global_BP/BP_Abstract_GameMode_Master.BP_Abstract_GameMode_Master_C|GetBoard_Master _gamemode_master)))
  (Utilities|FlowControl|Sequence
    (:then_0
      (Pawn|Input|AddMovementInput _returnvalue (Math|Vector|MakeVector (* (.Y (Math|Vector|BreakVector _directionvector)) -1.0) (.X (Math|Vector|BreakVector _directionvector)) 0.0) (.x ActionValue) false))
    (:then_1
      (Pawn|Input|AddMovementInput _returnvalue _directionvector (.y ActionValue) false))))

(event Input|EnhancedActionEvents|EnhancedInputActionplayer_looking
  (params (ActionValue :type Vector%202D%20Structure) (ElapsedSeconds :type Float%20%28double-precision%29) (TriggeredSeconds :type Float%20%28double-precision%29) (InputAction :type Input%20Action%20Object%20Reference :default "/Game/FP/BluePrints/Global_BP/Inputs/player_looking.player_looking"))
  (bind _returnvalue (Game|GetPlayerCharacter 0))
  ;[1 1 1] Movement
  (Class|Actor|AddActorWorldRotation _returnvalue (Math|Rotator|MakeRotator 0.0 0.0 (.x ActionValue)))
  (Transformation|AddActorLocalRotation _returnvalue (Math|Rotator|MakeRotator 0.0 (.y ActionValue) 0.0) false false))

(event Input|EnhancedActionEvents|EnhancedInputActionplayer_up_down
  (params (ActionValue :type Float%20%28double-precision%29) (ElapsedSeconds :type Float%20%28double-precision%29) (TriggeredSeconds :type Float%20%28double-precision%29) (InputAction :type Input%20Action%20Object%20Reference :default "/Game/FP/BluePrints/Global_BP/Inputs/player_up_down.player_up_down"))
  ;[1 1 1] Movement
  (Pawn|Input|AddMovementInput (Game|GetPlayerCharacter 0) "0.000000,0.000000,1.000000" ActionValue false))

(event EventSetBounds
  (params (bounds_box :type Box%20Structure) (bounds_external_margin :type Float%20%28double-precision%29) (bounds_internal_offset :type Float%20%28double-precision%29) (bounds_active :type Boolean))
  ;[1 1 1] Setup Player Bounds
  (Variables|Bounds|Setbounds_box (Math|Box|MakeBox (- (.min bounds_box) bounds_external_margin) (+ (.max bounds_box) bounds_external_margin)))
  (Variables|Bounds|Setbounds_offset bounds_internal_offset)
  (Variables|Bounds|Setbounds_active bounds_active))

(event Input|EnhancedActionEvents|EnhancedInputActionmenu_moving_sides
  (params (ActionValue :type Float%20%28double-precision%29) (ElapsedSeconds :type Float%20%28double-precision%29) (TriggeredSeconds :type Float%20%28double-precision%29) (InputAction :type Input%20Action%20Object%20Reference :default "/Game/FP/BluePrints/Global_BP/Inputs/menu_moving_sides.menu_moving_sides"))
  (CallFunction|Log 0 (Utilities|String|ToString(Float) ActionValue)))

(event Input|EnhancedActionEvents|EnhancedInputActionmenu_scroll
  (params (ActionValue :type Float%20%28double-precision%29) (ElapsedSeconds :type Float%20%28double-precision%29) (TriggeredSeconds :type Float%20%28double-precision%29) (InputAction :type Input%20Action%20Object%20Reference :default "/Game/FP/BluePrints/Global_BP/Inputs/menu_scroll.menu_scroll"))
  (Default|OnScroll (Variables|Menu3D|GetMenu3D_Controller) ActionValue))

(event EventClearMenus
  (Default|ClearMenus (Variables|Menu3D|GetMenu3D_Controller)))

(event EventShowMenu3D
  (params (Menu%203D%20Class :type BP%20Actor%20Menu%203D%20Class%20Reference))
  (Default|SetMenu3D (Variables|Menu3D|GetMenu3D_Controller) Menu%203D%20Class))

(fn ConstructionScript)

(fn SetSquare
  (params (newSquare :type BP%20Square%20Object%20Reference))
  (if (== newSquare (Variables|Board|GetCurrentSquare))
    (return false)
    (else
      (if (Utilities|IsValid (Variables|Board|GetCurrentSquare))
        (Default|SetOutlineonView (Variables|Board|GetCurrentSquare) false))
      (if (Utilities|IsValid newSquare)
        (bind _output_get (Variables|Board|SetCurrentSquare newSquare))
        (Default|SetOutlineonView _output_get true)
        (else
          (Variables|Board|SetCurrentSquare 0)))
      (return true))))