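; Mobile player controller that turns touch input into board-square and movement actions.
; The first two fingers each get a BPO_Touch object, tracked in TouchList, updated on move, and released and removed on lift.
; Select and Suspect events line-trace from screen position to a BP_Square, blocked while paused, and pass its coords to board actions.
; Move_XY remaps a swipe vector into player movement; debug mode draws the traces.
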(event EventBeginPlay
  (|CallParentFunction)
  (Variables|Default|SetbEnableTouchEvents true)
  (Variables|Default|SetbEnableClickEvents true))

(event EventTick
  (params (DeltaSeconds :type Float%20%28single-precision%29)))

(event EventActorOnInputTouchBegin
  (params (FingerIndex :type ETouchIndex%20Enum :default "Touch1"))
  (CallFunction|Log 0 (Utilities|String|EnumtoString FingerIndex)))

(event Input|TouchEvents|InputTouch
  (params (Location :type Vector) (FingerIndex :type ETouchIndex%20Enum))
  (bind _returnvalue (Math|Conversions|ToVector2D(Vector) Location))
  (bind _touchlist (Variables|Default|GetTouchList))
  (bind (_value _returnvalue_2) (Utilities|Map|Find _touchlist FingerIndex))
  (:Pressed
    (switch Utilities|FlowControl|Switch|SwitchonETouchIndex FingerIndex
      (:Touch1
        _)
      (:Touch2
        _))
    (bind _returnvalue_3 (Game|ConstructObjectfromClass "/Game/FP/BluePrints/Clases/BPO_Touch.BPO_Touch_C" self FingerIndex _returnvalue (Utilities|Time|GetRealTimeSeconds)))
    (Utilities|Map|Add (Variables|Default|GetTouchList) FingerIndex _returnvalue_3))
  (:Released
    (if _returnvalue_2
      (Default|Release _value _returnvalue (Utilities|Time|GetRealTimeSeconds))
      (Utilities|Map|Remove (Variables|Default|GetTouchList) FingerIndex)))
  (:Moved
    (if _returnvalue_2
      (Default|Moved _value _returnvalue (Utilities|Time|GetRealTimeSeconds)))))

(event Custom|Select
  (params (ScreenPosition :type Vector%202D%20Structure))
  (bind (_actor _validactor) (CallFunction|GetProjectEntitySquare ScreenPosition))
  (if _validactor
    (CallFunction|BoardSelectSquare (Default|GetCoords _actor))))

(event Custom|Suspect
  (params (ScreenPosition :type Vector%202D%20Structure))
  (bind (_actor _validactor) (CallFunction|GetProjectEntitySquare ScreenPosition))
  (if _validactor
    (CallFunction|BoardSuspectSquare (Default|GetCoords _actor))))

(event Custom|Move_XY
  (params (SwipeVector :type Vector%202D%20Structure))
  (CallFunction|PlayerMoveXY (.y SwipeVector) (* (.x SwipeVector) -1.0)))

(fn ConstructionScript
  (|CallParentFunction))

(fn GetProjectEntitySquare
  (params (ScreenPosition :type Vector%202D%20Structure))
  (bind _self self)
  (bind (_worldposition _worlddirection) (Class|GameplayStatics|DeprojectScreentoWorld _self ScreenPosition))
  (if (Default|IsPaused (Variables|Default|GetGameMode))
    (return 0 false)
    (else
      (bind _debugmode (CallFunction|GetDebugMode self))
      (bind _outhit (Collision|LineTraceByChannel _worldposition (+ _worldposition (* _worlddirection 10000)) "TraceTypeQuery4" false 0 (select _debugmode (Utilities|Enum|LiteralenumEDrawDebugTrace "ForDuration") (Utilities|Enum|LiteralenumEDrawDebugTrace "None"))))
      (bind _asbp_square (Utilities|Casting|CastToBP_Square (.hitactor _outhit))
        (:then
          (return _asbp_square true))
        (:CastFailed
          (return 0 false))))))

(fn GetTouchList
  (return (Variables|Default|GetTouchList)))