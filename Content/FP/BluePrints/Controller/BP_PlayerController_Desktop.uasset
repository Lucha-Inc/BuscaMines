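; Desktop player controller for a Minesweeper-style board game, tracking and outlining the board square under the mouse cursor.
; While unpaused, Tick runs a cursor trace and SetSquare moves the outline when the hovered square changes.
; Enhanced Input handlers cover square selection, mine suspicion, pause, movement, look and menus, but all sit behind constant-false branches.
; An alternative camera-forward line trace remains unconnected.
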(event EventBeginPlay
  (|CallParentFunction))

(event EventTick
  (params (DeltaSeconds :type Float%20%28single-precision%29))
  ;[1 1 1] Consulta que Casilla se está visualizando
  (if (not (Default|IsPaused (Variables|Default|GetGameMode)))
    (bind _asbp_square (Utilities|Casting|CastToBP_Square (.hitactor (.HitResult (Game|Player|GetHitResultUnderCursorbyChannel "TraceTypeQuery4" true))))
      (:then
        _)
      (:CastFailed
        _))
    (CallFunction|SetSquare _asbp_square)))

(event Input|EnhancedActionEvents|EnhancedInputActionmenu_moving_sides
  (params (ActionValue :type Float%20%28double-precision%29) (ElapsedSeconds :type Float%20%28double-precision%29) (TriggeredSeconds :type Float%20%28double-precision%29) (InputAction :type Input%20Action%20Object%20Reference :default "/Game/FP/BluePrints/Global_BP/Inputs/menu_moving_sides.menu_moving_sides"))
  (if false
    (CallFunction|Log 0 (Utilities|String|ToString(Float) ActionValue))))

(event Input|EnhancedActionEvents|EnhancedInputActionmenu_scroll
  (params (ActionValue :type Float%20%28double-precision%29) (ElapsedSeconds :type Float%20%28double-precision%29) (TriggeredSeconds :type Float%20%28double-precision%29) (InputAction :type Input%20Action%20Object%20Reference :default "/Game/FP/BluePrints/Global_BP/Inputs/menu_scroll.menu_scroll"))
  (if false
    (CallFunction|MenuScroll ActionValue)))

(event Input|EnhancedActionEvents|EnhancedInputActionplayer_up_down
  (params (ActionValue :type Float%20%28double-precision%29) (ElapsedSeconds :type Float%20%28double-precision%29) (TriggeredSeconds :type Float%20%28double-precision%29) (InputAction :type Input%20Action%20Object%20Reference :default "/Game/FP/BluePrints/Global_BP/Inputs/player_up_down.player_up_down"))
  (if false
    (CallFunction|PlayerMoveZ ActionValue)))

(event Input|EnhancedActionEvents|EnhancedInputActiongaming_pause
  (params (ActionValue :type Boolean) (ElapsedSeconds :type Float%20%28double-precision%29) (TriggeredSeconds :type Float%20%28double-precision%29) (InputAction :type Input%20Action%20Object%20Reference :default "/Game/FP/BluePrints/Global_BP/Inputs/gaming_pause.gaming_pause"))
  (if false
    (CallFunction|OnPause)))

(event Input|EnhancedActionEvents|EnhancedInputActionboard_suspectMine
  (params (ActionValue :type Boolean) (ElapsedSeconds :type Float%20%28double-precision%29) (TriggeredSeconds :type Float%20%28double-precision%29) (InputAction :type Input%20Action%20Object%20Reference :default "/Game/FP/BluePrints/Global_BP/Inputs/board_suspectMine.board_suspectMine"))
  (bind _currentsquare (Variables|Board|GetCurrentSquare))
  ;[1 1 1] Sospecha una Casilla
  (if false
    (if (Utilities|IsValid _currentsquare)
      (CallFunction|BoardSuspectSquare (Default|GetCoords _currentsquare)))))

(event Input|EnhancedActionEvents|EnhancedInputActionboard_selection
  (params (ActionValue :type Boolean) (ElapsedSeconds :type Float%20%28double-precision%29) (TriggeredSeconds :type Float%20%28double-precision%29) (InputAction :type Input%20Action%20Object%20Reference :default "/Game/FP/BluePrints/Global_BP/Inputs/board_selection.board_selection"))
  (bind _currentsquare (Variables|Board|GetCurrentSquare))
  ;[1 1 1] Selecciona una Casilla
  (if false
    (if (Utilities|IsValid _currentsquare)
      (CallFunction|BoardSelectSquare (Default|GetCoords _currentsquare)))))

(event Input|EnhancedActionEvents|EnhancedInputActiongaming_ESC
  (params (ActionValue :type Boolean) (ElapsedSeconds :type Float%20%28double-precision%29) (TriggeredSeconds :type Float%20%28double-precision%29) (InputAction :type Input%20Action%20Object%20Reference :default "/Game/FP/BluePrints/Global_BP/Inputs/gaming_ESC.gaming_ESC"))
  (if false
    (CallFunction|OnPause)))

(event Input|EnhancedActionEvents|EnhancedInputActionplayer_movement
  (params (ActionValue :type Vector%202D%20Structure) (ElapsedSeconds :type Float%20%28double-precision%29) (TriggeredSeconds :type Float%20%28double-precision%29) (InputAction :type Input%20Action%20Object%20Reference :default "/Game/FP/BluePrints/Global_BP/Inputs/player_movement.player_movement"))
  (if false
    (CallFunction|PlayerMoveXY (.x ActionValue) (.y ActionValue))))

(event Input|EnhancedActionEvents|EnhancedInputActionplayer_looking
  (params (ActionValue :type Vector%202D%20Structure) (ElapsedSeconds :type Float%20%28double-precision%29) (TriggeredSeconds :type Float%20%28double-precision%29) (InputAction :type Input%20Action%20Object%20Reference :default "/Game/FP/BluePrints/Global_BP/Inputs/player_looking.player_looking"))
  (if false
    (CallFunction|PlayerLook (.x ActionValue) (.y ActionValue))))

(fn ConstructionScript)

(fn SetSquare
  (params (newSquare :type BP%20Square%20Object%20Reference))
  (if (== newSquare (Variables|Board|GetCurrentSquare))
    (return false)
    (else
      (if (Utilities|IsValid (Variables|Board|GetCurrentSquare))
        (Default|SetOutlineonView (Variables|Board|GetCurrentSquare) false))
      (if (Utilities|IsValid newSquare)
        (bind _output_get (Variables|Board|SetCurrentSquare newSquare))
        (Default|SetOutlineonView _output_get true)
        (else
          (Variables|Board|SetCurrentSquare 0)))
      (return true))))