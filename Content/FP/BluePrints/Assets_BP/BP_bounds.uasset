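; BP_bounds is a box volume actor that answers containment and overlap queries, visible in game only in debug mode.
; IsOutterOf transforms two opposite corners of an actor's bounds into box space and compares them to the scaled extent minus an offset.
; Overlap checks test another bounds actor's box or filter overlapping BP_bounds by tag.
; Getters expose extent, origin and rotation, though GetBoundBox computes BoxMin as extent minus location.
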(event EventBeginPlay
  (bind _debugmode (CallFunction|GetDebugMode self))
  (Development|SetHiddeninGame (Variables|Default|GetBounds) (not _debugmode) false))

(event Collision|EventActorBeginOverlap
  (params (OtherActor :type Actor%20Object%20Reference)))

(event EventTick
  (params (DeltaSeconds :type Float%20%28single-precision%29)))

(fn ConstructionScript)

(fn GetBoundBox
  (bind _bounds (Variables|Default|GetBounds))
  (bind _returnvalue (Transformation|GetWorldRotation _bounds))
  (bind _returnvalue_2 (Transformation|GetWorldLocation _bounds))
  (bind _boxextent (Variables|/Script/Engine.BoxComponent|GetBoxExtent _bounds))
  (return (Math|Box|MakeBox (- _boxextent _returnvalue_2) (+ _boxextent _returnvalue_2)) _returnvalue_2 (Math|Vector|GetForwardVector _returnvalue) _returnvalue))

(fn GetBoundBoxCollision
  (return (Variables|Default|GetBounds)))

(fn IsOutterOf
  (params (inner :type BP%20Bounds%20Object%20Reference) (offset :type Vector))
  (bind (_origin _boxextent) (Collision|GetActorBounds inner false false))
  (bind _bounds (Variables|Default|GetBounds))
  (bind _returnvalue (Transformation|GetWorldTransform _bounds))
  (bind _returnvalue_2 (Components|Box|GetUnscaledBoxExtent _bounds))
  (bind _returnvalue_3 (+ _origin _boxextent))
  (bind _returnvalue_4 (- _origin _boxextent))
  (bind _scale (Math|Transform|BreakTransform _returnvalue))
  (bind _returnvalue_5 (Math|Transform|InverseTransformLocation _returnvalue _returnvalue_4))
  (bind _returnvalue_6 (Math|Transform|InverseTransformLocation _returnvalue _returnvalue_3))
  (bind _returnvalue_7 (* _returnvalue_2 _scale))
  (bind _returnvalue_8 (- _returnvalue_7 offset))
  (return (Math|Boolean|ANDBoolean (<= (Math|Float|Absolute(Float) (.x _returnvalue_6)) (.x _returnvalue_8)) (<= (Math|Float|Absolute(Float) (.y _returnvalue_6)) (.y _returnvalue_8)) (<= (Math|Float|Absolute(Float) (.z _returnvalue_6)) (.z _returnvalue_8)) (<= (Math|Float|Absolute(Float) (.x _returnvalue_5)) (.x _returnvalue_8)) (<= (Math|Float|Absolute(Float) (.y _returnvalue_5)) (.y _returnvalue_8)) (<= (Math|Float|Absolute(Float) (.z _returnvalue_5)) (.z _returnvalue_8)))))

(fn Overlapwith
  (params (BoundActor :type BP%20Bounds%20Object%20Reference))
  (return (Class|PrimitiveComponent|IsOverlappingComponent (Variables|Default|GetBounds) (CallFunction|GetBoundBoxCollision BoundActor))))

(fn IsOverlapedbyTag
  (params (tag :type Name))
  (bind _overlappingactors (CallFunction|EvaluateOverlappingbyTag tag))
  (return (> (Utilities|Array|Length _overlappingactors) 0)))

(fn EvaluateOverlappingbyTag
  (params (TAG :type Name))
  (for _array_element (Collision|GetOverlappingActors (Variables|Default|GetBounds) "BP_bounds_C" :!class /Script/Engine.PrimitiveComponent)
    (if (Actor|ActorHasTag _array_element TAG)
      (Utilities|Array|Add (LocalVariables|GetoverlappingActors) _array_element)))
  (bind _output_get (Variables|Default|Setoverlapping (LocalVariables|GetoverlappingActors)))
  (return _output_get))

(fn GetScaledExtent
  (bind _bounds (Variables|Default|GetBounds))
  (return (* (Variables|/Script/Engine.BoxComponent|GetBoxExtent _bounds) (Transformation|GetWorldScale _bounds))))