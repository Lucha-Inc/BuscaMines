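; Item display actor that presents either a static mesh or a spawned actor, with optional scale and rotation effects.
; The construction script adds a mesh component when a static mesh is set, otherwise spawns the given actor class.
; BeginPlay drives scale from a Timeline when enabled.
; Tick slowly yaws the mesh, but for a spawned actor it sets rather than adds the per-frame yaw, so rotation does not accumulate.
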(event EventBeginPlay
  (bind _actor (Variables|Default|GetActor))
  (if (and (Variables|Default|GeteffectScale) (CallFunction|IsValid))
    (bind _newtrack_0 (Timeline|Timeline Play)
      (:Update
        (Utilities|IsValid (Variables|Default|GetMeshComponent)
          (:Is%20Valid
            (Transformation|SetRelativeScale3D (Variables|Default|GetMeshComponent) (Math|Conversions|ToVector(Float) _newtrack_0)))
          (:Is%20Not%20Valid
            (Utilities|IsValid _actor
              (:Is%20Valid
                (Transformation|SetActorRelativeScale3D _actor (Math|Conversions|ToVector(Float) _newtrack_0))))))))))

(event Collision|EventActorBeginOverlap
  (params (OtherActor :type Actor%20Object%20Reference)))

(event EventTick
  (params (DeltaSeconds :type Float%20%28single-precision%29))
  (bind _returnvalue (* DeltaSeconds 1e+01))
  (bind _actor (Variables|Default|GetActor))
  (bind _meshcomponent (Variables|Default|GetMeshComponent))
  (if (and (Variables|Default|GeteffectRotate) (CallFunction|IsValid))
    (Utilities|IsValid _meshcomponent
      (:Is%20Valid
        (Transformation|AddRelativeRotation _meshcomponent (Math|Rotator|MakeRotator 0.0 0.0 _returnvalue) false false))
      (:Is%20Not%20Valid
        (Utilities|IsValid _actor
          (:Is%20Valid
            (Transformation|SetActorRelativeRotation _actor (Math|Rotator|MakeRotator 0.0 0.0 _returnvalue))))))))

(event Custom|InstanciateItem
  (bind _actorclass (Variables|Default|GetActorClass))
  (Utilities|IsValid (Variables|Default|GetStatickMesh)
    (:Is%20Valid
      (bind _returnvalue (AddComponent|AddStaticMeshComponent false))
      (bind _output_get (Variables|Default|SetMeshComponent _returnvalue))
      (Components|StaticMesh|SetStaticMesh _output_get (Variables|Default|GetStatickMesh)))
    (:Is%20Not%20Valid
      (if (Utilities|IsValidClass _actorclass)
        (bind _returnvalue_2 (Game|SpawnActorfromClass _actorclass (Math|Transform|MakeTransform "0, 0, 0" "0, 0, 0" "1.000000,1.000000,1.000000") "Undefined" "MultiplyWithRoot" 0 0))
        (Variables|Default|SetActor _returnvalue_2)))))

(fn ConstructionScript
  (CallFunction|InstanciateItem))

(fn IsValid
  (return (or (Utilities|IsValid (Variables|Default|GetStatickMesh)) (Utilities|IsValid (Variables|Default|GetActor)))))