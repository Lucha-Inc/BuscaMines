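; A single Minesweeper board square that can be revealed or flagged as a suspected mine, reporting sounds and stats to its Board.
; Setup maps the eight neighbors from the Board to count adjacent mines; selecting an empty square flood-reveals unflagged neighbors after a short delay.
; Custom depth stencil values drive hover and flag outlines, the number text bobs on Tick, and demo mode overrides piece visibility.
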(event Custom|Event%20Initialize)

(event Custom|propagateSelect
  (if (Variables|Properties|GetisEmptyArea)
    (Utilities|FlowControl|Delay 0.3)
    (bind _values (Utilities|Map|Values (Variables|Board|GetproximitySquares)))
    (for _array_element _values
      (if (not (or (Variables|BP_SquareActor_C|GetisSuspected _array_element) (Variables|BP_SquareActor_C|GetisSelected _array_element)))
        (CallFunction|Select _array_element)))))

(event EventBeginPlay
  (CallFunction|SetupDemo))

(event Collision|EventActorBeginOverlap
  (params (OtherActor :type Actor%20Object%20Reference)))

(event EventTick
  (params (DeltaSeconds :type Float%20%28single-precision%29))
  (if (Rendering|IsVisible (Variables|Default|GetText3D))
    (Transformation|AddLocalOffset (Variables|Default|GetText3D) (Math|Vector|MakeVector (* (Math|Trig|Sin(Radians) (* (Utilities|Time|GetGameTimeinSeconds) 2.0)) 0.5) 0.0 0.0) false false)))

(event EventSuspect
  (bind _board (Variables|board|Getboard))
  (bind _sound_manager_board (Variables|/Game/FP/BluePrints/Assets_BP/Board/BP_board_master.BP_board_master_C|GetSound%20Manager%20Board _board))
  ;[1 1 1] Marcando casilla como Sospechoza
  (if (not (Variables|Properties|GetisSelected))
    (bind _output_get (Variables|Properties|SetisSuspected (not (Variables|Properties|GetisSuspected))))
    (Utilities|FlowControl|Sequence
      (:then_0
        (CallFunction|SetOutlineSuspected _output_get))
      (:then_1
        (Rendering|SetVisibility (Variables|Default|GetsuspectedMine) _output_get false))
      (:then_2
        (if _output_get
          (Default|PlayFlagCreation _sound_manager_board)
          (else
            (Default|PlayFlagRemove _sound_manager_board))))
      (:then_3
        (Default|UpdateStats (Variables|board|Getboard))))))

(event EventSelect
  ;[1 1 1] Seleccionando una casilla
  (if (not (or (Variables|Properties|GetisSuspected) (Variables|Properties|GetisSelected)))
    (Utilities|FlowControl|DoOnce false
      (:Completed
        (Utilities|FlowControl|Sequence
          (:then_0
            (Rendering|SetVisibility (Variables|Default|GetsquereMesh) false false))
          (:then_1
            (Variables|Properties|SetisSelected true))
          (:then_2
            (Rendering|SetVisibility (Variables|Default|GetText3D) (> (Variables|board|GetproximityMines) 0) false))
          (:then_3
            (Default|PlaySquareSelected (Variables|/Game/FP/BluePrints/Assets_BP/Board/BP_board_master.BP_board_master_C|GetSound%20Manager%20Board (Variables|board|Getboard))))
          (:then_4
            (CallFunction|PropagateSelect))
          (:then_5
            (Default|UpdateStats (Variables|board|Getboard))))))))

(event Custom|setupDemo
  (bind _text3d (Variables|Default|GetText3D))
  (if (Variables|Demo|GetisDemoMode)
    (Utilities|FlowControl|Sequence
      (:then_0
        (Variables|/Script/Text3D.Text3DComponent|SetText _text3d (Utilities|Text|ToText(Integer) (Variables|Demo|Getdemo_setNumber)))
        (Rendering|SetVisibility _text3d (Variables|Demo|Getdemo_isNumberVisible) false))
      (:then_1
        (Rendering|SetVisibility (Variables|Default|GetsquereMesh) (Variables|Demo|Getdemo_isSquareVisible) false))
      (:then_2
        (Rendering|SetVisibility (Variables|Default|GetsuspectedMine) (Variables|Demo|Getdemo_isFlagVisible) false))
      (:then_3
        (Rendering|SetVisibility (Variables|Default|Getmine) (Variables|Demo|Getdemo_isMineVisible) false)))))

(fn ConstructionScript
  (Utilities|FlowControl|Sequence
    (:then_0
      (Rendering|Material|SetMaterial (Variables|Default|GetsquereMesh) 0 (Variables|Properties|Getsquare_material)))
    (:then_1
      (Rendering|Material|SetMaterial (Variables|Default|Getmine) 0 (Variables|Properties|Getsquare_mine_material)))
    (:then_2
      (Rendering|Material|SetMaterial (Variables|Default|GetsuspectedMine) 0 (Variables|Properties|Getsquare_flag_material)))))

(fn SetMine
  (params (withMine :type Boolean))
  (bind _output_get (Variables|Properties|SetwithMine withMine))
  (Rendering|SetVisibility (Variables|Default|Getmine) _output_get false))

(fn SetOutlineonView
  (params (onView :type Boolean))
  (if (not (Variables|Properties|GetisSuspected))
    (Rendering|SetCustomDepthStencilValue (Variables|Default|GetsquereMesh) (Math|Integer|SelectInt 1 0 onView))))

(fn SetOutlineSuspected
  (params (suspected :type Boolean))
  (Rendering|SetCustomDepthStencilValue (Variables|Default|GetsquereMesh) (Math|Integer|SelectInt 2 0 suspected)))

(fn Setup
  (Utilities|FlowControl|Sequence
    (:then_0
      (for _index (range -1 1)
        (for _index_2 (range -1 1)
          (if (not (and (== _index_2 0) (== _index 0)))
            (if (.ReturnValue (Utilities|Map|Find (Default|GetSquares (Variables|board|Getboard)) (+ (Math|Vector2D|MakeVector2D (Math|Conversions|ToFloat(Integer) _index_2) (Math|Conversions|ToFloat(Integer) _index)) (Math|Vector2D|MakeVector2D (Math|Conversions|ToFloat(Integer) (Variables|board|Getx)) (Math|Conversions|ToFloat(Integer) (Variables|board|Gety))))))
              (Utilities|Map|Add (Variables|Board|GetproximitySquares) (Math|Vector2D|MakeVector2D (Math|Conversions|ToFloat(Integer) _index_2) (Math|Conversions|ToFloat(Integer) _index)) (.Value (Utilities|Map|Find (Default|GetSquares (Variables|board|Getboard)) (+ (Math|Vector2D|MakeVector2D (Math|Conversions|ToFloat(Integer) _index_2) (Math|Conversions|ToFloat(Integer) _index)) (Math|Vector2D|MakeVector2D (Math|Conversions|ToFloat(Integer) (Variables|board|Getx)) (Math|Conversions|ToFloat(Integer) (Variables|board|Gety))))))))))))
    (:then_1
      (bind _values (Utilities|Map|Values (Variables|Board|GetproximitySquares)))
      (for _array_element _values
        (if (Variables|BP_SquareActor_C|GetwithMine _array_element)
          (Math|Integer|IncrementInt (LocalVariables|Getmines))))
      (bind _output_get (Variables|board|SetproximityMines (LocalVariables|Getmines)))
      (Variables|/Script/Text3D.Text3DComponent|SetText (Variables|Default|GetText3D) (Utilities|Text|ToText(Integer) _output_get)))
    (:then_2
      (Variables|Properties|SetisEmptyArea (and (== (Variables|board|GetproximityMines) 0) (not (Variables|Properties|GetwithMine)))))))