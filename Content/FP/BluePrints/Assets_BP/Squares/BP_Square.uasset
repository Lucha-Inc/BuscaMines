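; BP_Square is a single Minesweeper tile on a Board, which may hold a mine or be flagged as suspected.
; Setup caches its neighbours by coordinate to count nearby mines for a bobbing 3D number.
; Select reveals the tile, cascades through empty areas after a delay, and signals readiness once its chained sounds finish.
; Suspect toggles the flag, while custom depth stencil values drive hover and suspected outlines.
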(event EventBeginPlay)

(event Collision|EventActorBeginOverlap
  (params (OtherActor :type Actor%20Object%20Reference)))

(event EventTick
  (params (DeltaSeconds :type Float%20%28single-precision%29))
  (bind _text3d (Variables|Default|GetText3D))
  (if (Rendering|IsVisible _text3d)
    (Transformation|AddLocalOffset _text3d (Math|Vector|MakeVector (* (Math|Trig|Sin(Radians) (* (Utilities|Time|GetGameTimeinSeconds) 2.0)) 0.5) 0.0 0.0) false false)))

(event Custom|selectionAnimation
  (Variables|Properties|Setready false)
  (bind _audio_component (Default|PlaySquareSelected (Variables|/Game/FP/BluePrints/Assets_BP/Board/BP_board_master.BP_board_master_C|GetSound%20Manager%20Board (Variables|Board|Getboard))))
  (EventDispatchers|BindEventtoOnAudioFinished _audio_component (delegate Custom|onSelectesSoundFinished)))

(event Custom|onSelectesSoundFinished
  (if (Variables|Properties|GetwithMine)
    (bind _audio_component (Default|PlayMineExplote (Variables|/Game/FP/BluePrints/Assets_BP/Board/BP_board_master.BP_board_master_C|GetSound%20Manager%20Board (Variables|Board|Getboard))))
    (EventDispatchers|BindEventtoOnAudioFinished _audio_component (delegate Custom|finishAnimation))
    (else
      (CallFunction|FinishAnimation))))

(event Custom|displayNumber
  (bind _proximitymines (CallFunction|ProximityMines))
  (bind _text3d (Variables|Default|GetText3D))
  (Class|Text3DComponent|SetText _text3d (Utilities|Text|ToText(Integer) _proximitymines))
  (Rendering|SetVisibility _text3d (and (> _proximitymines 0) (not (Variables|Properties|GetwithMine))) false))

(event Custom|propagateSelect
  (if (CallFunction|IsEmptyArea)
    (Utilities|FlowControl|Delay 0.3)
    (bind _values (Utilities|Map|Values (Variables|Board|GetproximitySquares)))
    (for _array_element _values
      (CallFunction|Select _array_element))))

(event Custom|finishAnimation
  (Variables|Properties|Setready true)
  (Default|CallAnimationReady self))

(event Custom|Setup
  (bind _coord (Variables|Board|Getcoord))
  (Utilities|FlowControl|Sequence
    (:then_0
      (for _index (range -1 1)
        (for _index_2 (range -1 1)
          (if (not (and (== _index_2 0) (== _index 0)))
            (if (.ReturnValue (Utilities|Map|Find (Default|GetSquares (Variables|Board|Getboard)) (Utilities|Struct|MakeCoord_2D (+ _index_2 (.x _coord)) (+ _index (.y _coord)))))
              (Utilities|Map|Add (Variables|Board|GetproximitySquares) (Utilities|Struct|MakeCoord_2D (+ _index_2 (.x _coord)) (+ _index (.y _coord))) (.Value (Utilities|Map|Find (Default|GetSquares (Variables|Board|Getboard)) (Utilities|Struct|MakeCoord_2D (+ _index_2 (.x _coord)) (+ _index (.y _coord)))))))))))))

(fn ConstructionScript)

(fn ProximityMines
  (bind _values (Utilities|Map|Values (Variables|Board|GetproximitySquares)))
  (for _array_element _values
    (if (CallFunction|HasMine _array_element)
      (Math|Integer|IncrementInt (LocalVariables|GetnearlyMines))))
  (return (LocalVariables|GetnearlyMines)))

(fn HasMine
  (return (Variables|Properties|GetwithMine)))

(fn IsEmptyArea
  (return (and (== (CallFunction|ProximityMines) 0) (not (CallFunction|HasMine)))))

(fn SetOutlineonView
  (params (onView :type Boolean))
  (if (not (Variables|Properties|GetisSuspected))
    (Rendering|SetCustomDepthStencilValue (Variables|Default|GetSquare) (Math|Integer|SelectInt 1 0 onView))))

(fn SetOutlineSuspected
  (params (suspected :type Boolean))
  (Rendering|SetCustomDepthStencilValue (Variables|Default|GetSquare) (Math|Integer|SelectInt 2 0 suspected)))

(fn IsReady
  (return (Variables|Properties|Getready)))

(fn GetStatus
  (return (Variables|Properties|GetwithMine) (Variables|Properties|GetisSuspected) (Variables|Properties|GetisSelected)))

(fn GetCoords
  (return (Variables|Board|Getcoord)))

(fn Select
  (if (or (Variables|Properties|GetisSuspected) (Variables|Properties|GetisSelected))
    (return false)
    (else
      (Utilities|FlowControl|DoOnce false
        (:Completed
          (Utilities|FlowControl|Sequence
            (:then_0
              (Variables|Properties|Setready false)
              (Variables|Properties|SetisSelected true))
            (:then_1
              (Rendering|SetVisibility (Variables|Default|GetMine) (Variables|Properties|GetwithMine) false)
              (Rendering|SetVisibility (Variables|Default|GetSquare) false false)
              (CallFunction|DisplayNumber))
            (:then_4
              (CallFunction|SelectionAnimation))
            (:then_5
              (CallFunction|PropagateSelect))
            (:then_6
              (return (Variables|Properties|GetwithMine)))))))))

(fn Suspect
  (bind _board (Variables|Board|Getboard))
  (bind _sound_manager_board (Variables|/Game/FP/BluePrints/Assets_BP/Board/BP_board_master.BP_board_master_C|GetSound%20Manager%20Board _board))
  (if (not (Variables|Properties|GetisSelected))
    (bind _output_get (Variables|Properties|SetisSuspected (not (Variables|Properties|GetisSuspected))))
    (Utilities|FlowControl|Sequence
      (:then_0
        (CallFunction|SetOutlineSuspected _output_get))
      (:then_1
        (Rendering|SetVisibility (Variables|Default|GetFlag) _output_get false))
      (:then_2
        (if _output_get
          (Default|PlayFlagCreation _sound_manager_board)
          (else
            (Default|PlayFlagRemove _sound_manager_board))))
      (:then_3
        (return _output_get)))))