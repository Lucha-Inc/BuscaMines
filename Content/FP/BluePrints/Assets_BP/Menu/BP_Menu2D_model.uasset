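; BP_Menu2D_model is a menu actor with a widget component, moving the player's view between menu actors.
; On BeginPlay it passes itself to its UW_Menu3D_Model widget as the owning Menu.
; TransitionTo swaps actor collision to the target menu, then after a short delay eases the view target over to it.
; It can also record itself as the target's FromMenu.
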(event Custom|TransitionTo
  (params (NewMenu :type BP%20Menu%202D%20Model%20Object%20Reference) (saveFrom :type Boolean))
  (Collision|SetActorEnableCollision false)
  (Collision|SetActorEnableCollision NewMenu true)
  (Utilities|FlowControl|Delay 0.2)
  (Game|Player|SetViewTargetwithBlend (Game|GetPlayerController 0) NewMenu 3.0 "VTBlend_EaseInOut" 2.0 false)
  (if saveFrom
    (Variables|BP_Menu2D_model_C|SetfromMenu NewMenu self)))

(event EventBeginPlay
  (bind _asuw_menu_3d_model (Utilities|Casting|CastToUW_Menu3D_Model (UserInterface|GetUserWidgetObject (Variables|Default|GetWidget))))
  (Variables|/Game/FP/GUI/Widgets/UI_Menu/Master/UW_Menu3D_Model.UW_Menu3D_Model_C|SetMenu _asuw_menu_3d_model self))

(fn ConstructionScript)