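; Back button instance of the 3D text menu button, which returns the player to the last menu.
; On construction it asks the game mode master for the last menu and shows its button component only if that menu is valid.
; On click it runs the parent handler, repeats the lookup and goes to that menu's class when valid.
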(event EventBeginPlay
  (|CallParentFunction) ; This node is disabled and will not be called.\nDrag off pins to build functionality.
)

(event Collision|EventActorBeginOverlap
  (params (OtherActor :type Actor%20Object%20Reference)))

(event EventTick
  (params (DeltaSeconds :type Float%20%28single-precision%29)))

(fn ConstructionScript
  (|CallParentFunction)
  (bind _gamemode_master (CallFunction|GetCustomClasses self))
  (bind _validmenu (Default|GetLastMenu _gamemode_master))
  (Rendering|SetVisibility (Variables|Default|GetBP_Menu_Text3D_Button) _validmenu false))

(fn OnClick
  (|CallParentFunction)
  (bind _gamemode_master (CallFunction|GetCustomClasses self))
  (bind (_menuclass _validmenu) (Default|GetLastMenu _gamemode_master))
  (if _validmenu
    (CallFunction|GotoMenu _menuclass)))