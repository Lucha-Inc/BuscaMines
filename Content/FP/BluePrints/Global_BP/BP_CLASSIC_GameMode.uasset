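; Game mode for the Classic mode, extending a parent game mode with a classic-specific board, key-driven menu access and pause handling.
; Setup runs the parent logic, then casts and stores the board as BP_CLASSIC_Board, which GetBoard returns.
; Key presses are uppercased and looked up in the MenuAccess map to jump to a menu.
; Pause toggles between the pause menu with its HUD display and gameplay.
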(event EventBeginPlay
  (|CallParentFunction))

(event EventOnKeyPressed
  (params (char :type String))
  (bind _returnvalue (Class|KismetStringLibrary|ToUpper char))
  (bind _menuaccess (Variables|Default|GetmenuAccess))
  (bind (_value _returnvalue_2) (Utilities|Map|Find _menuaccess _returnvalue))
  (if _returnvalue_2
    (CallFunction|GotoMenu _value)))

(event EventSetup
  (params (Level :type BPI%20Level%20Master%20Interface) (Board :type BP%20Board%20Master%20Object%20Reference) (Sound%20Manager%20Level :type BP%20Sound%20Manager%20Level%20Object%20Reference))
  (|CallParentFunction Level Board Sound%20Manager%20Level)
  (bind _asbp_classic_board (Utilities|Casting|CastToBP_CLASSIC_Board Board))
  (Variables|Board|SetBoard_Classic _asbp_classic_board))

(event EventOnPause
  (CallFunction|SetPauseToogle)
  (if (Variables|Default|Getpaused)
    (CallFunction|SetMenu "/Game/FP/GUI/Widgets/3D_Menu/Instance/BP_Menu_Pause.BP_Menu_Pause_C")
    (Default|ShowPause (Variables|Default|GetHUD))
    (else
      (CallFunction|SetGame))))

(fn ConstructionScript
  (|CallParentFunction))

(fn GetBoard
  (return (Variables|Board|GetBoard_Classic)))