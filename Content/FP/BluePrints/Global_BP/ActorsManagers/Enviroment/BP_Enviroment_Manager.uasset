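; Environment manager actor that triggers procedural forest generation and signals when the environment is ready.
; Its Generate event casts the PCGForest child actor to A_PCG_Forest and calls GeneratePCG on it.
; Readiness is called after a fixed delay from BeginPlay, independent of generation.
; A PCG-completion handler also signals readiness, but its binding is disconnected, as are direct PCG generation and the construction-time scaling.
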(event Custom|PCG_ready
  (params (PCGComponent :type PCG%20Component%20Object%20Reference))
  (Default|CallEnviromentReady))

(event EventBeginPlay
  (Utilities|FlowControl|Delay 5.0)
  (Default|CallEnviromentReady))

(event Collision|EventActorBeginOverlap
  (params (OtherActor :type Actor%20Object%20Reference)))

(event EventTick
  (params (DeltaSeconds :type Float%20%28single-precision%29)))

(event Custom|Generate
  (bind _asa_pcg_forest (Utilities|Casting|CastToA_PCG_Forest (Variables|/Script/Engine.ChildActorComponent|GetChildActor (Variables|Default|GetPCG_Forest))))
  (Default|GeneratePCG _asa_pcg_forest))

(fn ConstructionScript)