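; BP_Sound_Manager_App is a sound manager that plays app-level UI click sounds and menu background music from the DAThemeApp theme data.
; Button clicks spawn a fresh audio component each time and play it immediately.
; Menu music lazily creates one persistent, non-auto-destroyed component in MusicBg, then fades it in and out slowly along an S-curve on start and stop events.
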(event Custom|Play_UI_Button_Click
  (bind _audio_component (CallFunction|CreateAudioComponent (Variables|/Game/FP/BluePrints/Global_BP/DataAsset/DA_ThemeData_App.DA_ThemeData_App_C|Getsound_ui_click (Variables|DataAsset|GetDA%20Theme%20App)) 0 true true))
  (Audio|Components|Audio|Play _audio_component 0.0))

(event Custom|Stop%20Music%20bg
  (bind _music_bg (Variables|Default|GetMusic%20bg))
  (Utilities|IsValid _music_bg
    (:Is%20Valid
      (Audio|Components|Audio|FadeOut _music_bg 1e+01 0.0 "SCurve" :!class /Script/Engine.AudioComponent))))

(event Custom|Play%20Music%20bg
  (bind _music_bg (Variables|Default|GetMusic%20bg))
  (Utilities|IsValid _music_bg
    (:Is%20Valid
      _)
    (:Is%20Not%20Valid
      (CallFunction|CreateAudioComponent (Variables|/Game/FP/BluePrints/Global_BP/DataAsset/DA_ThemeData_App.DA_ThemeData_App_C|Getsound_cue_menu_music (Variables|DataAsset|GetDA%20Theme%20App)) _music_bg true false)))
  (Audio|Components|Audio|FadeIn (Variables|Default|GetMusic%20bg) 1e+01 1.0 0.0 "SCurve" :!class /Script/Engine.AudioComponent))