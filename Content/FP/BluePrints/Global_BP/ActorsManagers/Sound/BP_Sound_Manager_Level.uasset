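; Level sound manager that plays a level's intro music, gameplay music and win/lose finish sounds.
; Each event pulls its sound from the DAThemeLevel theme data, so audio follows the level's theme.
; Background tracks are kept in non-auto-destroy audio components with long fade-ins, letting matching stop events fade them out.
; Finish sounds play as one-shots without a stored component.
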(event Custom|Play%20Level%20Finish%20Lose
  (CallFunction|CreatePlaySound (Variables|/Game/FP/BluePrints/Global_BP/DataAsset/DA_ThemeData_Level.DA_ThemeData_Level_C|Getsound_final_lose (Variables|DataAsset|GetDA%20Theme%20Level)) 0 true true 0.0))

(event Custom|Play%20Level%20Finish%20Win
  (CallFunction|CreatePlaySound (Variables|/Game/FP/BluePrints/Global_BP/DataAsset/DA_ThemeData_Level.DA_ThemeData_Level_C|Getsound_final_win (Variables|DataAsset|GetDA%20Theme%20Level)) 0 true true 0.0))

(event Custom|Play%20Level%20Game%20Music%20bg
  (CallFunction|CreatePlaySound (Variables|/Game/FP/BluePrints/Global_BP/DataAsset/DA_ThemeData_Level.DA_ThemeData_Level_C|Getsound_cue_game_music (Variables|DataAsset|GetDA%20Theme%20Level)) (Variables|Default|GetGame_Music_bg) true false 1e+01))

(event Custom|Stop%20Level%20Game%20Music%20bg
  (CallFunction|StopAudioComponent (Variables|Default|GetGame_Music_bg) 1e+01))

(event Custom|Play%20Level%20Intro%20Music%20bg
  (CallFunction|CreatePlaySound (Variables|/Game/FP/BluePrints/Global_BP/DataAsset/DA_ThemeData_Level.DA_ThemeData_Level_C|Getsound_cue_intro_music (Variables|DataAsset|GetDA%20Theme%20Level)) (Variables|Default|GetIntro_Music_bg) true false 1e+01))

(event Custom|Stop%20Level%20Intro%20Music%20bg
  (CallFunction|StopAudioComponent (Variables|Default|GetIntro_Music_bg) 1e+01))