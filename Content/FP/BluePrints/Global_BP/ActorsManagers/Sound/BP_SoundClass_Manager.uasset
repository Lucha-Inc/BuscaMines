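; BP_SoundClass_Manager controls per-category audio volume and mute through a map of sound class setups, each pairing a sound mix, class, volume and mute flag.
; Construction applies every entry as a sound mix class override, with muted entries forced to zero volume.
; Setters update the map, reapply that override and save the setup through the GameInstance.
; Setting volume on one specific category also cascades it to three others.
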(fn ConstructionScript
  (bind _valuepin (Utilities|Map|ForEachLoop(Map) (Variables|Default|GetsoundClasses))
    (:then
      (Audio|SetSoundMixClassOverride (.soundmix _valuepin) (.soundclass _valuepin) (select (.mute _valuepin) 0.0 (.volume _valuepin)) 1.0 0.0 true))))

(fn SetClassSetup
  (params (soundClass :type E_SoundClasses%20Enum :default "NewEnumerator0"))
  (bind _soundclasses (Variables|Default|GetsoundClasses))
  (bind (_value _returnvalue) (Utilities|Map|Find _soundclasses soundClass))
  (if _returnvalue
    (Audio|SetSoundMixClassOverride (.soundmix _value) (.soundclass _value) (select (.mute _value) 0.0 (.volume _value)) 1.0 0.0 true)
    (Default|SaveSoundClassesSetup (Variables|Default|GetGameInstance) (Variables|Default|GetsoundClasses))))

(fn SetVolume
  (params (SoundClass :type E_SoundClasses%20Enum :default "NewEnumerator0") (volume :type Float%20%28double-precision%29))
  (bind _soundclasses (Variables|Default|GetsoundClasses))
  (bind _value (Utilities|Map|Find _soundclasses SoundClass))
  (if (Utilities|Enum|Equal(Enum) SoundClass "NewEnumerator3")
    (CallFunction|SetVolume "NewEnumerator4" volume)
    (CallFunction|SetVolume "NewEnumerator5" volume)
    (CallFunction|SetVolume "NewEnumerator6" volume))
  (Utilities|Map|Add _soundclasses SoundClass (Utilities|Struct|MakeStruct_SOUND_CLASS_MIX (.soundmix _value) (.soundclass _value) volume false))
  (CallFunction|SetClassSetup SoundClass))

(fn SetMute
  (params (soundClass :type E_SoundClasses%20Enum :default "NewEnumerator0") (mute :type Boolean))
  (bind _soundclasses (Variables|Default|GetsoundClasses))
  (bind _value (Utilities|Map|Find _soundclasses soundClass))
  (Utilities|Map|Add _soundclasses soundClass (Utilities|Struct|MakeStruct_SOUND_CLASS_MIX (.soundmix _value) (.soundclass _value) (.volume _value) mute))
  (CallFunction|SetClassSetup soundClass))

(fn ToggleMute
  (params (soundClass :type E_SoundClasses%20Enum :default "NewEnumerator0"))
  (CallFunction|SetMute soundClass (not (.mute (.Value (Utilities|Map|Find (Variables|Default|GetsoundClasses) soundClass))))))

(fn GetSoundClassesBORRAR
  (return (Variables|Default|GetsoundClasses)))

(fn GetSoundClassSetup
  (params (SoundClass :type E_SoundClasses%20Enum :default "NewEnumerator0"))
  (return (.Value (Utilities|Map|Find (Variables|Default|GetsoundClasses) SoundClass))))