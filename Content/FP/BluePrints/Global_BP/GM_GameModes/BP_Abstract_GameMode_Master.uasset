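; Master game mode for board-based levels, driving the flow from setup through presentation, camera intro, gameplay and win/lose menus.
; Board events end the level, while status and pause state coordinate the timer, HUD, level music and movement bounds.
; SetMenu and SetGame swap Enhanced Input contexts and 3D menus.
; A reversible timeline blends camera FOV, player height and pitch, and menu scale between both modes.
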(event Custom|BoardStatsUpdated
  (params (StatsObject :type BP%20Stats%20Master%20Object%20Reference)))

(event Custom|BoardFinished
  (params (Won :type Boolean))
  (CallFunction|LevelCompleted Won))

(event EventBeginPlay
  (bind _self self)
  (Utilities|FlowControl|Sequence
    (:then_0
      (bind (_gameinstance _thememanager _soundmanager_app _player _gamemode_master _playercontroller_master) (CallFunction|GetCustomClasses _self))
      (Variables|Managers|SetPlayer%20Controller%20Master _playercontroller_master)
      (Variables|Managers|SetPlayer _player))
    (:then_1
      (bind _hud_classic (CallFunction|GetCustomClassic _self))
      (Variables|Managers|SetHUD _hud_classic))
    (:then_3
      (bind _gameinstance_2 (CallFunction|GetCustomClasses _self))
      (bind _soundmanager (Default|GetSoundClassManager _gameinstance_2))
      (Default|SetMute _soundmanager "NewEnumerator4" true))))

(event EventSetup
  (params (Level :type BPI%20Level%20Master%20Interface) (Board :type BP%20Board%20Master%20Object%20Reference) (Sound%20Manager%20Level :type BP%20Sound%20Class%20Manager%20Level%20Object%20Reference) (PostProcessVolume :type Post%20Process%20Volume%20Object%20Reference))
  (Utilities|FlowControl|Sequence
    (:then_0
      (Variables|State|Setstatus "NewEnumerator0"))
    (:then_1
      (Variables|Level|SetLevel Level)
      (Variables|Level|SetPostProcessVolume PostProcessVolume))
    (:then_2
      (Variables|Managers|SetSound%20Manager%20Level Sound%20Manager%20Level))
    (:then_3
      (bind _output_get (Variables|Board|SetBoard_Master Board))
      (EventDispatchers|BindEventtoBoardStatsUpdated _output_get (delegate Custom|BoardStatsUpdated))
      (EventDispatchers|BindEventtoBoardFinished _output_get (delegate Custom|BoardFinished)))
    (:then_5
      (bind _soundmanager_app (CallFunction|GetCustomClasses self))
      (Variables|Managers|SetSound%20Manager%20App _soundmanager_app))
    (:then_6
      (Default|ShowDebugModeUW (Variables|Managers|GetHUD)))))

(event Custom|setPauseOn
  (CallFunction|SetPauseto true))

(event Custom|setPauseOff
  (CallFunction|SetPauseto true))

(event Custom|setPauseTo
  (params (pause :type Boolean))
  (if (!= pause (Variables|State|Getpaused))
    (bind _output_get (Variables|State|Setpaused pause))
    (Default|SetPauseto (Variables|Default|GetTimer) _output_get)
    (Default|CallPauseChanged _output_get)))

(event Custom|setPauseToogle
  (CallFunction|SetPauseto (not (Variables|State|Getpaused))))

(event Custom|_Menu%20Transition
  (params (toMenuMode :type Boolean) (Menu%203D :type BP%20Actor%20Menu%203D%20Object%20Reference))
  (bind _returnvalue (Game|GetPlayerCharacter 0))
  (bind _returnvalue_2 (Game|GetPlayerCharacter 0))
  (bind _returnvalue_3 (Transformation|GetActorTransform _returnvalue))
  (bind _returnvalue_4 (Transformation|GetActorTransform _returnvalue_2))
  (if toMenuMode
    (Variables|Default|SetTransitionProps (Utilities|Struct|MakeStruct_Transition_Menu_Game_Mode (.gamemode_fov (Variables|Default|GetTransitionProps)) (.z (.location _returnvalue_4)) (.pitch (.rotation _returnvalue_4)) (.menumode_fov (Variables|Default|GetTransitionProps)) (Math|Float|Max(Float) (.menumode_z_heigh (Variables|Default|GetTransitionProps)) (.z (.location _returnvalue_4))) (.menumode_y_angle (Variables|Default|GetTransitionProps)) (Transformation|GetActorScale3D Menu%203D) (.blur (Variables|Default|GetTransitionProps)) (.alpha (Variables|Default|GetTransitionProps)) (.transitiontime (Variables|Default|GetTransitionProps))))
    (Components|Timeline|SetPlayRate (Variables|Default|GetTransition_MenuMode_Timeline) (/ 1.0 (.transitiontime (Variables|Default|GetTransitionProps))))
    (bind _alpha_auto (Timeline|Transition_MenuMode_Timeline Play)
      (:Update
        (Utilities|FlowControl|Sequence
          (:then_0
            ;[0.15 0.15 0.15 0.5] Set FOV
            (Camera|SetFieldOfView (Variables|/Game/FP/BluePrints/Chareacters/Player/BP_player.BP_player_C|GetCamera (Variables|Managers|GetPlayer)) (Math|Float|Lerp (.gamemode_fov (Variables|Default|GetTransitionProps)) (.menumode_fov (Variables|Default|GetTransitionProps)) _alpha_auto))
            (Default|CallChangingFOV (Math|Float|Lerp (.gamemode_fov (Variables|Default|GetTransitionProps)) (.menumode_fov (Variables|Default|GetTransitionProps)) _alpha_auto)))
          (:then_1
            ;[0.15 0.15 0.15 0.5] Set Player Location and Rotation
            (if (Utilities|Enum|Equal(Enum) (Variables|State|Getstatus) "NewEnumerator4")
              (Transformation|SetActorLocationAndRotation _returnvalue (Math|Vector|MakeVector (.x (.location _returnvalue_3)) (.y (.location _returnvalue_3)) (Math|Float|Lerp (.gamemode_z_heigh (Variables|Default|GetTransitionProps)) (.menumode_z_heigh (Variables|Default|GetTransitionProps)) _alpha_auto)) (Math|Rotator|MakeRotator (.roll (.rotation _returnvalue_3)) (Math|Float|Lerp (.gamemode_y_angle (Variables|Default|GetTransitionProps)) (.menumode_y_angle (Variables|Default|GetTransitionProps)) _alpha_auto) (.yaw (.rotation _returnvalue_3))))))
          (:then_2
            ;[0.15 0.15 0.15 0.5] Set Menu Scale
            (Utilities|IsValid Menu%203D
              (:Is%20Valid
                (Transformation|SetActorScale3D Menu%203D (Math|Vector|Lerp(Vector) "0, 0, 0" (.menumode_finalscale (Variables|Default|GetTransitionProps)) _alpha_auto))))))))
    (else
      (Components|Timeline|SetPlayRate (Variables|Default|GetTransition_MenuMode_Timeline) (/ 1.0 (.transitiontime (Variables|Default|GetTransitionProps))))
      (Timeline|Transition_MenuMode_Timeline Reverse))))

(event Custom|SetMenu
  (params (Menu%20Actor :type BP%20Actor%20Menu%203D%20Class%20Reference))
  (bind _player_controller_master (Variables|Managers|GetPlayer%20Controller%20Master))
  (Utilities|FlowControl|Sequence
    (:then_0
      (Default|ClearMenus3D _player_controller_master)
      (Variables|Default|SetlastMenu (Variables|Default|GetcurrentMenu))
      (bind _output_get (Variables|Default|SetcurrentMenu Menu%20Actor))
      (bind _menu_3d (Default|ShowMenu3D _player_controller_master _output_get)))
    (:then_1
      ;[1 1 1] Si no viene de un modo MENU, hace una transición Visual
      (if (not (Variables|State|GetmenuMode))
        (bind _output_get_2 (Variables|State|SetmenuMode true))
        (CallFunction|MenuTransition _output_get_2 _menu_3d)
        (CallFunction|RemoveGameInputs)
        (CallFunction|AddMenuInputs)
        (Variables|/Script/Engine.PlayerController|SetbEnableClickEvents (Game|GetPlayerController 0) true)
        (switch Utilities|FlowControl|Switch|SwitchonEGameMode_Status (Variables|State|Getstatus)
          (:NewEnumerator4
            (Default|StopLevelGameMusicBg (Variables|Managers|GetSound%20Manager%20Level))))))
    (:then_2
      (Variables|/Script/Engine.PostProcessVolume|SetbEnabled (Variables|Level|GetPostProcessVolume) false))))

(event Custom|SetGame
  (Utilities|FlowControl|Sequence
    (:then_0
      (Variables|/Script/Engine.PostProcessVolume|SetbEnabled (Variables|Level|GetPostProcessVolume) true))
    (:then_1
      ;[1 1 1] Si no viene de un modo MENU, hace una transición Visual
      (if (Variables|State|GetmenuMode)
        (bind _output_get (Variables|State|SetmenuMode false))
        (CallFunction|MenuTransition _output_get)
        (CallFunction|RemoveMenuInputs)
        (else
          (Default|PlayLevelGameMusicBg (Variables|Managers|GetSound%20Manager%20Level)))))
    (:then_2
      (Default|ClearMenus3D (Variables|Managers|GetPlayer%20Controller%20Master))
      (Variables|Default|SetlastMenu 0)
      (Variables|Default|SetcurrentMenu 0))
    (:then_3
      (switch Utilities|FlowControl|Switch|SwitchonEGameMode_Status (Variables|State|Getstatus)
        (:NewEnumerator4
          (Default|ShowGaming (Variables|Managers|GetHUD))
          (CallFunction|AddGameInputs))))))

(event Custom|_Add_MenuInputs
  (CallFunction|AddRemoveInputMappingContext "/Game/FP/BluePrints/Global_BP/Inputs/menu_inputs.menu_inputs" true)
  (Variables|/Script/Engine.PlayerController|SetbShowMouseCursor (Variables|Managers|GetPlayer%20Controller%20Master) true))

(event Custom|_Remove_MenuInputs
  (CallFunction|AddRemoveInputMappingContext "/Game/FP/BluePrints/Global_BP/Inputs/menu_inputs.menu_inputs" false)
  (Variables|/Script/Engine.PlayerController|SetbShowMouseCursor (Variables|Managers|GetPlayer%20Controller%20Master) false))

(event Custom|_Add_GameInputs
  (bind _player_controller_master (Variables|Managers|GetPlayer%20Controller%20Master))
  (CallFunction|AddRemoveInputMappingContext "/Game/FP/BluePrints/Global_BP/Inputs/board_inputs.board_inputs" true)
  (CallFunction|AddRemoveInputMappingContext "/Game/FP/BluePrints/Global_BP/Inputs/player_inputs.player_inputs" true)
  ;[0.15 0.15 0.15 0.5] To see the Mouse in the Game
  (Variables|/Script/Engine.PlayerController|SetbShowMouseCursor _player_controller_master true)
  (Variables|/Script/Engine.PlayerController|SetbEnableClickEvents _player_controller_master true)
  (Variables|/Script/Engine.PlayerController|SetbEnableMouseOverEvents _player_controller_master true))

(event Custom|Remove_GameInputs
  (bind _player_controller_master (Variables|Managers|GetPlayer%20Controller%20Master))
  (CallFunction|AddRemoveInputMappingContext "/Game/FP/BluePrints/Global_BP/Inputs/board_inputs.board_inputs" false)
  (CallFunction|AddRemoveInputMappingContext "/Game/FP/BluePrints/Global_BP/Inputs/player_inputs.player_inputs" false)
  ;[0.15 0.15 0.15 0.5] To see the Mouse in the Game
  (Variables|/Script/Engine.PlayerController|SetbShowMouseCursor _player_controller_master false)
  (Variables|/Script/Engine.PlayerController|SetbEnableClickEvents _player_controller_master false)
  (Variables|/Script/Engine.PlayerController|SetbEnableMouseOverEvents _player_controller_master false))

(event EventGotoMenu
  (params (menuClass :type BP%20Actor%20Menu%203D%20Class%20Reference))
  (CallFunction|SetMenu menuClass)
  (switch Utilities|FlowControl|Switch|SwitchonEGameMode_Status (Variables|State|Getstatus)
    (:NewEnumerator4
      (if (not (Variables|State|Getpaused))
        (CallFunction|SetPauseon)
        (Default|ShowPause (Variables|Managers|GetHUD))))))

(event Custom|LevelCompleted
  (params (won :type Boolean))
  (bind _hud (Variables|Managers|GetHUD))
  (Variables|State|Setstatus "NewEnumerator6")
  (Default|EndTimer (Variables|Default|GetTimer))
  (CallFunction|AddRemoveInputMappingContext "/Game/FP/BluePrints/Global_BP/Inputs/pause_inputs.pause_inputs" false)
  (if won
    (Default|ClearAllUW _hud)
    (Default|PlayLevelFinishWin (Variables|Managers|GetSound%20Manager%20Level))
    (CallFunction|SetMenu "/Game/FP/GUI/Widgets/3D_Menu/Instance/BP_Menu_Won.BP_Menu_Won_C")
    (else
      (Default|ClearAllUW _hud)
      (Default|PlayLevelFinishLose (Variables|Managers|GetSound%20Manager%20Level))
      (CallFunction|SetMenu "/Game/FP/GUI/Widgets/3D_Menu/Instance/BP_Menu_Lose.BP_Menu_Lose_C"))))

(event EventOnLevelReady
  ;[1 1 1] Show Presentation Menu
  (Variables|State|Setstatus "NewEnumerator1")
  (Default|PlayLevelIntroMusicBg (Variables|Managers|GetSound%20Manager%20Level))
  (CallFunction|SetMenu "/Game/FP/GUI/Widgets/3D_Menu/Instance/BP_Menu_Presentation.BP_Menu_Presentation_C")
  (Default|ShowDebugModeUW (Variables|Managers|GetHUD)))

(event EventStartIntro
  (bind _sound_manager_level (Variables|Managers|GetSound%20Manager%20Level))
  (Variables|State|Setstatus "NewEnumerator2")
  (Default|StopLevelIntroMusicBg _sound_manager_level)
  (Default|PlayLevelGameMusicBg _sound_manager_level)
  (CallFunction|SetGame)
  ;[1 1 1] Intro Movemente of Camera
  (bind _playermovement (CallFunction|GetCustomPlayer self))
  (Default|PlayMovement _playermovement (Default|GetStartPosition (Variables|Board|GetBoard_Master)) 6.0)
  (EventDispatchers|BindEventtoMovementFinished _playermovement (delegate EventOnIntroReady)))

(event EventOnIntroReady
  (bind _board_master (Variables|Board|GetBoard_Master))
  (bind _bounds (Default|GetBoardMovementsBounds _board_master))
  (Variables|State|Setstatus "NewEnumerator4")
  (bind (_gameinstance _thememanager _soundmanager_app _player _gamemode_master _playercontroller_master) (CallFunction|GetCustomClasses self))
  (Utilities|FlowControl|Sequence
    (:then_0
      (bind _soundmanager (Default|GetSoundClassManager _gameinstance))
      (Default|SetMute _soundmanager "NewEnumerator4" false))
    (:then_1
      (bind _debugmode (CallFunction|GetDebugMode self))
      (Default|SetPlayerMovementBounds _playercontroller_master (Utilities|Struct|MakePlayerMovementBoundsDefinition (not _debugmode) (.bounds_origin _bounds) (+ (.bounds_extents _bounds) "1000.000000,1000.000000,1500.000000") "500.000000,500.000000,500.000000" (.normal_vector_x _bounds) (.normal_vector_y _bounds))))
    (:then_2
      (Default|StartTimer (Variables|Default|GetTimer))
      (CallFunction|SetGame)
      (CallFunction|AddRemoveInputMappingContext "/Game/FP/BluePrints/Global_BP/Inputs/pause_inputs.pause_inputs" true))
    (:then_3
      (Default|BoardStart (Variables|Board|GetBoard_Master)))))

(fn ConstructionScript)

(fn AddRemoveInputMappingContext
  (params (Input%20Mapping%20Context :type Input%20Mapping%20Context%20Object%20Reference) (Add%20Input :type Boolean))
  (bind _returnvalue (Game|GetPlayerController 0))
  (bind _returnvalue_2 (PlayerController|LocalPlayerSubsystems|GetEnhancedInputLocalPlayerSubsystem _returnvalue))
  (if Add%20Input
    (Input|AddMappingContext _returnvalue_2 Input%20Mapping%20Context 0 "(bIgnoreAllPressedKeysUntilRelease=True,bForceImmediately=False,bNotifyUserSettings=False)")
    (else
      (Input|RemoveMappingContext _returnvalue_2 Input%20Mapping%20Context "(bIgnoreAllPressedKeysUntilRelease=True,bForceImmediately=False,bNotifyUserSettings=False)"))))

(fn GetLastMenu
  (bind _lastmenu (Variables|Default|GetlastMenu))
  (return _lastmenu (Utilities|IsValidClass _lastmenu)))

(fn IsPaused
  (return (Variables|State|Getpaused)))