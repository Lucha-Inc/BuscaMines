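; Abstract master GameMode that runs a board level through setup, presentation, camera intro, gameplay and win or lose end.
; A Status variable drives the flow, reacting to the board's finished event and controlling the timer, HUD, level music and sound muting.
; SetMenu and SetGame switch between 3D menus and gameplay, swapping Enhanced Input mapping contexts and blending camera FOV on a timeline.
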(event Custom|BoardStatsUpdated
  (params (StatsObject :type BP%20Stats%20Master%20Object%20Reference)))

(event Custom|BoardFinished
  (params (Won :type Boolean))
  (CallFunction|LevelCompleted Won))

(event EventBeginPlay
  (bind _self self)
  (Utilities|FlowControl|Sequence
    (:then_0
      (bind (_gameinstance _thememanager _soundmanager_app _playercontroller _player) (CallFunction|GetCustomClasses _self))
      (Variables|Managers|SetPlayer%20Controller _playercontroller)
      (Variables|Managers|SetPlayer _player))
    (:then_1
      (bind _hud_classic (CallFunction|GetCustomClassic _self))
      (Variables|HUD|SetHUD _hud_classic))
    (:then_3
      (bind _gameinstance_2 (CallFunction|GetCustomClasses _self))
      (bind _soundmanager (Default|GetSoundClassManager _gameinstance_2))
      (Default|SetMute _soundmanager "NewEnumerator4" true))))

(event EventSetup
  (params (Level :type BPI%20Level%20Master%20Interface) (Board :type BP%20Board%20Master%20Object%20Reference) (Sound%20Manager%20Level :type BP%20Sound%20Manager%20Level%20Object%20Reference))
  (Utilities|FlowControl|Sequence
    (:then_0
      (Variables|State|Setstatus "NewEnumerator0"))
    (:then_1
      (Variables|Level|SetLevel Level))
    (:then_2
      (Variables|Managers|SetSound%20Manager%20Level Sound%20Manager%20Level))
    (:then_3
      (bind _output_get (Variables|Board|SetBoard_Master Board))
      (EventDispatchers|BindEventtoBoardStatsUpdated _output_get (delegate Custom|BoardStatsUpdated))
      (EventDispatchers|BindEventtoBoardFinished _output_get (delegate Custom|BoardFinished)))
    (:then_4
      (bind _soundmanager_app (CallFunction|GetCustomClasses self))
      (Variables|Managers|SetSound%20Manager%20App _soundmanager_app))))

(event Custom|setPauseOn
  (CallFunction|SetPauseto true))

(event Custom|setPauseOff
  (CallFunction|SetPauseto true))

(event Custom|setPauseTo
  (params (pause :type Boolean))
  (bind _output_get (Variables|State|Setpaused pause))
  (Default|SetPauseto (Variables|Default|GetTimer) _output_get))

(event Custom|setPauseToogle
  (CallFunction|SetPauseto (not (Variables|State|Getpaused))))

(event Custom|_Menu%20Transition
  (params (toMenuMode :type Boolean))
  (bind _transitionprops (Variables|Default|GetTransitionProps))
  (bind _transitionprops_2 (Variables|Default|GetTransitionProps))
  (if toMenuMode
    (Components|Timeline|SetPlayRate (Variables|Default|GetTransition_MenuMode_Timeline) (/ 1.0 (.transitiontime _transitionprops_2)))
    (bind _alpha_auto (Timeline|Transition_MenuMode_Timeline Play)
      (:Update
        (Utilities|FlowControl|Sequence
          (:then_0
            (Camera|SetFieldOfView (Variables|/Game/FP/BluePrints/Chareacters/Player/BP_player.BP_player_C|GetCamera (Variables|Managers|GetPlayer)) (Math|Float|Lerp (.fov_gamemode _transitionprops) (.fov_menumode _transitionprops) _alpha_auto))
            (Default|CallChangingFOV (Math|Float|Lerp (.fov_gamemode _transitionprops) (.fov_menumode _transitionprops) _alpha_auto))))))
    (else
      (Components|Timeline|SetPlayRate (Variables|Default|GetTransition_MenuMode_Timeline) (/ 1.0 (.transitiontime _transitionprops_2)))
      (Timeline|Transition_MenuMode_Timeline Reverse))))

(event Custom|SetMenu
  (params (Menu%20Actor :type BP%20Actor%20Menu%203D%20Class%20Reference))
  (bind _player_controller (Variables|Managers|GetPlayer%20Controller))
  (Utilities|FlowControl|Sequence
    (:then_0
      ;[1 1 1] Si no viene de un modo MENU, hace una transición Visual
      (if (not (Variables|State|GetmenuMode))
        (bind _output_get (Variables|State|SetmenuMode true))
        (CallFunction|MenuTransition _output_get)
        (CallFunction|RemoveGameInputs)
        (CallFunction|AddMenuInputs)
        (Variables|/Script/Engine.PlayerController|SetbEnableClickEvents (Game|GetPlayerController 0) true)
        (switch Utilities|FlowControl|Switch|SwitchonEGameMode_Status (Variables|State|Getstatus)
          (:NewEnumerator4
            (Default|StopLevelGameMusicBg (Variables|Managers|GetSound%20Manager%20Level))))))
    (:then_1
      (Class|BPIPlayerController|ClearMenus(Message) _player_controller)
      (Variables|Default|SetlastMenu (Variables|Default|GetcurrentMenu))
      (bind _output_get_2 (Variables|Default|SetcurrentMenu Menu%20Actor))
      (Class|BPIPlayerController|ShowMenu3D(Message) _player_controller _output_get_2))))

(event Custom|SetGame
  (Utilities|FlowControl|Sequence
    (:then_1
      ;[1 1 1] Si no viene de un modo MENU, hace una transición Visual
      (if (Variables|State|GetmenuMode)
        (bind _output_get (Variables|State|SetmenuMode false))
        (CallFunction|MenuTransition _output_get)
        (CallFunction|RemoveMenuInputs)
        (else
          (Default|PlayLevelGameMusicBg (Variables|Managers|GetSound%20Manager%20Level)))))
    (:then_3
      (Default|ClearMenus (Variables|Managers|GetPlayer%20Controller))
      (Variables|Default|SetlastMenu 0)
      (Variables|Default|SetcurrentMenu 0))
    (:then_4
      (switch Utilities|FlowControl|Switch|SwitchonEGameMode_Status (Variables|State|Getstatus)
        (:NewEnumerator4
          (Default|ShowGaming (Variables|HUD|GetHUD))
          (CallFunction|AddGameInputs))))))

(event Custom|_Add_MenuInputs
  (Variables|/Script/Engine.PlayerController|SetbShowMouseCursor (Variables|Managers|GetPlayer%20Controller) true)
  (CallFunction|AddRemoveInputMappingContext "/Game/FP/BluePrints/Global_BP/Inputs/menu_inputs.menu_inputs" true))

(event Custom|_Remove_MenuInputs
  (Variables|/Script/Engine.PlayerController|SetbShowMouseCursor (Variables|Managers|GetPlayer%20Controller) false)
  (CallFunction|AddRemoveInputMappingContext "/Game/FP/BluePrints/Global_BP/Inputs/menu_inputs.menu_inputs" false))

(event Custom|_Add_GameInputs
  (CallFunction|AddRemoveInputMappingContext "/Game/FP/BluePrints/Global_BP/Inputs/board_inputs.board_inputs" true)
  (CallFunction|AddRemoveInputMappingContext "/Game/FP/BluePrints/Global_BP/Inputs/player_inputs.player_inputs" true))

(event Custom|Remove_GameInputs
  (CallFunction|AddRemoveInputMappingContext "/Game/FP/BluePrints/Global_BP/Inputs/board_inputs.board_inputs" false)
  (CallFunction|AddRemoveInputMappingContext "/Game/FP/BluePrints/Global_BP/Inputs/player_inputs.player_inputs" false))

(event EventGotoMenu
  (params (menuClass :type BP%20Actor%20Menu%203D%20Class%20Reference))
  (CallFunction|SetMenu menuClass)
  (switch Utilities|FlowControl|Switch|SwitchonEGameMode_Status (Variables|State|Getstatus)
    (:NewEnumerator4
      (if (not (Variables|State|Getpaused))
        (CallFunction|SetPauseon)
        (Default|ShowPause (Variables|HUD|GetHUD))))))

(event Custom|LevelCompleted
  (params (won :type Boolean))
  (bind _hud (Variables|HUD|GetHUD))
  (Variables|State|Setstatus "NewEnumerator6")
  (Default|EndTimer (Variables|Default|GetTimer))
  (CallFunction|AddRemoveInputMappingContext "/Game/FP/BluePrints/Global_BP/Inputs/pause_inputs.pause_inputs" false)
  (if won
    (Default|ClearAll _hud)
    (Default|PlayLevelFinishWin (Variables|Managers|GetSound%20Manager%20Level))
    (CallFunction|SetMenu "/Game/FP/GUI/Widgets/3D_Menu/Instance/BP_Menu_Won.BP_Menu_Won_C")
    (else
      (Default|ClearAll _hud)
      (Default|PlayLevelFinishLose (Variables|Managers|GetSound%20Manager%20Level))
      (CallFunction|SetMenu "/Game/FP/GUI/Widgets/3D_Menu/Instance/BP_Menu_Lose.BP_Menu_Lose_C"))))

(event EventOnLevelReady
  ;[1 1 1] Show Presentation Menu
  (Variables|State|Setstatus "NewEnumerator1")
  (Default|PlayLevelIntroMusicBg (Variables|Managers|GetSound%20Manager%20Level))
  (CallFunction|SetMenu "/Game/FP/GUI/Widgets/3D_Menu/Instance/BP_Menu_Presentation.BP_Menu_Presentation_C"))

(event EventStartIntro
  (bind _sound_manager_level (Variables|Managers|GetSound%20Manager%20Level))
  (Variables|State|Setstatus "NewEnumerator2")
  (Default|StopLevelIntroMusicBg _sound_manager_level)
  (Default|PlayLevelGameMusicBg _sound_manager_level)
  (CallFunction|SetGame)
  ;[1 1 1] Intro Movemente of Camera
  (bind _playermovement (CallFunction|GetCustomPlayer self))
  (Default|PlayMovement _playermovement (Default|GetStartPosition (Variables|Board|GetBoard_Master)) 6.0)
  (EventDispatchers|BindEventtoMovementFinished _playermovement (delegate EventOnIntroReady)))

(event EventOnIntroReady
  (bind _board_master (Variables|Board|GetBoard_Master))
  (bind _bounds (Default|GetBoardMovementsBounds _board_master))
  (Variables|State|Setstatus "NewEnumerator4")
  (bind (_gameinstance _thememanager _soundmanager_app _playercontroller) (CallFunction|GetCustomClasses self))
  (bind _soundmanager (Default|GetSoundClassManager _gameinstance))
  (Default|SetMute _soundmanager "NewEnumerator4" false)
  (Default|SetBoundsBORRAR _playercontroller (Default|GetBoardBoundsBORRAR _board_master) 1e+03 5e+02 true)
  (bind _debugmode (CallFunction|GetDebugMode self))
  (Default|SetMovementBoundsParameters _playercontroller (Utilities|Struct|MakePlayerMovementBoundsDefinition (not _debugmode) (.bounds_origin _bounds) (+ (.bounds_extents _bounds) 1000) "500.000000,500.000000,500.000000" (.normal_vector_x _bounds) (.normal_vector_y _bounds)))
  (Default|StartTimer (Variables|Default|GetTimer))
  (CallFunction|SetGame)
  (CallFunction|AddRemoveInputMappingContext "/Game/FP/BluePrints/Global_BP/Inputs/pause_inputs.pause_inputs" true))

(fn ConstructionScript)

(fn AddRemoveInputMappingContext
  (params (Input%20Mapping%20Context :type Input%20Mapping%20Context%20Object%20Reference) (Add%20Input :type Boolean))
  (bind _returnvalue (Game|GetPlayerController 0))
  (bind _returnvalue_2 (PlayerController|LocalPlayerSubsystems|GetEnhancedInputLocalPlayerSubsystem _returnvalue))
  (if Add%20Input
    (Input|AddMappingContext _returnvalue_2 Input%20Mapping%20Context 0 "(bIgnoreAllPressedKeysUntilRelease=True,bForceImmediately=False,bNotifyUserSettings=False)")
    (else
      (Input|RemoveMappingContext _returnvalue_2 Input%20Mapping%20Context "(bIgnoreAllPressedKeysUntilRelease=True,bForceImmediately=False,bNotifyUserSettings=False)"))))

(fn GetLastMenu
  (bind _lastmenu (Variables|Default|GetlastMenu))
  (return _lastmenu (Utilities|IsValidClass _lastmenu)))