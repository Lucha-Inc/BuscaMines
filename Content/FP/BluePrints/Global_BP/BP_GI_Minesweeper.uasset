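; Game instance for the Minesweeper game that owns shared managers and handles level travel.
; Init constructs the theme manager and caches its app theme data asset, which feeds the lazily created sound manager; a sound-class manager actor is also spawned on demand.
; Classic games store their level config for restarts, then open the game level through a fade-in widget callback.
; It also provides menu travel, fade-out, 2D audio creation and a log-order counter.
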(event EventInit
  (Utilities|FlowControl|Sequence
    (:then_0
      (bind _returnvalue (Game|ConstructObjectfromClass "/Game/FP/BluePrints/Global_BP/ActorsManagers/Theme/BP_ThemeManager.BP_ThemeManager_C"))
      (Variables|ManagersandDataAsset|SetTheme_Manager _returnvalue))
    (:then_1
      (Variables|Theme|SetDA%20Theme%20App (Default|GetDataAssetThemeApp (Variables|ManagersandDataAsset|GetTheme_Manager) "NewEnumerator0")))))

(event Custom|Go%20to%20level%20CLASSIC
  (params (Level%20Config :type Structu%20Level%20Configuration%20Structure))
  (Variables|LASTLEVEL|SetLast_level_config Level%20Config)
  (bind _returnvalue (UserInterface|CreateWidget "/Game/FP/GUI/Widgets/LevelTransition/LevelTransitio_FadeIn.LevelTransitio_FadeIn_C" (Game|GetPlayerController 0) true))
  (UserInterface|Viewport|AddtoViewport _returnvalue 0)
  (EventDispatchers|BindEventtoFadeinFinished _returnvalue (delegate Custom|createNewLevel)))

(event Custom|Go%20to%20level%20Main%20Menu
  (Game|OpenLevel(byObjectReference) "/Game/FP/Maps/menu_level.menu_level"))

(event Custom|Go%20to%20level%20Restart
  (CallFunction|GotoLevelCLASSIC (Variables|LASTLEVEL|GetLast_level_config)))

(event Custom|PlayFadeOutLevel
  (bind _returnvalue (UserInterface|CreateWidget "/Game/FP/GUI/Widgets/LevelTransition/LevelTransitio_FadeIn.LevelTransitio_FadeIn_C" (Game|GetPlayerController 0) false true))
  (UserInterface|Viewport|AddtoViewport _returnvalue 0))

(event Custom|createNewLevel
  (Game|OpenLevel(byObjectReference) "/Game/FP/Maps/game_level.game_level"))

(fn GetLogOrder
  (bind _output_get (Variables|DEBUG|Setlog_counter (+ (Variables|DEBUG|Getlog_counter) 1)))
  (return _output_get))

(fn GetSoundClassManager
  (Utilities|IsValid (Variables|ManagersandDataAsset|GetSoundClass_Manager)
    (:Is%20Valid
      (return (Variables|ManagersandDataAsset|GetSoundClass_Manager)))
    (:Is%20Not%20Valid
      (bind _returnvalue (Game|SpawnActorfromClass "/Game/FP/BluePrints/Global_BP/ActorsManagers/Sound/BP_SoundClass_Manager.BP_SoundClass_Manager_C" (Math|Transform|MakeTransform "0, 0, 0") "Undefined" "MultiplyWithRoot" 0 0))
      (bind _output_get (Variables|ManagersandDataAsset|SetSoundClass_Manager _returnvalue))
      (return _output_get))))

(fn GetThemeManager
  (return (Variables|ManagersandDataAsset|GetTheme_Manager)))

(fn CreateAudio
  (params (Sound :type Sound%20Base%20Object%20Reference) (Persist :type Boolean) (Destroy :type Boolean))
  (bind _returnvalue (Audio|CreateSound2D Sound 1.0 1.0 0.0 0 Persist Destroy))
  (return _returnvalue))

(fn GetSoundManagerApp
  (Utilities|IsValid (Variables|ManagersandDataAsset|GetSound_Manager_App)
    (:Is%20Valid
      (return (Variables|ManagersandDataAsset|GetSound_Manager_App)))
    (:Is%20Not%20Valid
      (bind _returnvalue (Game|ConstructObjectfromClass "/Game/FP/BluePrints/Global_BP/ActorsManagers/Sound/BP_Sound_Manager_App.BP_Sound_Manager_App_C" (Variables|Theme|GetDA%20Theme%20App) self))
      (bind _output_get (Variables|ManagersandDataAsset|SetSound_Manager_App _returnvalue))
      (return _output_get))))

(fn GetLastLevelConfig
  (return (Variables|LASTLEVEL|GetLast_level_config)))